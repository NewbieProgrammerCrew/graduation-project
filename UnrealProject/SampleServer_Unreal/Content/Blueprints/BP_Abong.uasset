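; BP_Abong is an actor that mirrors data from a DataUpdater reference and shows a floating role label.
; Each Tick, while DataUpdater is valid, it copies CurrentSpeed into its own Speed and writes MRole to a TextRender.
; The label rotates every frame to face the player camera, billboard style.
; An FInterpTo speed-smoothing step is left unconnected, so Speed follows the source value directly.
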(event EventBeginPlay)

(event Collision|EventActorBeginOverlap
  (params (OtherActor :type Actor%20Object%20Reference)))

(event EventTick
  (params (DeltaSeconds :type Float%20%28single-precision%29))
  (bind _dataupdater (Variables|Default|GetDataUpdater))
  (bind _textrender (Variables|Default|GetTextRender))
  (Utilities|IsValid _dataupdater
    (:Is%20Valid
      (Variables|Default|SetSpeed (Variables|/Script/NPC_World.DataUpdater|GetCurrentSpeed _dataupdater))
      (Rendering|Components|TextRender|SetText (Variables|Default|GetTextRender) (Utilities|Text|ToText(String) (Variables|/Script/NPC_World.DataUpdater|Getm_role _dataupdater)))
      (Transformation|SetWorldRotation _textrender (Math|Rotator|FindLookatRotation (Transformation|GetWorldLocation _textrender) (Camera|GetCameraLocation (Game|GetPlayerCameraManager 0))) false false))))

(fn ConstructionScript)