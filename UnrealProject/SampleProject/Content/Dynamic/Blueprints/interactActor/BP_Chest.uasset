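; BP_Chest is an interactable loot chest that players open through the repair interaction.
; Server-side overlap with a BP_Parent shows the interact UI while closed and hides the progress bar on exit.
; Completed repair plays the opening animation, then the server spawns random loot at random spots, adds a part from GamePlayState's shared pool while shrinking it, and recolors the lamp.
; Cancelling repair spawns a flare.
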(event OnComponentBeginOverlap(Bound)
  (params (OverlappedComponent :type Primitive%20Component%20Object%20Reference) (OtherActor :type Actor%20Object%20Reference) (OtherComp :type Primitive%20Component%20Object%20Reference) (OtherBodyIndex :type Integer) (bFromSweep :type Boolean) (SweepResult :type Hit%20Result%20Structure%20%28by%20ref%29))
  ;[1 0.5 0.5] Player Overlap
  (Networking|SwitchHasAuthority
    (:Authority
      (bind _asbp_parent (Utilities|Casting|CastToBP_Parent OtherActor))
      (if (not (Variables|Default|GetOpen))
        (Default|UIINFO _asbp_parent self)))))

(event OnComponentEndOverlap(Bound)
  (params (OverlappedComponent :type Primitive%20Component%20Object%20Reference) (OtherActor :type Actor%20Object%20Reference) (OtherComp :type Primitive%20Component%20Object%20Reference) (OtherBodyIndex :type Integer))
  ;[1 0.5 0.5] Player Overlap
  (Networking|SwitchHasAuthority
    (:Authority
      (bind _asbp_parent (Utilities|Casting|CastToBP_Parent OtherActor))
      (Default|PBarHidden _asbp_parent))))

(event Custom|ClearRepair
  ;[1 0.375 0.375] Repairing Bool
  (CallFunction|ServerClearRepair))

(event Custom|CancleRepair
  (CallFunction|ShootFlare))

(event Custom|ShootFlare
  (bind _returnvalue (Game|SpawnActorfromClass "/Game/Dynamic/Blueprints/AllLevels/BP_ChestFlare.BP_ChestFlare_C" (Transformation|GetWorldTransform (Variables|Default|GetSpawnPoint)) "Undefined" 0 0))
  (Variables|Default|SetFlare _returnvalue))

(event Custom|Server_ClearRepair
  (bind _returnvalue (Game|GetGameState))
  (bind _asgame_play_state (Utilities|Casting|CastToGamePlayState _returnvalue))
  (bind _partsitems (Variables|/Game/Dynamic/Blueprints/AllLevels/GamePlayState.GamePlayState_C|GetPartsItems _asgame_play_state))
  (bind (_outitem _outindex) (Utilities|Array|Random _partsitems))
  ;[1 0.375 0.375] Repairing Bool
  (Variables|Default|SetOpen true)
  (Components|Animation|PlayAnimation (Variables|Default|GetSkeletalMesh) "/Game/Static/Chest/ChestOpenAnimation_Anim.ChestOpenAnimation_Anim" false)
  (Networking|SwitchHasAuthority
    (:Authority
      (Utilities|FlowControl|Delay 0.7)
      (if (Utilities|Array|IsEmpty (Variables|/Game/Dynamic/Blueprints/AllLevels/GamePlayState.GamePlayState_C|GetPartsItems (.AsGame%20Play%20State (Utilities|Casting|CastToGamePlayState (Game|GetGameState)))))
        (Game|SpawnActorfromClass (.OutItem (Utilities|Array|Random (Variables|Default|Getitems))) (Math|Transform|MakeTransform (Transformation|GetWorldLocation (.OutItem (Utilities|Array|Random (Variables|Default|GetspawnArea)))) "0, 0, 0" "1.000000,1.000000,1.000000") "Undefined" 0 0)
        (else
          (Game|SpawnActorfromClass (.OutItem (Utilities|Array|Random (Variables|Default|Getitems))) (Math|Transform|MakeTransform (Transformation|GetWorldLocation (.OutItem (Utilities|Array|Random (Variables|Default|GetspawnArea)))) "0, 0, 0" "1.000000,1.000000,1.000000") "Undefined" 0 0)
          (Game|SpawnActorfromClass _outitem (Math|Transform|MakeTransform (Transformation|GetWorldLocation (.OutItem (Utilities|Array|Random (Variables|Default|GetspawnArea)))) "0, 0, 0" "1.000000,1.000000,1.000000") "Undefined" 0 0)
          (Default|RemoveItemIndex (.AsGame%20Play%20State (Utilities|Casting|CastToGamePlayState (Game|GetGameState))) _outindex)))
      (CallFunction|SendChangeColor))))

(event Custom|sendChangeColor
  ;[1 0.375 0.375] Repairing Bool
  (bind _asbp_lamp (Utilities|Casting|CastToBP_Lamp (Variables|/Script/Engine.ChildActorComponent|GetChildActor (Variables|Default|GetBP_Lamp))))
  (Rendering|Components|Light|SetLightColor (Variables|/Game/Dynamic/Blueprints/AllLevels/BP_Lamp.BP_Lamp_C|GetPointLight _asbp_lamp) "(R=0.000000,G=0.598466,B=1.000000,A=1.000000)" true))

(event EventBeginPlay
  (Variables|Default|SetspawnArea (Utilities|Array|MakeArray (Variables|Default|GetCube6) (Variables|Default|GetCube5) (Variables|Default|GetCube4) (Variables|Default|GetCube2) (Variables|Default|GetCube1) (Variables|Default|GetCube7))))

(event Collision|EventActorBeginOverlap
  (params (OtherActor :type Actor%20Object%20Reference)))

(event EventTick
  (params (DeltaSeconds :type Float%20%28single-precision%29)))

(fn ConstructionScript)

(fn RepairState
  (return (Variables|Default|GetOpen)))