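; BP_Handle is a handle actor that opens a pair of doors when pulled down.
; Its Down event plays the HandleDown timeline, which drives the mesh's relative pitch.
; When the timeline finishes, it finds the first BP_LeftDoor and BP_RightDoor in the level and passes both to ServerOpenDoor on GamePlayState.
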(event Custom|Down
  (bind _handle (Timeline|HandleDown Play)
    (:Update
      (Transformation|SetRelativeRotation (Variables|Debug|GetStaticMeshComponent) (Math|Rotator|MakeRotator 0.0 _handle 0.0) false false))
    (:Finished
      (bind _outactors (Actor|GetAllActorsOfClass "/Game/Dynamic/Blueprints/interactActor/BP_LeftDoor.BP_LeftDoor_C"))
      (bind _output_get (Variables|Default|SetleftDoor _outactors))
      (bind _outactors_2 (Actor|GetAllActorsOfClass "/Game/Dynamic/Blueprints/interactActor/BP_RightDoor.BP_RightDoor_C"))
      (bind _output_get_2 (Variables|Default|SetRightDoor _outactors_2))
      (Default|ServerOpenDoor (.AsGame%20Play%20State (Utilities|Casting|CastToGamePlayState (Game|GetGameState))) (Utilities|Array|Get(acopy) _output_get) (Utilities|Array|Get(acopy) _output_get_2)))))

(event EventBeginPlay)

(event Collision|EventActorBeginOverlap
  (params (OtherActor :type Actor%20Object%20Reference)))

(event EventTick
  (params (DeltaSeconds :type Float%20%28single-precision%29)))

(fn ConstructionScript)