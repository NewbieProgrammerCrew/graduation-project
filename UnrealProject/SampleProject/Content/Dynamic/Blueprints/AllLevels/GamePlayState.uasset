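; GamePlayState is the game state for a killer-versus-survivors match, tracking remaining parts and deciding which side wins.
; CheckPlayerDie scans PlayerArray, giving survivors the win if the killer dies, or the killer if all survivors are dead or iced.
; Earning all parts shows a survivor win widget once and flags the door open.
; Helper events refill or remove part items, decrement the parts count and open both doors.
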(event Custom|CheckPlayerDie
  (bind _playerarray (Variables|Default|GetPlayerArray))
  (bind _array_element (Utilities|Array|ForEachLoopwithBreak _playerarray :!label _label)
    (:LoopBody
      (if (Variables|/Game/Dynamic/Blueprints/AllLevels/PlayerStateBP.PlayerStateBP_C|GetIsKiller? (.AsPlayer%20State%20BP (Utilities|Casting|CastToPlayerStateBP _array_element)))
        (if (Variables|/Game/Dynamic/Blueprints/AllLevels/PlayerStateBP.PlayerStateBP_C|GetKillerDie? (.AsPlayer%20State%20BP (Utilities|Casting|CastToPlayerStateBP _array_element)))
          (Variables|Default|Setplayer false)
          (goto _label Break))
        (elif (or (Variables|/Game/Dynamic/Blueprints/AllLevels/PlayerStateBP.PlayerStateBP_C|GetDie? (.AsPlayer%20State%20BP (Utilities|Casting|CastToPlayerStateBP _array_element))) (Variables|/Game/Dynamic/Blueprints/AllLevels/PlayerStateBP.PlayerStateBP_C|Getice? (.AsPlayer%20State%20BP (Utilities|Casting|CastToPlayerStateBP _array_element))))
          (Math|Integer|IncrementInt (Variables|Default|Getcount)
            (:%20%20
              (Variables|Default|Setplayer true))))))
    (:Completed
      (if (Variables|Default|Getplayer)
        (if (== (Utilities|Array|LastIndex _playerarray) (Variables|Default|Getcount))
          (CallFunction|KillerWinVDPlay)
          (else
            (Variables|Default|Setcount 0)))
        (else
          (CallFunction|SurvivorWinWB))))))

(event Custom|KillerWinVDPlay
  (bind _returnvalue (UserInterface|CreateWidget "/Game/Dynamic/Blueprints/Widget/WBP_KillerWin.WBP_KillerWin_C"))
  (UserInterface|Viewport|AddtoViewport _returnvalue 0)
  (Variables|/Script/Engine.PlayerController|SetbShowMouseCursor (Game|GetPlayerController 0) true))

(event Custom|SurvivorWinVDPlay
  (Utilities|FlowControl|DoOnce false
    (:Completed
      (bind _returnvalue (UserInterface|CreateWidget "/Game/Dynamic/Blueprints/Widget/WBP_SurvivorWin.WBP_SurvivorWin_C"))
      (UserInterface|Viewport|AddtoViewport _returnvalue 0)
      (Variables|Default|SetdoorisOpen true))))

(event Custom|ResetItems
  (for _index (range 1 8)
    (Utilities|Array|Add (Variables|Default|GetPartsItems) (Variables|Default|GetPartsItem))))

(event Custom|Survivor_WinWB
  (bind _returnvalue (UserInterface|CreateWidget "/Game/Dynamic/Blueprints/Widget/SurvivorWinWBPR.SurvivorWinWBPR_C"))
  (UserInterface|Viewport|AddtoViewport _returnvalue 0)
  (Variables|/Script/Engine.PlayerController|SetbShowMouseCursor (Game|GetPlayerController 0) true))

(event Custom|RemoveItemIndex
  (params (index :type Integer))
  (Utilities|Array|RemoveIndex (Variables|Default|GetPartsItems) index))

(event Custom|Server_OpenDoor
  (params (leftDoor :type BP%20Left%20Door%20Object%20Reference) (rightDoor :type BP%20Right%20Door%20Object%20Reference))
  (Default|OpenDoor leftDoor)
  (Default|OpenDoor rightDoor))

(event Custom|DecreasePartsCount
  (Math|Integer|DecrementInt (Variables|Default|GetRemainPartsCount)))

(event Custom|CheckEarnAllParts
  (CallFunction|SurvivorWinVDPlay))

(event EventBeginPlay
  (Variables|Default|SetRemainPartsCount 6))

(fn ConstructionScript)