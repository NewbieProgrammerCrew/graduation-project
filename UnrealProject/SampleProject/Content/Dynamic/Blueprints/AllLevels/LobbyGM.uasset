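; Lobby game mode that manages joining players, character pawns and the server travel into a match.
; On authority, PostLogin registers each controller, sets up its LobbyPC menu and possesses a pawn at a random PlayerStart.
; EveryoneUpdate pushes player info and available characters to all controllers, clearing CanWeStart if anyone still has BP_Parent.
; SwapCharacter respawns the chosen class; LaunchTheGame randomly travels to World1 or World2, while kick and settings events are empty.
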(event Custom|Respawn%20Player
  (params (PlayerController :type Player%20Controller%20Object%20Reference))
  (bind _returnvalue (Pawn|GetControlledPawn PlayerController))
  (bind _spawnpoint (Variables|Default|GetSpawnPoint))
  (Utilities|IsValid _returnvalue
    (:Is%20Valid
      (Actor|DestroyActor _returnvalue))
    (:Is%20Not%20Valid
      _))
  (bind _returnvalue_2 (Game|SpawnActorfromClass "/Game/Dynamic/Blueprints/Lobby_Character/0_Base.0_Base_C" (Transformation|GetActorTransform (Utilities|Array|Get(acopy) _spawnpoint (Math|Random|RandomIntegerinRange 0 (- (Utilities|Array|Length _spawnpoint) 1)))) "Undefined" 0 0))
  (Pawn|Possess PlayerController _returnvalue_2)
  (CallFunction|EveryoneUpdate))

(event Custom|EveryoneUpdate
  (bind _allplayercontrollers (Variables|ServerSettings|GetAllPlayerControllers))
  ;[1 1 1] Update all Connected Player 's lobby information when called
  (bind _output_get (Variables|ServerSettings|SetCurrentPlayers (Utilities|Array|Length (Variables|ServerSettings|GetAllPlayerControllers))))
  (if (> _output_get 0)
    (Utilities|Array|Clear (Variables|ServerSettings|GetConnectedPlayers))
    (for _array_element _allplayercontrollers
      (bind _aslobby_pc (Utilities|Casting|CastToLobbyPC _array_element))
      (Utilities|Array|Add (Variables|ServerSettings|GetConnectedPlayers) (Variables|/Game/Dynamic/Blueprints/AllLevels/LobbyPC.LobbyPC_C|GetPlayer%20Settings _aslobby_pc))
      (Default|UpdateNumberOfPlayer _aslobby_pc (Variables|ServerSettings|GetCurrentPlayers) (Variables|ServerSettings|GetMax%20Player)))
    (for _array_element_2 _allplayercontrollers
      (bind _aslobby_pc_2 (Utilities|Casting|CastToLobbyPC _array_element_2))
      (Default|AddPlayerInfo _aslobby_pc_2 (Variables|ServerSettings|GetConnectedPlayers))
      (Default|UpdateAvailableCharacters _aslobby_pc_2 (Variables|ServerSettings|GetAvailable%20Characters))
      (CallFunction|AddtoKickList))
    (bind _array_element_3 (Utilities|Array|ForEachLoopwithBreak (Variables|ServerSettings|GetConnectedPlayers))
      (:LoopBody
        (if (== (.MyPlayerCharacter (Utilities|Struct|BreakPlayerInfo _array_element_3)) "/Game/Dynamic/Blueprints/Character_BP/BP_Parent.BP_Parent_C")
          (Variables|ServerSettings|SetCanWeStart? false)
          (CallFunction|CannotStartGame)
          (else
            (Variables|ServerSettings|SetCanWeStart? true)))))))

(event Custom|SwapCharacter
  (params (PlayerController :type Player%20Controller%20Object%20Reference) (CharacterClass :type Character%20Class%20Reference) (ChangeStatus :type Boolean))
  (bind _returnvalue (Pawn|GetControlledPawn PlayerController))
  (bind _spawnpoint (Variables|Default|GetSpawnPoint))
  (if (not ChangeStatus)
    (Utilities|IsValid _returnvalue
      (:Is%20Valid
        (Actor|DestroyActor _returnvalue))
      (:Is%20Not%20Valid
        _))
    (bind _returnvalue_2 (Game|SpawnActorfromClass CharacterClass (Transformation|GetActorTransform (Utilities|Array|Get(acopy) _spawnpoint (Math|Random|RandomIntegerinRange 0 (- (Utilities|Array|Length _spawnpoint) 1)))) "Undefined" 0 0))
    (Pawn|Possess PlayerController _returnvalue_2)))

(event Custom|LaunchTheGame
  (bind _returnvalue (Game|GetPlayerController 0))
  ;[1 1 1] Launch the game rnadom Map
  (switch int (Math|Random|RandomIntegerinRange 0 3)
    (:0
      (Development|ExecuteConsoleCommand "servertravel/Game/Static/Maps/World1" _returnvalue :!label _label))
    (:1
      (Development|ExecuteConsoleCommand "servertravel/Game/Static/Maps/World2" _returnvalue :!label _label_2))
    (:2
      (goto _label))
    (:3
      (goto _label_2))))

(event Custom|AddToKickList)

(event Custom|CannotStartGame
  ;[1 1 1] Update all Connected Player 's lobby information when called
  (Utilities|Array|ForEachLoopwithBreak (Variables|ServerSettings|GetConnectedPlayers)) ; enters at Break
)

(event Custom|ServerUpdateGameSettings
  (params (Map%20Name :type Text) (MapId :type Integer)))

(event EventPostLogin
  (params (NewPlayer :type Player%20Controller%20Object%20Reference))
  (Networking|SwitchHasAuthority
    (:Authority
      (Utilities|Array|Add (Variables|ServerSettings|GetAllPlayerControllers) NewPlayer)
      (bind _outactors (Actor|GetAllActorsOfClass "/Script/Engine.PlayerStart"))
      (Variables|Default|SetSpawnPoint _outactors)
      (bind _asgame_info_instance (Utilities|Casting|CastToGameInfoInstance (Game|GetGameInstance)))
      (Variables|ServerSettings|SetServer%20Name (Variables|/Game/Dynamic/Blueprints/AllLevels/GameInfoInstance.GameInfoInstance_C|GetServer%20Name _asgame_info_instance))
      (Variables|ServerSettings|SetMax%20Player (Variables|/Game/Dynamic/Blueprints/AllLevels/GameInfoInstance.GameInfoInstance_C|GetMax%20Player _asgame_info_instance))
      (bind _aslobby_pc (Utilities|Casting|CastToLobbyPC NewPlayer))
      (Default|InitialSetup _aslobby_pc)
      (Default|SetupLobbyMenu _aslobby_pc (Variables|ServerSettings|GetServer%20Name))
      (CallFunction|RespawnPlayer NewPlayer))))

(fn ConstructionScript)