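; Gameplay player controller that loads saved player settings, has the game mode respawn the chosen character and manages the player's inventory and door UI.
; On local BeginPlay it loads the save and passes it on for respawn, then creates the inventory widget, which is rebuilt as items change.
; The door widget polls GamePlayState's remaining parts count on Tick; matching items decrement it, and zero triggers the all-parts-earned check.
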(event Custom|PassCharacterInfoToServer
  (params (PlayerSettingINfo :type Player%20Info%20Structure))
  (Variables|Default|SetPlayerSettings PlayerSettingINfo)
  (bind _asgame_play_gm (Utilities|Casting|CastToGamePlayGM (Game|GetGameMode)))
  (Default|RespawnPlayer _asgame_play_gm self (.MyPlayerCharacter (Utilities|Struct|BreakPlayerInfo (Variables|Default|GetPlayerSettings))))
  (CallFunction|SetupInventoryWidget))

(event Custom|Setup%20Inventory%20Widget
  ;[1 1 1] Set up and display the Inventory
  (bind _returnvalue (UserInterface|CreateWidget "/Game/Dynamic/Blueprints/Widget/Inventory.Inventory_C"))
  (bind _output_get (Variables|Default|SetInventoryWB _returnvalue))
  (UserInterface|Viewport|AddtoViewport _output_get 0))

(event Custom|CallServerDecreasePartsCount
  (params (widget :type Door%20Widget%20Object%20Reference))
  (Default|DecreasePartsCount (.AsGame%20Play%20State (Utilities|Casting|CastToGamePlayState (Game|GetGameState)))))

(event Custom|SendServer
  (Default|CheckEarnAllParts (.AsGame%20Play%20State (Utilities|Casting|CastToGamePlayState (Game|GetGameState)))))

(event Custom|AddItemInfo
  (params (ItemInfo :type Array%20of%20Item%20INFO%20Structures))
  (bind _inventorywb (Variables|Default|GetInventoryWB))
  (Variables|Default|Setinventory ItemInfo)
  (Utilities|IsValid _inventorywb
    (:Is%20Valid
      (Default|ClearItemList _inventorywb)
      (for _array_element (Variables|Default|Getinventory)
        (Default|UpdateInventoryWindow (Variables|Default|GetInventoryWB) _array_element)))))

(event Custom|SelectItem
  (params (index :type Integer))
  (bind _inventorywb (Variables|Default|GetInventoryWB))
  (Utilities|IsValid _inventorywb
    (:Is%20Valid
      (Default|SelectItem _inventorywb index))))

(event Custom|ClearInventory
  (params (index :type Integer))
  (bind _inventorywb (Variables|Default|GetInventoryWB))
  (Utilities|Array|RemoveIndex (Variables|Default|Getinventory) index)
  (Utilities|IsValid _inventorywb
    (:Is%20Valid
      (Default|ClearItemList _inventorywb)
      (for _array_element (Variables|Default|Getinventory)
        (Default|UpdateInventoryWindow (Variables|Default|GetInventoryWB) _array_element)))))

(event Custom|CallIceBreak
  (params (iced%20player :type Actor%20Object%20Reference))
  (bind _asbp_parent (Utilities|Casting|CastToBP_Parent iced%20player))
  (Default|SeverRockHidden _asbp_parent))

(event Custom|Setup%20Door%20Widget
  ;[1 1 1] Setup Door Widget
  (bind _returnvalue (UserInterface|CreateWidget "/Game/Dynamic/Blueprints/Widget/DoorWidget.DoorWidget_C"))
  (bind _output_get (Variables|Default|SetDoorWB _returnvalue))
  (UserInterface|Viewport|AddtoViewport _output_get 0)
  (Default|SetCountValue (Variables|Default|GetDoorWB) (Variables|/Game/Dynamic/Blueprints/AllLevels/GamePlayState.GamePlayState_C|GetRemainPartsCount (.AsGame%20Play%20State (Utilities|Casting|CastToGamePlayState (Game|GetGameState))))))

(event Custom|FindItem
  (params (itemInventory :type Array%20of%20Item%20INFO%20Structures))
  (bind _doorwb (Variables|Default|GetDoorWB))
  (bind _array_element (Utilities|Array|ForEachLoopwithBreak itemInventory)
    (:LoopBody
      (if (Utilities|Enum|Equal(Enum) (.ItemType (Utilities|Struct|BreakItemINFO _array_element)) "NewEnumerator2")
        (Utilities|IsValid _doorwb
          (:Is%20Valid
            (CallFunction|CallServerDecreasePartsCount _doorwb)
            (if (<= (Variables|/Game/Dynamic/Blueprints/Widget/DoorWidget.DoorWidget_C|Getcount _doorwb) 0)
              (CallFunction|SendServer))))))))

(event Custom|CustomEvent)

(event Custom|Destroy%20Door%20Widget
  (Widget|RemovefromParent (Variables|Default|GetDoorWB))
  (Variables|Default|SetDoorWB 0))

(event EventBeginPlay
  ;[1 1 1] Loads Player Info and Pass to Server player Controller
  (if (Pawn|IsLocalController)
    (Viewport|RemoveAllWidgets)
    (CallFunction|LoadGame)
    (CallFunction|PassCharacterInfotoServer (Variables|Default|GetPlayerSettings))
    (Input|SetInputModeGameOnly self false)))

(event EventTick
  (params (DeltaSeconds :type Float%20%28single-precision%29))
  (bind _doorwb (Variables|Default|GetDoorWB))
  (Utilities|IsValid _doorwb
    (:Is%20Valid
      (Default|SetCountValue _doorwb (Variables|/Game/Dynamic/Blueprints/AllLevels/GamePlayState.GamePlayState_C|GetRemainPartsCount (.AsGame%20Play%20State (Utilities|Casting|CastToGamePlayState (Game|GetGameState)))))
      (if (<= (Variables|/Game/Dynamic/Blueprints/Widget/DoorWidget.DoorWidget_C|Getcount (Variables|Default|GetDoorWB)) 0)
        (CallFunction|SendServer)))))

(fn ConstructionScript)

(fn LoadGame
  (bind _returnvalue (SaveGame|LoadGamefromSlot (Variables|Default|GetPlayerSettingsSave)))
  (bind _asplayer_save_game (Utilities|Casting|CastToPlayerSaveGame _returnvalue))
  (Variables|Default|SetPlayerSettings (Variables|/Game/Dynamic/Blueprints/AllLevels/PlayerSaveGame.PlayerSaveGame_C|GetS_PlayerInfo _asplayer_save_game)))