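; BP_ChestFlare is a rising flare actor that flies straight up until it hits a trigger box.
; On BeginPlay it attaches the NS_Flare Niagara effect to its Box component.
; Tick moves the Box up by a fixed, frame-rate-dependent step without sweeping, and plays a launch sound once through a DoOnce.
; When the Box overlaps a TriggerBox, the actor destroys itself.
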(event OnComponentBeginOverlap(Box)
  (params (OverlappedComponent :type Primitive%20Component%20Object%20Reference) (OtherActor :type Actor%20Object%20Reference) (OtherComp :type Primitive%20Component%20Object%20Reference) (OtherBodyIndex :type Integer) (bFromSweep :type Boolean) (SweepResult :type Hit%20Result%20Structure%20%28by%20ref%29))
  (Utilities|Casting|CastToTriggerBox OtherActor)
  (Actor|DestroyActor))

(event Collision|EventActorBeginOverlap
  (params (OtherActor :type Actor%20Object%20Reference)))

(event EventBeginPlay
  (Niagara|SpawnSystemAttached "/Game/Static/NS_Flare.NS_Flare" (Variables|Default|GetBox) "None" "0, 0, 0" "0, 0, 0" "KeepRelativeOffset" false))

(event EventTick
  (params (DeltaSeconds :type Float%20%28single-precision%29))
  (Transformation|AddWorldOffset (Variables|Default|GetBox) "0.000000,0.000000,10.000000" false false)
  (Utilities|FlowControl|DoOnce false
    (:Completed
      (Audio|PlaySoundatLocation "/Game/Static/Music/Missile_Launch_Sound_Effect_Cue.Missile_Launch_Sound_Effect_Cue" (Transformation|GetWorldLocation (Variables|Default|GetBox)) "0, 0, 0" 0.3 1.0 0.0 0 0 0 0))))

(fn ConstructionScript)