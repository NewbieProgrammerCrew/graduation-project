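; Child character Blueprint that supplies Kate's aim, shoot, slash and death animations by overriding the parent's animation functions.
; Most overrides call a server event that relays to an RPC or multicast event playing the montage, but StopAimAnim calls its RPC event directly, skipping the server relay.
; DoOnce gates stop aim and slash montages restarting until completed or interrupted.
; Death plays a non-looping animation directly on the mesh.
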(event Custom|Server_RPC_Aim_Animation
  (CallFunction|RPCAimAnimation))

(event Custom|RPC_Aim_Animation
  (Utilities|FlowControl|DoOnce false :!label _label
    (:Completed
      (Animation|Montage|PlayMontage (Variables|Character|GetMesh) "/Game/Static/Characters/Animation/RifleAnim/MTG_Kate_Fire.MTG_Kate_Fire" 1.0 0.0 "Aim"
        (:OnCompleted
          (goto _label Reset))
        (:OnInterrupted
          (goto _label Reset))))))

(event Custom|RPC_NonAim_Animation
  (Animation|StopAnimMontage "/Game/Static/Characters/Animation/RifleAnim/MTG_Kate_Fire.MTG_Kate_Fire"))

(event Custom|Server_RPC_NonAim_Animation
  (CallFunction|RPCNonAimAnimation))

(event Custom|RPC_Server_Shoot
  (CallFunction|RPCShoot))

(event Custom|RPC_Shoot
  (Animation|PlayAnimMontage "/Game/Static/Characters/Animation/RifleAnim/MTG_Kate_Fire.MTG_Kate_Fire" 1.0 "Fire"))

(event Custom|Server_RPC_SlashAnim
  (CallFunction|RPCSlashAnim))

(event Custom|RPC_SlashAnim
  (Utilities|FlowControl|DoOnce false :!label _label
    (:Completed
      (Animation|Montage|PlayMontage (Variables|Character|GetMesh) "/Game/Static/Characters/Animation/Sword/MTG_KateSlash.MTG_KateSlash"
        (:OnCompleted
          (goto _label Reset))
        (:OnInterrupted
          (goto _label Reset))))))

(event Custom|Server_Play_Die
  (CallFunction|MulticastPlayDie))

(event Custom|Multicast_PlayDie
  (Components|Animation|PlayAnimation (Variables|Character|GetMesh) "/Game/Static/Characters/Animation/Kate_Falling_Back_Death__1_.Kate_Falling_Back_Death__1_" false))

(event EventBeginPlay
  (|CallParentFunction))

(event Collision|EventActorBeginOverlap
  (params (OtherActor :type Actor%20Object%20Reference))
  (|CallParentFunction OtherActor) ; This node is disabled and will not be called.\nDrag off pins to build functionality.
)

(event EventTick
  (params (DeltaSeconds :type Float%20%28single-precision%29))
  (|CallParentFunction DeltaSeconds))

(fn ConstructionScript
  (|CallParentFunction))

(fn PlayAimAnim
  (CallFunction|ServerRPCAimAnimation))

(fn StopAimAnim
  (CallFunction|RPCNonAimAnimation))

(fn PlayShootAnim
  (CallFunction|RPCServerShoot))

(fn PlaySlashAnim
  (CallFunction|ServerRPCSlashAnim))

(fn PlayDie
  (CallFunction|ServerPlayDie))