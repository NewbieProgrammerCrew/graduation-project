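; GamePlayPC is the gameplay player controller that hands the saved character choice to the game mode for spawning and manages the inventory UI.
; On local BeginPlay it loads player settings from the save slot and passes them toward the server, where GamePlayGM respawns the chosen character.
; That same event then creates the inventory widget.
; AddItemInfo rebuilds the widget's item list from the given items, and SelectItem forwards a selection index to it.
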(event Custom|PassCharacterInfoToServer
  (params (PlayerSettingINfo :type Player%20Info%20Structure))
  (Variables|Default|SetPlayerSettings PlayerSettingINfo)
  (bind _asgame_play_gm (Utilities|Casting|CastToGamePlayGM (Game|GetGameMode)))
  (Default|RespawnPlayer _asgame_play_gm self (.MyPlayerCharacter (Utilities|Struct|BreakPlayerInfo (Variables|Default|GetPlayerSettings))))
  (CallFunction|SetupInventoryWidget))

(event Custom|Setup%20Inventory%20Widget
  ;[1 1 1] Set up and display the Inventory
  (bind _returnvalue (UserInterface|CreateWidget "/Game/Blueprints/Widget/Inventory.Inventory_C"))
  (bind _output_get (Variables|Default|SetInventoryWB _returnvalue))
  (UserInterface|Viewport|AddtoViewport _output_get 0))

(event Custom|AddItemInfo
  (params (ItemInfo :type Array%20of%20Item%20INFO%20Structures))
  (bind _inventorywb (Variables|Default|GetInventoryWB))
  (Variables|Default|Setinventory ItemInfo)
  (Utilities|IsValid _inventorywb
    (:Is%20Valid
      (Default|ClearItemList _inventorywb)
      (for _array_element (Variables|Default|Getinventory)
        (Default|UpdateInventoryWindow (Variables|Default|GetInventoryWB) _array_element)))))

(event Custom|SelectItem
  (params (index :type Integer))
  (bind _inventorywb (Variables|Default|GetInventoryWB))
  (Utilities|IsValid _inventorywb
    (:Is%20Valid
      (Default|SelectItem _inventorywb index))))

(event EventBeginPlay
  ;[1 1 1] Loads Player Info and Pass to Server player Controller
  (if (Pawn|IsLocalController)
    (Viewport|RemoveAllWidgets)
    (CallFunction|LoadGame)
    (CallFunction|PassCharacterInfotoServer (Variables|Default|GetPlayerSettings))
    (Input|SetInputModeGameOnly self false)))

(fn ConstructionScript)

(fn LoadGame
  (bind _returnvalue (SaveGame|LoadGamefromSlot (Variables|Default|GetPlayerSettingsSave)))
  (bind _asplayer_save_game (Utilities|Casting|CastToPlayerSaveGame _returnvalue))
  (Variables|Default|SetPlayerSettings (Variables|/Game/Blueprints/AllLevels/PlayerSaveGame.PlayerSaveGame_C|GetS_PlayerInfo _asplayer_save_game)))