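; PlayerGameMode assigns each player who logs in a random, unique character and possesses it.
; PostLogin shuffles AvailableCharacters, spawns the first at the Note actor location indexed by PlayerCount, then removes it from the pool.
; Note actors are gathered only while SpawnPos is empty.
; If the spawn casts to BP_Parent or BP_Killer, the player controller at that index possesses it and PlayerCount increments.
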(event EventBeginPlay)

(event EventTick
  (params (DeltaSeconds :type Float%20%28single-precision%29)))

(event EventPostLogin
  (params (NewPlayer :type Player%20Controller%20Object%20Reference))
  (bind _availablecharacters (Variables|Default|GetAvailableCharacters))
  (bind _output (Utilities|Array|Get(acopy) _availablecharacters))
  (Utilities|Array|Shuffle (Variables|Default|GetAvailableCharacters))
  (if (> (Utilities|Array|Length (Variables|Default|GetSpawnPos)) 0)
    _
    (else
      (bind _outactors (Actor|GetAllActorsOfClass "/Script/Engine.Note"))
      (Variables|Default|SetSpawnPos _outactors)))
  (bind _returnvalue (Game|SpawnActorfromClass _output (Math|Transform|MakeTransform (Transformation|GetActorLocation (Utilities|Array|Get(acopy) (Variables|Default|GetSpawnPos) (Variables|Default|GetPlayerCount))) "0, 0, 0" "1.000000,1.000000,1.000000") "Undefined" 0 0))
  (Utilities|Array|RemoveItem (Variables|Default|GetAvailableCharacters) _output)
  (bind _asbp_parent (Utilities|Casting|CastToBP_Parent _returnvalue)
    (:then
      (Utilities|IsValid (Game|GetPlayerController (Variables|Default|GetPlayerCount))
        (:Is%20Valid
          (Pawn|Possess (Game|GetPlayerController (Variables|Default|GetPlayerCount)) _asbp_parent)
          (Math|Integer|IncrementInt (Variables|Default|GetPlayerCount)))))
    (:CastFailed
      (bind _asbp_killer (Utilities|Casting|CastToBP_Killer _returnvalue))
      (Utilities|IsValid (Game|GetPlayerController (Variables|Default|GetPlayerCount))
        (:Is%20Valid
          (Pawn|Possess (Game|GetPlayerController (Variables|Default|GetPlayerCount)) _asbp_killer)
          (Math|Integer|IncrementInt (Variables|Default|GetPlayerCount)))))))

(fn ConstructionScript)