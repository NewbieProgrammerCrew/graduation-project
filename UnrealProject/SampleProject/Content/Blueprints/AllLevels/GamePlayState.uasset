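; GamePlayState is a game state Blueprint that decides round outcome in a killer-versus-players match.
; CheckPlayerDie scans PlayerArray as PlayerStateBP, stopping if the killer is dead and otherwise counting dead non-killers.
; When that count equals the array's last index, KillerWinVDPlay shows the WBP_KillerWin widget and mouse cursor.
; The player-win branch only prints a debug string.
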(event Custom|CheckPlayerDie
  (bind _playerarray (Variables|Default|GetPlayerArray))
  (bind _array_element (Utilities|Array|ForEachLoopwithBreak _playerarray :!label _label)
    (:LoopBody
      (if (Variables|/Game/Blueprints/AllLevels/PlayerStateBP.PlayerStateBP_C|GetIsKiller? (.AsPlayer%20State%20BP (Utilities|Casting|CastToPlayerStateBP _array_element)))
        (if (Variables|/Game/Blueprints/AllLevels/PlayerStateBP.PlayerStateBP_C|GetKillerDie? (.AsPlayer%20State%20BP (Utilities|Casting|CastToPlayerStateBP _array_element)))
          (Variables|Default|Setplayer false)
          (goto _label Break))
        (elif (Variables|/Game/Blueprints/AllLevels/PlayerStateBP.PlayerStateBP_C|GetDie? (.AsPlayer%20State%20BP (Utilities|Casting|CastToPlayerStateBP _array_element)))
          (Math|Integer|IncrementInt (Variables|Default|Getcount)
            (:%20%20
              (Variables|Default|Setplayer true))))))
    (:Completed
      (if (Variables|Default|Getplayer)
        (if (== (Utilities|Array|LastIndex _playerarray) (Variables|Default|Getcount))
          (CallFunction|KillerWinVDPlay)
          (else
            (Variables|Default|Setcount 0)))
        (else
          (Development|PrintString "PlayerWin"))))))

(event Custom|KillerWinVDPlay
  (bind _returnvalue (UserInterface|CreateWidget "/Game/Blueprints/Widget/WBP_KillerWin.WBP_KillerWin_C"))
  (UserInterface|Viewport|AddtoViewport _returnvalue 0)
  (Variables|/Script/Engine.PlayerController|SetbShowMouseCursor (Game|GetPlayerController 0) true))

(event EventBeginPlay)

(fn ConstructionScript)