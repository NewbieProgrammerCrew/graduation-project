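; BP_L_Louis is the playable Louis survivor character for the lobby, providing basic look and movement control.
; BeginPlay adds the IMC_Survivor Enhanced Input context and clamps camera pitch.
; Rotate input drives controller yaw and pitch, while movement input follows control rotation with pitch zeroed for forward and right directions.
; Interact, MissionResult, RepairState and ReturnItemInfo are empty stubs returning nothing or false.
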(event Input|EnhancedActionEvents|EnhancedInputActionIA_SurvivorRotate
  (params (ActionValue :type Vector%202D%20Structure) (ElapsedSeconds :type Float%20%28double-precision%29) (TriggeredSeconds :type Float%20%28double-precision%29) (InputAction :type Input%20Action%20Object%20Reference :default "/Game/Blueprints/Input/Survivor/IA_SurvivorRotate.IA_SurvivorRotate"))
  ;[0 1 0.3718] Player Control
  (:Triggered
    (Pawn|Input|AddControllerYawInput (.x ActionValue))
    (Pawn|Input|AddControllerPitchInput (.y ActionValue))))

(event Input|EnhancedActionEvents|EnhancedInputActionIA_SurvivorMovement
  (params (ActionValue :type Vector%202D%20Structure) (ElapsedSeconds :type Float%20%28double-precision%29) (TriggeredSeconds :type Float%20%28double-precision%29) (InputAction :type Input%20Action%20Object%20Reference :default "/Game/Blueprints/Input/Survivor/IA_SurvivorMovement.IA_SurvivorMovement"))
  (bind _returnvalue (Pawn|GetControlRotation :!class /Script/Engine.Pawn))
  ;[0 1 0.3718] Player Control
  (:Triggered
    ;;[1 0 0.1904] WOW movement
    (Pawn|Input|AddMovementInput (Math|Vector|GetForwardVector (Math|Rotator|MakeRotator (.roll _returnvalue) 0.0 (.yaw _returnvalue))) (.y ActionValue) false)
    (Pawn|Input|AddMovementInput (Math|Vector|GetRightVector (Math|Rotator|MakeRotator (.roll _returnvalue) 0.0 (.yaw _returnvalue))) (.x ActionValue) false)))

(event Collision|EventActorBeginOverlap
  (params (OtherActor :type Actor%20Object%20Reference)))

(event EventBeginPlay
  (bind _returnvalue (Game|GetPlayerController 0))
  (bind _returnvalue_2 (Game|GetPlayerCameraManager 0))
  (Utilities|IsValid _returnvalue
    (:Is%20Valid
      (Input|AddMappingContext (PlayerController|LocalPlayerSubsystems|GetEnhancedInputLocalPlayerSubsystem _returnvalue) "/Game/Blueprints/Input/Survivor/IMC_Survivor.IMC_Survivor" 0 "(bIgnoreAllPressedKeysUntilRelease=True,bForceImmediately=False)")
      (Variables|/Script/Engine.PlayerCameraManager|SetViewPitchMin _returnvalue_2 -4e+01)
      (Variables|/Script/Engine.PlayerCameraManager|SetViewPitchMax _returnvalue_2 4e+01))))

(fn ConstructionScript)

(fn Interact
  (params (player :type BP%20Parent%20Object%20Reference))
  (return))

(fn MissionResult
  (return false))

(fn RepairState
  (return false))

(fn ReturnItemInfo
  (return ""))