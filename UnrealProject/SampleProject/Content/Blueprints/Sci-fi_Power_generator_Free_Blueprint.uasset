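; Repairable sci-fi power generator actor that tracks whether its repair is complete.
; On the server, a BP_Ch1 character entering its Bound volume is shown a progress bar while repair is incomplete, hidden again on exit.
; Clearing the repair on the server sets RepairComplete, exposed through RepairState, and recolours the mesh's state material blue via a dynamic instance.
; The server cancel handler is empty.
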(event OnComponentBeginOverlap(Bound)
  (params (OverlappedComponent :type Primitive%20Component%20Object%20Reference) (OtherActor :type Actor%20Object%20Reference) (OtherComp :type Primitive%20Component%20Object%20Reference) (OtherBodyIndex :type Integer) (bFromSweep :type Boolean) (SweepResult :type Hit%20Result%20Structure%20%28by%20ref%29))
  ;[1 0.5 0.5] Player Overlap
  (Networking|SwitchHasAuthority
    (:Authority
      (bind _asbp_ch_1 (Utilities|Casting|CastToBP_Ch1 OtherActor))
      (if (not (Variables|Default|GetRepairComplete))
        (Default|PBarVisibility _asbp_ch_1 self)))))

(event OnComponentEndOverlap(Bound)
  (params (OverlappedComponent :type Primitive%20Component%20Object%20Reference) (OtherActor :type Actor%20Object%20Reference) (OtherComp :type Primitive%20Component%20Object%20Reference) (OtherBodyIndex :type Integer))
  ;[1 0.5 0.5] Player Overlap
  (Networking|SwitchHasAuthority
    (:Authority
      (bind _asbp_ch_1 (Utilities|Casting|CastToBP_Ch1 OtherActor))
      (Default|PBarHidden _asbp_ch_1))))

(event Custom|ClearRepair
  ;[1 0.375 0.375] Repairing Bool
  (CallFunction|ServerClearRepair))

(event Custom|CancleRepair
  ;[1 0.375 0.375] Repairing Bool
  (CallFunction|ServerCancleRepair))

(event Custom|Server_ClearRepair
  ;[1 0.375 0.375] Repairing Bool
  (Variables|Default|SetRepairComplete true)
  (bind _returnvalue (Rendering|Material|CreateDynamicMaterialInstance (Variables|Debug|GetStaticMeshComponent) 3 "/Game/PowerGenerator/MI_STATE.MI_STATE" "None" :!class /Script/Engine.PrimitiveComponent))
  (Rendering|Material|SetVectorParameterValue _returnvalue "Color" "(R=0.000000,G=0.125763,B=0.552083,A=1.000000)" :!class /Script/Engine.MaterialInstanceDynamic))

(event Custom|Server_CancleRepair
  ;[1 0.375 0.375] Repairing Bool
)

(event EventBeginPlay)

(event Collision|EventActorBeginOverlap
  (params (OtherActor :type Actor%20Object%20Reference)))

(event EventTick
  (params (DeltaSeconds :type Float%20%28single-precision%29)))

(fn ConstructionScript)

(fn RepairState
  (return (Variables|Default|GetRepairComplete)))