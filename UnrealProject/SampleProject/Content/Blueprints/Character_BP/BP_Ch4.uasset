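; BP_Ch4 is a character Blueprint that supplies networked animations for aiming, shooting and slashing, using Alex montages.
; Overrides of the play and stop animation functions call server RPC events, which relay to RPC events that play or stop the montages.
; Aim and shoot use sections of one fire montage, which stopping aim halts.
; DoOnce gates block aim and slash retriggers until their montage completes or is interrupted.
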(event Custom|Server_RPC_Aim_Animation
  (CallFunction|RPCAimAnim))

(event Custom|RPC_Aim_Anim
  (Utilities|FlowControl|DoOnce false :!label _label
    (:Completed
      (Animation|Montage|PlayMontage (Variables|Character|GetMesh) "/Game/Characters/Animation/RifleAnim/MTG_Alex_Fire.MTG_Alex_Fire" 1.0 0.0 "Aim"
        (:OnCompleted
          (goto _label Reset))
        (:OnInterrupted
          (goto _label Reset))))))

(event Custom|RPC_NonAim_Animation
  (Animation|StopAnimMontage "/Game/Characters/Animation/RifleAnim/MTG_Alex_Fire.MTG_Alex_Fire"))

(event Custom|Server_RPC_NonAim_Animation
  (CallFunction|RPCNonAimAnimation))

(event Custom|RPC_Server_Shoot
  (CallFunction|RPCShoot))

(event Custom|RPC_Shoot
  (Animation|PlayAnimMontage "/Game/Characters/Animation/RifleAnim/MTG_Alex_Fire.MTG_Alex_Fire" 1.0 "Fire"))

(event Custom|Server_RPC_SlashAnim
  (CallFunction|RPCSlashAnim))

(event Custom|RPC_SlashAnim
  (Utilities|FlowControl|DoOnce false :!label _label
    (:Completed
      (Animation|Montage|PlayMontage (Variables|Character|GetMesh) "/Game/Characters/Animation/Sword/MTG_AlexSlash.MTG_AlexSlash"
        (:OnCompleted
          (goto _label Reset))
        (:OnInterrupted
          (goto _label Reset))))))

(event EventBeginPlay
  (|CallParentFunction) ; This node is disabled and will not be called.\nDrag off pins to build functionality.
)

(event Collision|EventActorBeginOverlap
  (params (OtherActor :type Actor%20Object%20Reference))
  (|CallParentFunction OtherActor) ; This node is disabled and will not be called.\nDrag off pins to build functionality.
)

(event EventTick
  (params (DeltaSeconds :type Float%20%28single-precision%29))
  (|CallParentFunction DeltaSeconds) ; This node is disabled and will not be called.\nDrag off pins to build functionality.
)

(fn ConstructionScript
  (|CallParentFunction))

(fn PlayAimAnim
  (CallFunction|ServerRPCAimAnimation))

(fn PlayShootAnim
  (CallFunction|RPCServerShoot))

(fn PlaySlashAnim
  (CallFunction|ServerRPCSlashAnim))

(fn StopAimAnim
  (CallFunction|ServerRPCNonAimAnimation))