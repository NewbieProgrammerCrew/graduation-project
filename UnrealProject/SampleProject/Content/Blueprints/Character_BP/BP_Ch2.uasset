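; BP_Ch2 is a child character Blueprint that plays the Louis character's aim, shoot and sword slash animations through RPC-named events.
; Play and stop functions call Server_RPC events, which relay to RPC events that start or stop the fire and slash montages.
; DoOnce gates block restarting aim or slash until the montage completes or is interrupted.
; SwordColEnable and SwordColDisable are empty, with their collision logic left disconnected.
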(event Custom|Server_RPC_AimAnim
  (CallFunction|RPCAimAnim))

(event Custom|RPC_AimAnim
  (Utilities|FlowControl|DoOnce false :!label _label
    (:Completed
      (Animation|Montage|PlayMontage (Variables|Character|GetMesh) "/Game/Characters/Animation/RifleAnim/MTG_Louis_Fire.MTG_Louis_Fire" 1.0 0.0 "Aim"
        (:OnCompleted
          (goto _label Reset))
        (:OnInterrupted
          (goto _label Reset))))))

(event Custom|Server_RPC_NonAimAnim
  (CallFunction|RPCNonAimAnim))

(event Custom|RPC_NonAimAnim
  (Animation|StopAnimMontage "/Game/Characters/Animation/RifleAnim/MTG_Louis_Fire.MTG_Louis_Fire"))

(event Custom|Server_RPC_SlashAnim
  (CallFunction|RPCSlashAnim))

(event Custom|RPC_SlashAnim
  (Utilities|FlowControl|DoOnce false :!label _label
    (:Completed
      (Animation|Montage|PlayMontage (Variables|Character|GetMesh) "/Game/Characters/Animation/Sword/MTG_LouisSlash.MTG_LouisSlash"
        (:OnCompleted
          (goto _label Reset))
        (:OnInterrupted
          (goto _label Reset))))))

(event Custom|Server_RPC_StopSlashAnim
  (CallFunction|RPCStopSlashAnim))

(event Custom|RPC_StopSlashAnim
  (Animation|StopAnimMontage "/Game/Characters/Animation/Sword/MTG_LouisSlash.MTG_LouisSlash"))

(event Custom|Server_RPC_ShootAnim
  (CallFunction|RPCShootAnim))

(event Custom|RPC_ShootAnim
  (Animation|PlayAnimMontage "/Game/Characters/Animation/RifleAnim/MTG_Louis_Fire.MTG_Louis_Fire" 1.0 "Fire"))

(event EventBeginPlay
  (|CallParentFunction))

(event Collision|EventActorBeginOverlap
  (params (OtherActor :type Actor%20Object%20Reference))
  (|CallParentFunction OtherActor) ; This node is disabled and will not be called.\nDrag off pins to build functionality.
)

(event EventTick
  (params (DeltaSeconds :type Float%20%28single-precision%29))
  (|CallParentFunction DeltaSeconds) ; This node is disabled and will not be called.\nDrag off pins to build functionality.
)

(fn ConstructionScript
  (|CallParentFunction))

(fn PlayAimAnim
  (CallFunction|ServerRPCAimAnim))

(fn StopAimAnim
  (CallFunction|ServerRPCNonAimAnim))

(fn PlaySlashAnim
  (CallFunction|ServerRPCSlashAnim))

(fn StopSlashAnim
  (CallFunction|ServerRPCStopSlashAnim))

(fn PlayShootAnim
  (CallFunction|ServerRPCShootAnim))

(fn SwordColEnable)

(fn SwordColDisable)