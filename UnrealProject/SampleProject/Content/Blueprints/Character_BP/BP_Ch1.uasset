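; Survivor player character that moves with Enhanced Input and repairs sci-fi power generators.
; PBarVisibility stores a generator and shows a fix-it prompt on the WBP_Mission widget; left click locks movement, right click cancels.
; While locked, Tick calls a server RPC chained to an update RPC that, while left mouse is held, advances generator progress and the bar, or changes its color once complete.
; Look input drives yaw only.
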(event Custom|PBarVisibility
  (params (generator :type Actor%20Object%20Reference))
  ;[0 1 0.5887] UIVisibility
  (Variables|Default|SetGenerator generator)
  (CallFunction|ShowLeftMouseLOGO)
  (Variables|Default|SetSelectAvailable true))

(event Custom|PBarHidden
  ;[0 1 0.5887] UIVisibility
  (CallFunction|HideLeftMouseLOGO)
  (CallFunction|HideProgressBar)
  (Variables|Default|SetSelectAvailable false)
  (Variables|Default|SetLock false))

(event Custom|RPC_Server_UpdateProgressBar
  (CallFunction|RPCUpdateProgressBar))

(event Custom|RPC_UpdateProgressBar
  (if (Variables|Default|GetLHold)
    (Utilities|IsValid (Variables|Default|GetGenerator)
      (:Is%20Valid
        (bind _assci_fi_power_generator_free_blueprint (Utilities|Casting|CastToSci-fi_Power_generator_Free_Blueprint (Variables|Default|GetGenerator)))
        (if (Variables|/Game/Characters/Sci-fi_Power_generator_Free_Blueprint.Sci-fi_Power_generator_Free_Blueprint_C|GetRepairComplete _assci_fi_power_generator_free_blueprint)
          (Default|RPCChangeColor _assci_fi_power_generator_free_blueprint)
          (else
            (bind _output_get (Variables|/Game/Characters/Sci-fi_Power_generator_Free_Blueprint.Sci-fi_Power_generator_Free_Blueprint_C|SetRepairProgress _assci_fi_power_generator_free_blueprint (+ (Variables|/Game/Characters/Sci-fi_Power_generator_Free_Blueprint.Sci-fi_Power_generator_Free_Blueprint_C|GetRepairProgress _assci_fi_power_generator_free_blueprint) (* (Variables|/Game/Characters/Sci-fi_Power_generator_Free_Blueprint.Sci-fi_Power_generator_Free_Blueprint_C|GetRepairSpeed _assci_fi_power_generator_free_blueprint) (Utilities|Time|GetWorldDeltaSeconds)))))
            (Progress|SetPercent (Variables|/Game/Blueprints/Widget/WBP_Mission.WBP_Mission_C|GetProgressBar_0 (Variables|Default|GetProgressWidget)) _output_get)))))))

(event Input|EnhancedActionEvents|EnhancedInputActionIA_SurvivorRotate
  (params (ActionValue :type Vector%202D%20Structure) (ElapsedSeconds :type Float%20%28double-precision%29) (TriggeredSeconds :type Float%20%28double-precision%29) (InputAction :type Input%20Action%20Object%20Reference :default "/Game/Blueprints/Input/Survivor/IA_SurvivorRotate.IA_SurvivorRotate"))
  (:Triggered
    (Pawn|Input|AddControllerYawInput (.x ActionValue))
    (Pawn|Input|AddControllerPitchInput (* 0.0 -1.0))))

(event Input|EnhancedActionEvents|EnhancedInputActionIA_SurvivorMovement
  (params (ActionValue :type Vector%202D%20Structure) (ElapsedSeconds :type Float%20%28double-precision%29) (TriggeredSeconds :type Float%20%28double-precision%29) (InputAction :type Input%20Action%20Object%20Reference :default "/Game/Blueprints/Input/Survivor/IA_SurvivorMovement.IA_SurvivorMovement"))
  (bind _returnvalue (Pawn|GetControlRotation :!class /Script/Engine.Pawn))
  (:Triggered
    ;[0.5512 0.8369 1] WOW movement
    (if (not (Variables|Default|GetLock))
      (Pawn|Input|AddMovementInput (Math|Vector|GetForwardVector (Math|Rotator|MakeRotator (.roll _returnvalue) 0.0 (.yaw _returnvalue))) (.y ActionValue) false)
      (Pawn|Input|AddMovementInput (Math|Vector|GetRightVector (Math|Rotator|MakeRotator (.roll _returnvalue) 0.0 (.yaw _returnvalue))) (.x ActionValue) false))))

(event EventBeginPlay
  (bind _asplayer_controller (Utilities|Casting|CastToPlayerController (Pawn|GetController)))
  (Utilities|IsValid (PlayerController|LocalPlayerSubsystems|GetEnhancedInputLocalPlayerSubsystem _asplayer_controller)
    (:Is%20Valid
      (Input|AddMappingContext (PlayerController|LocalPlayerSubsystems|GetEnhancedInputLocalPlayerSubsystem _asplayer_controller) "/Game/Blueprints/Input/Survivor/IMC_Survivor.IMC_Survivor" 0 "(bIgnoreAllPressedKeysUntilRelease=True,bForceImmediately=False)")
      (bind _returnvalue (UserInterface|CreateWidget "/Game/Blueprints/Widget/WBP_Mission.WBP_Mission_C" 0 self))
      (bind _output_get (Variables|Default|SetProgressWidget _returnvalue))
      (UserInterface|Viewport|AddtoViewport _output_get 0))))

(event Collision|EventActorBeginOverlap
  (params (OtherActor :type Actor%20Object%20Reference)))

(event EventTick
  (params (DeltaSeconds :type Float%20%28single-precision%29))
  (if (Variables|Default|GetLock)
    (Utilities|IsValid (Variables|Default|GetGenerator)
      (:Is%20Valid
        (CallFunction|RPCServerUpdateProgressBar)))))

(event Input|MouseEvents|LeftMouseButton
  (params (Key :type Key%20Structure :default "None"))
  (:Pressed
    (if (Variables|Default|GetSelectAvailable)
      (Variables|Default|SetLock true)
      (if (Widget|IsVisible (Variables|/Game/Blueprints/Widget/WBP_Mission.WBP_Mission_C|GetProgressBar_0 (Variables|Default|GetProgressWidget)))
        (Variables|Default|SetLHold true)
        (else
          (CallFunction|ShowProgressBar)
          (CallFunction|HideLeftMouseLOGO)
          (Variables|Default|SetLHold true)))
      (else
        (CallFunction|HideProgressBar))))
  (:Released
    (Variables|Default|SetLHold false)))

(event Input|MouseEvents|RightMouseButton
  (params (Key :type Key%20Structure :default "None"))
  (:Pressed
    (if (Variables|Default|GetSelectAvailable)
      (Variables|Default|SetLock false)
      (CallFunction|ShowLeftMouseLOGO)
      (CallFunction|HideProgressBar)
      (Variables|Default|SetSelectAvailable true)
      (Variables|Default|SetLHold false))))

(fn ConstructionScript)

(fn HideLeftMouseLOGO
  (Widget|SetVisibility (Variables|/Game/Blueprints/Widget/WBP_Mission.WBP_Mission_C|GetFixitText (Variables|Default|GetProgressWidget)) "Hidden"))

(fn HideProgressBar
  (Widget|SetVisibility (Variables|/Game/Blueprints/Widget/WBP_Mission.WBP_Mission_C|GetProgressBar_0 (Variables|Default|GetProgressWidget)) "Hidden"))

(fn ShowProgressBar
  (Widget|SetVisibility (Variables|/Game/Blueprints/Widget/WBP_Mission.WBP_Mission_C|GetProgressBar_0 (Variables|Default|GetProgressWidget)) "Visible"))

(fn ShowLeftMouseLOGO
  (Widget|SetVisibility (Variables|/Game/Blueprints/Widget/WBP_Mission.WBP_Mission_C|GetFixitText (Variables|Default|GetProgressWidget)) "Visible")
  (Variables|Default|SetSelectAvailable true))