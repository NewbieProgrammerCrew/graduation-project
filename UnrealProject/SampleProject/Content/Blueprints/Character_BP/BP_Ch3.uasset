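; BP_Ch3 is a child character Blueprint that supplies Megan's aim, fire and slash montages.
; It overrides the parent's animation functions to call Server-prefixed events, which relay to RPC events that play or stop the montages, a pattern named for network replication.
; DoOnce gates keep aim and slash from restarting until their montage completes or is interrupted.
; The sword collision enable and disable functions do nothing, as their hitbox logic is disconnected.
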(event Custom|Server_Play_RPC_AimAnim
  (CallFunction|RPCPlayAimAnim))

(event Custom|RPC_Play_AimAnim
  (Utilities|FlowControl|DoOnce false :!label _label
    (:Completed
      (Animation|Montage|PlayMontage (Variables|Character|GetMesh) "/Game/Characters/Animation/RifleAnim/MTG_Megan_Fire.MTG_Megan_Fire" 1.0 0.0 "Aim"
        (:OnCompleted
          (goto _label Reset))
        (:OnInterrupted
          (goto _label Reset))))))

(event Custom|Server_RPC_Stop_AimAnim
  (CallFunction|RPCStopAimAnim))

(event Custom|RPC_Stop_AimAnim
  (Animation|StopAnimMontage "/Game/Characters/Animation/RifleAnim/MTG_Megan_Fire.MTG_Megan_Fire"))

(event Custom|Server_RPC_ShootAnim
  (CallFunction|RPCShootAnim))

(event Custom|RPC_ShootAnim
  (Animation|PlayAnimMontage "/Game/Characters/Animation/RifleAnim/MTG_Megan_Fire.MTG_Megan_Fire" 1.0 "Fire"))

(event Custom|Server_RPC_SlashAnim
  (CallFunction|RPCSlashAnim))

(event Custom|RPC_SlashAnim
  (Utilities|FlowControl|DoOnce false :!label _label
    (:Completed
      (Animation|Montage|PlayMontage (Variables|Character|GetMesh) "/Game/Characters/Animation/Sword/MTG_MeganSlash.MTG_MeganSlash"
        (:OnCompleted
          (goto _label Reset))
        (:OnInterrupted
          (goto _label Reset))))))

(event EventBeginPlay
  (|CallParentFunction))

(event Collision|EventActorBeginOverlap
  (params (OtherActor :type Actor%20Object%20Reference))
  (|CallParentFunction OtherActor) ; This node is disabled and will not be called.\nDrag off pins to build functionality.
)

(event EventTick
  (params (DeltaSeconds :type Float%20%28single-precision%29))
  (|CallParentFunction DeltaSeconds) ; This node is disabled and will not be called.\nDrag off pins to build functionality.
)

(fn ConstructionScript
  (|CallParentFunction))

(fn PlayAimAnim
  (CallFunction|ServerPlayRPCAimAnim))

(fn StopAimAnim
  (CallFunction|ServerRPCStopAimAnim))

(fn PlayShootAnim
  (CallFunction|ServerRPCShootAnim))

(fn PlaySlashAnim
  (CallFunction|ServerRPCSlashAnim))

(fn SwordColDisable)

(fn SwordColEnable)