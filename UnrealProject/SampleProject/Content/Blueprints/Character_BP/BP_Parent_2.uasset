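; Parent Blueprint for survivor player characters, handling movement, inventory selection, rifle and sword combat, and chest repair missions.
; Equipped items attach to a weapon socket via RPCs and set the combat mode Tick applies, switching camera, aiming and hitscan shooting.
; Clicking at a chest opens a random mission widget and locks movement until Tick sees success or right-click cancels.
; Animation functions are empty stubs, apparently for child classes.
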(event Custom|UI%20INFO
  (params (generator :type Actor%20Object%20Reference))
  ;[0 1 0.5887] UIVisibility
  (CallFunction|SetChest generator)
  (task|ShowLeftMouseLOGO generator)
  (Variables|task|SetSelectAvailable true))

(event Custom|PBarHidden
  ;[0 1 0.5887] UIVisibility
  (task|HideLeftMouseLOGO)
  (task|HideProgressBar)
  (Variables|task|SetSelectAvailable false)
  (Variables|task|SetLock false))

(event Custom|RPC_Destroy%20Item
  ;[0.07432 0.2141 1] Detach Equipment
  (Utilities|IsValid (Variables|item|GetEquipItem)
    (:Is%20Valid
      (Transformation|DetachFromActor (Variables|item|GetEquipItem) "KeepWorld" "KeepWorld" "KeepWorld")
      (Actor|DestroyActor (Variables|item|GetEquipItem))
      (Variables|item|SetEquipItem 0))))

(event Custom|Server_RPC_UpdateRotator
  (params (rotator :type Rotator))
  ;[1 0 0.3547] Server_UpdateRotation
  (Transformation|SetActorRotation (Math|Rotator|MakeRotator (.roll rotator) 0.0 (.yaw rotator))))

(event Custom|Server_RPC_Equip
  (params (result :type Boolean) (result2 :type Boolean))
  (Variables|Attack|SetRifle? result)
  (Variables|Attack|SetBrret? result2))

(event Custom|Cancel%20Mission
  ;[0.4366 0.9701 1] Chest Event On Server
  (Utilities|IsValid (Variables|task|GetChest)
    (:Is%20Valid
      (bind _asbp_chest (Utilities|Casting|CastToBP_Chest (Variables|task|GetChest)))
      (Default|CancleRepair _asbp_chest))
    (:Is%20Not%20Valid
      (Development|PrintString "Gener is None"))))

(event Custom|Clear%20Mission
  ;[0.4366 0.9701 1] Chest Event On Server
  (Utilities|IsValid (Variables|task|GetChest)
    (:Is%20Valid
      (bind _asbp_chest (Utilities|Casting|CastToBP_Chest (Variables|task|GetChest)))
      (Default|ClearRepair _asbp_chest))
    (:Is%20Not%20Valid
      (Development|PrintString "Gener is None"))))

(event Custom|Set%20Chest
  (params (generator :type Actor%20Object%20Reference))
  ;[0 1 0.5887] UIVisibility
  (Variables|task|SetChest generator))

(event Custom|RPC_Server_Equipment
  ;[0.1583 0.4888 1] Equip Equipment
  (CallFunction|RPCEquipment))

(event Custom|RPC_Equipment
  (bind _cpy_item_info (Variables|item|GetCpy%20Item%20INFO))
  ;[0.1583 0.4888 1] Equip Equipment
  (Networking|SwitchHasAuthority
    (:Authority
      (bind _returnvalue (Game|SpawnActorfromClass (.itemclass (Variables|item|GetCpy%20Item%20INFO)) (Math|Transform|MakeTransform (Transformation|GetWorldLocation (Variables|Character|GetMesh)) "0, 0, 0" "1.000000,1.000000,1.000000") "Undefined" 0 0))
      (Utilities|IsValid _returnvalue
        (:Is%20Valid
          (bind _output_get (Variables|item|SetEquipItem _returnvalue))
          (Transformation|AttachComponentToComponent _output_get (Variables|Character|GetMesh) "Weapon" "SnapToTarget" "SnapToTarget" "SnapToTarget" true)
          (Variables|Attack|Setequip? true)
          (CallFunction|ServerRPCEquip (Utilities|Enum|Equal(Enum) (.itemtype _cpy_item_info) "NewEnumerator0") (Utilities|Enum|Equal(Enum) (.itemtype _cpy_item_info) "NewEnumerator1"))
          (Attack|StopAimAnim)
          (Attack|StopSlashAnim))))))

(event Custom|RPC_Server_destroy%20Item
  ;[0.07432 0.2141 1] Detach Equipment
  (CallFunction|RPCDestroyItem)
  (Variables|Attack|Setequip? false)
  (Variables|Attack|SetRifle? false)
  (Variables|Attack|SetBrret? false))

(event Input|EnhancedActionEvents|EnhancedInputActionIA_SurvivorRotate
  (params (ActionValue :type Vector%202D%20Structure) (ElapsedSeconds :type Float%20%28double-precision%29) (TriggeredSeconds :type Float%20%28double-precision%29) (InputAction :type Input%20Action%20Object%20Reference :default "/Game/Blueprints/Input/Survivor/IA_SurvivorRotate.IA_SurvivorRotate"))
  ;[0 1 0.3718] Player Control
  (:Triggered
    (Pawn|Input|AddControllerYawInput (.x ActionValue))
    (Pawn|Input|AddControllerPitchInput (.y ActionValue))))

(event Input|EnhancedActionEvents|EnhancedInputActionIA_SurvivorMovement
  (params (ActionValue :type Vector%202D%20Structure) (ElapsedSeconds :type Float%20%28double-precision%29) (TriggeredSeconds :type Float%20%28double-precision%29) (InputAction :type Input%20Action%20Object%20Reference :default "/Game/Blueprints/Input/Survivor/IA_SurvivorMovement.IA_SurvivorMovement"))
  (bind _returnvalue (Pawn|GetControlRotation :!class /Script/Engine.Pawn))
  ;[0 1 0.3718] Player Control
  (:Triggered
    ;;[1 0 0.1904] WOW movement
    (if (not (Variables|task|GetLock))
      (Pawn|Input|AddMovementInput (Math|Vector|GetForwardVector (Math|Rotator|MakeRotator (.roll _returnvalue) 0.0 (.yaw _returnvalue))) (.y ActionValue) false)
      (Pawn|Input|AddMovementInput (Math|Vector|GetRightVector (Math|Rotator|MakeRotator (.roll _returnvalue) 0.0 (.yaw _returnvalue))) (.x ActionValue) false))))

(event Collision|EventActorBeginOverlap
  (params (OtherActor :type Actor%20Object%20Reference)))

(event EventTick
  (params (DeltaSeconds :type Float%20%28single-precision%29))
  (bind _missionwidget (Variables|task|GetMissionWidget))
  (bind _missionwidget_2 (Variables|task|GetMissionWidget))
  ;[0.1377 0.1279 1] Judge Mission result
  (if (Variables|task|GetLock)
    (task|UpdateProgress)
    (Utilities|IsValid _missionwidget
      (:Is%20Valid
        (if (Utilities|Array|Get(acopy) (Variables|task|GetaddViewport?) (Variables|Widget|GetWidgetIndex))
          (bind _result (Class|BPIMissionClear|MissionResult(Message) _missionwidget))
          (if _result
            (Class|BPIMissionClear|RemoveMission(Message) _missionwidget_2 _missionwidget_2)
            (CallFunction|ClearMission)
            (Utilities|Array|SetArrayElem (Variables|task|GetaddViewport?) (Variables|Widget|GetWidgetIndex) false)
            (task|DeactivateCusor)
            (task|HideLeftMouseLOGO)
            (Variables|task|SetLHold false)))))
    (elif (Variables|Attack|GetRifle?)
      (Attack|SetRifleMode?)
      (if (Variables|Attack|GetAiming)
        (Attack|PlayAimAnim))
      (elif (Variables|Attack|GetBrret?)
        (Attack|SetSwordMode?)
        (else
          (Attack|NoneAimMode))))))

(event EventBeginPlay
  (bind _returnvalue (Game|GetPlayerController 0))
  (bind _returnvalue_2 (Game|GetPlayerCameraManager 0))
  (Variables|Character|SetCurHP (Variables|Character|GetFullHP))
  (Utilities|IsValid _returnvalue
    (:Is%20Valid
      (Input|AddMappingContext (PlayerController|LocalPlayerSubsystems|GetEnhancedInputLocalPlayerSubsystem _returnvalue) "/Game/Blueprints/Input/Survivor/IMC_Survivor.IMC_Survivor" 0 "(bIgnoreAllPressedKeysUntilRelease=True,bForceImmediately=False)")
      (Variables|/Script/Engine.PlayerCameraManager|SetViewPitchMin _returnvalue_2 -4e+01)
      (Variables|/Script/Engine.PlayerCameraManager|SetViewPitchMax _returnvalue_2 4e+01))))

(event Input|MouseEvents|LeftMouseButton
  (params (Key :type Key%20Structure :default "None"))
  (bind _missionwc (Variables|task|GetMissionWC))
  (bind _chest (Variables|task|GetChest))
  (bind (_outitem _outindex) (Utilities|Array|Random _missionwc))
  ;[0 0.3382 0.7344] ATK/Open Chest(task)
  (:Pressed
    (if (Variables|Attack|GetSlashAvailable)
      (Attack|PlaySlashAnim)
      (else
        (Attack|StopSlashAnim)
        (Variables|Attack|SetSlashAvailable false)
        (if (Variables|Attack|GetShootable)
          (Attack|Shoot)
          (Variables|Attack|Setfire true)
          (else
            (Variables|Attack|Setfire false)))))
    (Utilities|IsValid _chest
      (:Is%20Valid
        (bind _asbp_chest (Utilities|Casting|CastToBP_Chest _chest))
        (bind _result (Default|RepairState _asbp_chest))
        (if (not _result)
          (if (Variables|task|GetSelectAvailable)
            (if (not (Variables|task|GetLHold))
              (Variables|task|SetLock true)
              (Variables|task|SetLHold true)
              (Variables|Widget|SetWidgetIndex _outindex)
              (bind _returnvalue (UserInterface|CreateWidget _outitem))
              (bind _output_get (Variables|task|SetMissionWidget _returnvalue))
              (UserInterface|Viewport|AddtoViewport _output_get 0)
              (Utilities|Array|SetArrayElem (Variables|task|GetaddViewport?) (Variables|Widget|GetWidgetIndex) true)
              (task|ActivateCusor))
            (else
              (task|HideProgressBar)))))))
  (:Released
    (Variables|Attack|Setfire false)
    (Variables|Attack|SetSlashAvailable false)))

(event Input|MouseEvents|RightMouseButton
  (params (Key :type Key%20Structure :default "None"))
  (bind _missionwidget (Variables|task|GetMissionWidget))
  (bind _chest (Variables|task|GetChest))
  ;[0 0.3382 0.7344] ATK/Open Chest(task)
  (:Pressed
    (if (Variables|task|GetSelectAvailable)
      (Variables|task|SetLHold false)
      (Variables|task|SetLock false)
      (task|ShowLeftMouseLOGO)
      (task|HideProgressBar)
      (Variables|task|SetSelectAvailable true)
      (Variables|task|SetLHold false)
      (if (Utilities|Array|Get(acopy) (Variables|task|GetaddViewport?) (Variables|Widget|GetWidgetIndex))
        (Class|BPIMissionClear|RemoveMission(Message) _missionwidget _missionwidget)
        (Utilities|Array|SetArrayElem (Variables|task|GetaddViewport?) (Variables|Widget|GetWidgetIndex) false)
        (Utilities|IsValid _chest
          (:Is%20Valid
            (bind _asbp_chest (Utilities|Casting|CastToBP_Chest _chest))
            (bind _result (Default|RepairState _asbp_chest))
            (if (not _result)
              (task|ShowLeftMouseLOGO _asbp_chest)
              (task|DeactivateCusor))))))))

(event Input|MouseEvents|RightMouseButton
  (params (Key :type Key%20Structure :default "None"))
  (:Pressed
    (Variables|Attack|SetAiming true))
  (:Released
    (Variables|Attack|SetAiming false)
    (Attack|StopAimAnim)))

(event Input|KeyboardEvents|1
  (params (Key :type Key%20Structure :default "None"))
  ;[1 0.8669 0] Select Item in Inventory
  (:Pressed
    (Variables|item|Setindex 1)
    (Default|SelectItem (Variables|Widget|GetInfoWidget) (Variables|item|Getindex) self)))

(event Input|KeyboardEvents|2
  (params (Key :type Key%20Structure :default "None"))
  ;[1 0.8669 0] Select Item in Inventory
  (:Pressed
    (Variables|item|Setindex 2)
    (Default|SelectItem (Variables|Widget|GetInfoWidget) (Variables|item|Getindex) self)))

(event Input|KeyboardEvents|3
  (params (Key :type Key%20Structure :default "None"))
  ;[1 0.8669 0] Select Item in Inventory
  (:Pressed
    (Variables|item|Setindex 3)
    (Default|SelectItem (Variables|Widget|GetInfoWidget) (Variables|item|Getindex) self)))

(event Input|KeyboardEvents|4
  (params (Key :type Key%20Structure :default "None"))
  ;[1 0.8669 0] Select Item in Inventory
  (:Pressed
    (Variables|item|Setindex 4)
    (Default|SelectItem (Variables|Widget|GetInfoWidget) (Variables|item|Getindex) self)))

(event Input|KeyboardEvents|5
  (params (Key :type Key%20Structure :default "None"))
  ;[1 0.8669 0] Select Item in Inventory
  (:Pressed
    (Variables|item|Setindex 5)
    (Default|SelectItem (Variables|Widget|GetInfoWidget) (Variables|item|Getindex) self)))

(event Input|KeyboardEvents|6
  (params (Key :type Key%20Structure :default "None"))
  ;[1 0.8669 0] Select Item in Inventory
  (:Pressed
    (Variables|item|Setindex 6)
    (Default|SelectItem (Variables|Widget|GetInfoWidget) (Variables|item|Getindex) self)))

(fn ConstructionScript)

(fn HideLeftMouseLOGO
  (Widget|SetVisibility (Variables|/Game/Blueprints/Widget/WBP_INFO.WBP_INFO_C|GetFixitText (Variables|Widget|GetInfoWidget)) "Hidden"))

(fn HideProgressBar
  (Widget|SetVisibility (Variables|/Game/Blueprints/Widget/WBP_INFO.WBP_INFO_C|GetProgressBar_0 (Variables|Widget|GetInfoWidget)) "Hidden"))

(fn ShowProgressBar
  (Widget|SetVisibility (Variables|/Game/Blueprints/Widget/WBP_INFO.WBP_INFO_C|GetProgressBar_0 (Variables|Widget|GetInfoWidget)) "Visible"))

(fn ShowLeftMouseLOGO
  (params (generator :type Actor%20Object%20Reference))
  (Utilities|IsValid generator
    (:Is%20Valid
      (bind _asbp_chest (Utilities|Casting|CastToBP_Chest generator))
      (if (not (Variables|/Game/Blueprints/interactActor/BP_Chest.BP_Chest_C|GetOpen _asbp_chest))
        (Widget|SetVisibility (Variables|/Game/Blueprints/Widget/WBP_INFO.WBP_INFO_C|GetFixitText (Variables|Widget|GetInfoWidget)) "Visible")
        (Variables|task|SetSelectAvailable true)))))

(fn UpdateProgress
  (Utilities|IsValid (Variables|task|GetChest)
    (:Is%20Valid
      (Utilities|Casting|CastToBP_Chest (Variables|task|GetChest)))))

(fn ActivateCusor
  (bind _asplayer_controller (Utilities|Casting|CastToPlayerController (Pawn|GetController)))
  (Input|SetInputModeGameandUI _asplayer_controller 0 "DoNotLock" true false)
  (Variables|/Script/Engine.PlayerController|SetbShowMouseCursor _asplayer_controller true)
  (task|HideLeftMouseLOGO))

(fn DeactivateCusor
  (bind _asplayer_controller (Utilities|Casting|CastToPlayerController (Pawn|GetController)))
  (Input|SetInputModeGameOnly _asplayer_controller false)
  (Variables|/Script/Engine.PlayerController|SetbShowMouseCursor _asplayer_controller false)
  (Variables|task|SetLock false))

(fn SetRifleMode?
  (if (Variables|Attack|GetRifle?)
    ;[1 1 1] Rifle Mode
    (if (Variables|Attack|GetAiming)
      (Variables|Attack|SetShootable true)
      (Attack|AimMode)
      (else
        (Variables|Attack|SetShootable false)))
    (else
      (Variables|Attack|SetShootable false)
      (Attack|NoneAimMode))))

(fn NoneAimMode
  (bind _returnvalue (Game|GetPlayerCameraManager 0))
  (bind _infowidget (Variables|Widget|GetInfoWidget))
  (bind _springarm (Variables|Default|GetSpringArm))
  (bind _springarm_2 (Variables|Default|GetSpringArm))
  (bind _returnvalue_2 (Class|SpringArmComponent|GetTargetRotation _springarm))
  (Variables|/Script/Engine.SpringArmComponent|SetTargetArmLength _springarm_2 2.5e+02)
  (Transformation|SetRelativeLocation _springarm_2 "0, 0, 0" false false)
  (Variables|/Script/Engine.CharacterMovementComponent|SetbOrientRotationToMovement (Variables|Character|GetCharacterMovement) true)
  (Variables|Default|SetbUseControllerRotationYaw false)
  (Utilities|IsValid _infowidget
    (:Is%20Valid
      (Widget|SetVisibility (Variables|/Game/Blueprints/Widget/WBP_INFO.WBP_INFO_C|Getaim _infowidget) "Hidden")
      (Attack|StopAimAnim)
      (Transformation|SetWorldRotation _springarm (Math|Rotator|MakeRotator (.roll _returnvalue_2) 0.0 (.yaw _returnvalue_2)) false false)
      (Variables|/Script/Engine.PlayerCameraManager|SetViewPitchMin _returnvalue -4e+01)
      (Variables|/Script/Engine.PlayerCameraManager|SetViewPitchMax _returnvalue 4e+01))))

(fn AimMode
  (bind _returnvalue (Game|GetPlayerCameraManager 0))
  (bind _infowidget (Variables|Widget|GetInfoWidget))
  (bind _springarm (Variables|Default|GetSpringArm))
  (bind _springarm_2 (Variables|Default|GetSpringArm))
  (bind _returnvalue_2 (Class|SpringArmComponent|GetTargetRotation _springarm_2))
  (Variables|/Script/Engine.SpringArmComponent|SetTargetArmLength _springarm 1e+02)
  (Transformation|SetRelativeLocation _springarm "0.000000,50.000000,70.000000" false false)
  (Variables|/Script/Engine.CharacterMovementComponent|SetbOrientRotationToMovement (Variables|Character|GetCharacterMovement) false)
  (Variables|Default|SetbUseControllerRotationYaw true)
  (Utilities|IsValid _infowidget
    (:Is%20Valid
      (Widget|SetVisibility (Variables|/Game/Blueprints/Widget/WBP_INFO.WBP_INFO_C|Getaim _infowidget) "Visible")
      (CallFunction|ServerRPCUpdateRotator (Transformation|GetActorRotation))
      (Transformation|SetWorldRotation _springarm_2 (Math|Rotator|MakeRotator (.roll _returnvalue_2) (+ (.pitch _returnvalue_2) (Variables|Attack|GetAction%20Value%20Y)) (.yaw _returnvalue_2)) false false)
      (Variables|/Script/Engine.PlayerCameraManager|SetViewPitchMin _returnvalue -35.0)
      (Variables|/Script/Engine.PlayerCameraManager|SetViewPitchMax _returnvalue 35.0))))

(fn Shoot
  (bind _springarm (Variables|Default|GetSpringArm))
  (Attack|PlayShootAnim)
  (bind (_outhit _returnvalue) (Collision|LineTraceByChannel (Transformation|GetWorldLocation _springarm) (* (Math|Vector|GetForwardVector _springarm) 5e+04) "TraceTypeQuery1" false 0 "ForDuration"))
  (if _returnvalue
    (Effects|SpawnEmitteratLocation "/Game/StarterContent/Particles/P_Explosion.P_Explosion" (.Location (Collision|BreakHitResult _outhit)) "0, 0, 0" "0.500000,0.500000,0.500000")
    (Game|Damage|ApplyDamage (.HitActor (Collision|BreakHitResult _outhit)) 5e+01 0 0)))

(fn PlayAimAnim)

(fn StopAimAnim)

(fn PlaySlashAnim)

(fn StopSlashAnim)

(fn PlayShootAnim)

(fn SetSwordMode?
  (bind _infowidget (Variables|Widget|GetInfoWidget))
  (bind _infowidget_2 (Variables|Widget|GetInfoWidget))
  (bind _springarm (Variables|Default|GetSpringArm))
  (if (Variables|Attack|GetBrret?)
    (if (Variables|Attack|GetAiming)
      (Variables|Attack|SetSlashAvailable true)
      (Variables|/Script/Engine.SpringArmComponent|SetTargetArmLength _springarm 1e+02)
      (Transformation|SetRelativeLocation _springarm "0.000000,0.000000,90.000000" false false)
      (Utilities|IsValid _infowidget_2
        (:Is%20Valid
          (Widget|SetVisibility (Variables|/Game/Blueprints/Widget/WBP_INFO.WBP_INFO_C|Getaim _infowidget_2) "Visible")
          (Variables|/Script/Engine.CharacterMovementComponent|SetbOrientRotationToMovement (Variables|Character|GetCharacterMovement) false)
          (Variables|Default|SetbUseControllerRotationYaw true)
          (CallFunction|ServerRPCUpdateRotator (Transformation|GetActorRotation))))
      (else
        (Variables|Attack|SetSlashAvailable false)
        (Attack|NoneAimMode)
        (Utilities|IsValid _infowidget
          (:Is%20Valid
            (Widget|SetVisibility (Variables|/Game/Blueprints/Widget/WBP_INFO.WBP_INFO_C|Getaim _infowidget) "Hidden")))))
    (else
      (Variables|Attack|SetSlashAvailable false)
      (Attack|NoneAimMode))))

(fn SwordColDisable)

(fn SwordColEnable)

(fn OnRepInventoryArray
  (Default|AddInventory (Variables|Widget|GetInfoWidget) (Variables|item|GetInventory%20Array)))

(fn Interact
  (params (player :type BP%20Parent%20Object%20Reference))
  (return))

(fn MissionResult
  (return false))

(fn RepairState
  (return false))

(fn ReturnItemInfo
  (return ""))