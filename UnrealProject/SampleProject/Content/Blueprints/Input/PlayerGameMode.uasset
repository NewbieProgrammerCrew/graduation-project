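; Game mode that gives each joining player a character from the AvailableCharacters list, which it shuffles on BeginPlay.
; On PostLogin it spawns the class at CharacterIndex at a fixed location and casts it to BP_Ch1.
; It possesses that character with the controller found by the PlayerCount index rather than the login's controller, then increments both counters.
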(event EventBeginPlay
  (Utilities|Array|Shuffle (Variables|Default|GetAvailableCharacters)))

(event EventTick
  (params (DeltaSeconds :type Float%20%28single-precision%29)))

(event EventPostLogin
  (params (NewPlayer :type Player%20Controller%20Object%20Reference))
  (bind _returnvalue (Game|SpawnActorfromClass (Utilities|Array|Get(acopy) (Variables|Default|GetAvailableCharacters) (Variables|Default|GetCharacterIndex)) (Math|Transform|MakeTransform "2670.000000,-510.000000,192.000000" "0, 0, 0" "1.000000,1.000000,1.000000") "Undefined" 0 0))
  (bind _asbp_ch_1 (Utilities|Casting|CastToBP_Ch1 _returnvalue))
  (Utilities|IsValid (Game|GetPlayerController (Variables|Default|GetPlayerCount))
    (:Is%20Valid
      (Pawn|Possess (Game|GetPlayerController (Variables|Default|GetPlayerCount)) _asbp_ch_1)
      (Variables|Default|SetPlayerCount (+ (Variables|Default|GetPlayerCount) 1))
      (Variables|Default|SetCharacterIndex (+ (Variables|Default|GetCharacterIndex) 1)))))

(fn ConstructionScript)