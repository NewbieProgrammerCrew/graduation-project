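; Blueprint for the Abong chaser character, handling its dash skill, stick attack, death and resurrection, and player UI.
; Dash chains timelines and Niagara effects to dissolve the mesh, boost movement and FOV, then reform, with timer-driven cooldown.
; Death and resurrection animate dissolve materials and Niagara, detaching the stick with physics, then reattaching it.
; Tick searches for fuse boxes in view; events update widgets, send attack packets and show win screens.
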(event Custom|ApplyDamage
  ;[0.4531 0 0] Add Widget
  (Animation|PlayAnimMontage "/Game/Animation/Abong/AMTG_Aebong_Attacked.AMTG_Aebong_Attacked" 1.0 "Hitted")
  (Default|CallUpdateCurrentHPtoWidget))

(event Custom|AtkAnimEvent
  ;[0.4531 0 0] Add Widget
  (Utilities|FlowControl|DoOnce false :!label _label
    (:Completed
      (Class|PacketExchangeComponent|SendAttackPacket (Variables|Default|GetPacketExchange))
      (Animation|Montage|PlayMontage (Variables|Character|GetMesh) "/Game/Animation/Abong/AMTG_Aebong_Hit.AMTG_Aebong_Hit" 1.0 0.0 "Attack"
        (:OnCompleted
          (goto _label Reset))
        (:OnBlendOut
          (goto _label Reset))
        (:OnInterrupted
          (goto _label Reset))))))

(event Custom|DashSkillEvent
  ;[0 0.06815 1] DashEffect
  (if (not (Variables|Default|GetDash))
    (Variables|Default|SetDash true)
    (Default|CallDashCoolTime)
    (Utilities|Time|SetTimerbyEvent (delegate Custom|ResetDashCoolTime) 4.0)
    (bind _returnvalue (Utilities|Time|SetTimerbyEvent (delegate Custom|UpdateTime) 1.0 true))
    (Variables|Default|SetNewVar _returnvalue)
    (Animation|Montage|PlayMontage (Variables|Character|GetMesh) "/Game/Static/Characters/Aebong/Animation/MTG_Dash.MTG_Dash"
      (:then
        (Utilities|IsValid (Variables|Material|GetMI_Aebong2)
          (:Is%20Valid
            (bind _newtrack_0 (Timeline|DisappearTimeLine PlayFromStart)
              (:Update
                (Rendering|Material|SetScalarParameterValue (Variables|Material|GetMI_Aebong2) "Animation" _newtrack_0 :!class /Script/Engine.MaterialInstanceDynamic))
              (:Finished
                (bind _returnvalue_2 (Utilities|AttachDashStartEffect))
                (Variables|Default|SetNS_Middle _returnvalue_2)
                (Utilities|DashSetup (Variables|Default|GetDash%20Speed) 1e+09 "0.000000,1000000000.000000,0.000000" false)
                (Utilities|FlowControl|Delay 0.05)
                (Components|Activation|Deactivate (Variables|Default|GetNS_Middle))
                (Utilities|FlowControl|Delay 0.15)
                (bind _returnvalue_3 (Utilities|AttachFireBallEffect))
                (Variables|Default|SetNS_FireBall _returnvalue_3)
                (bind _newtrack_0_2 (Timeline|DashTM PlayFromStart)
                  (:Update
                    (Utilities|ForwardCharacter _newtrack_0_2))
                  (:Finished
                    (Utilities|DashSetup (Variables|Default|GetMax%20Walk%20Speed) (Variables|Default|GetMax%20Acceleration) "0.000000,1000000000.000000,0.000000" true)
                    (Utilities|StopDash (Variables|Default|GetNS_FireBall))
                    (bind _a (Timeline|RegenrateTimeline PlayFromStart)
                      (:Update
                        (Rendering|Material|SetScalarParameterValue (Variables|Material|GetMI_Aebong2) "Animation" _a :!class /Script/Engine.MaterialInstanceDynamic))))))))
          (:Is%20Not%20Valid
            (CallFunction|CreateMeshDynamicMaterial)
            (Timeline|DisappearTimeLine PlayFromStart)))))))

(event Custom|ResetDashCoolTime
  ;[0 0.06815 1] DashEffect
  (Variables|Default|SetDash false)
  (Default|CallResetDashCool)
  (Utilities|Time|PauseTimerbyHandle (Variables|Default|GetNewVar)))

(event Custom|UpdateTime
  ;[0 0.06815 1] DashEffect
  (Default|CallUpdateCoolTime))

(event Custom|UpdatePortalStatusWidget
  ;[0.4531 0 0] Add Widget
  (Default|CallApplyPortalGaugetoWidget))

(event Custom|GameResultWidget
  ;[0.4531 0 0] Add Widget
  (bind _win (Class|BaseChaser|GetGameResult))
  (if _win
    (Widget|RemovefromParent (Variables|Default|GetWBP_PlayerUI))
    (bind _returnvalue (UserInterface|CreateWidget "/Game/Blueprints/WidgetBP/WBP_ChaserWin1.WBP_ChaserWin1_C"))
    (UserInterface|Viewport|AddtoViewport _returnvalue 0)
    (else
      (Widget|RemovefromParent (Variables|Default|GetWBP_PlayerUI))
      (bind _returnvalue_2 (UserInterface|CreateWidget "/Game/Blueprints/WidgetBP/WBP_RunnerWin.WBP_RunnerWin_C"))
      (UserInterface|Viewport|AddtoViewport _returnvalue_2 0))))

(event Custom|DeadEvent
  ;[1 0 0] DeadEvent
  (Variables|Default|Setdead true)
  (Collision|SetCollisionEnabled (Variables|Default|GetCapsuleComponent) "NoCollision")
  (Default|CallUpdateCurrentHPtoWidget)
  (Utilities|IsValid (Variables|Material|GetMI_Stick_handle)
    (:Is%20Valid
      _)
    (:Is%20Not%20Valid
      (CallFunction|CreateStickDynamicMaterial)))
  (Utilities|IsValid (Variables|Material|GetMI_Aebong2)
    (:Is%20Valid
      _)
    (:Is%20Not%20Valid
      (CallFunction|CreateMeshDynamicMaterial)))
  (Utilities|FlowControl|Delay 1.5)
  (Components|Activation|SetActive (Variables|Default|GetSpawnNiagra) true true)
  (bind (_direction _newtrack_0 _newtrack_1) (Timeline|Timeline_0 PlayFromStart)
    (:Update
      (Utilities|UpdateNiagaraParmeterDeadEffect _newtrack_0 _newtrack_1)
      (if (> _newtrack_0 0.5)
        (CallFunction|DetachStick)))
    (:Finished
      (Utilities|FlowControl|Delay 0.4)
      (Utilities|EnableStick)
      (bind (_direction_2 _newtrack_0_2 _newtrack_1_2) (Timeline|Timeline_1 PlayFromStart)
        (:Update
          (Rendering|Material|SetScalarParameterValue (Variables|Material|GetMI_Stick_handle) "Animation" _newtrack_1_2 :!class /Script/Engine.MaterialInstanceDynamic)
          (Rendering|Material|SetScalarParameterValue (Variables|Material|GetMI_Stick_head) "Animation" _newtrack_1_2 :!class /Script/Engine.MaterialInstanceDynamic)
          (Niagara|SetNiagaraVariable(Float) (Variables|Default|GetNM_Stick) "User_Animation" _newtrack_0_2))))))

(event Custom|ResurrentionEvent
  ;[1 0.5448 0] Resurrention
  (Collision|SetCollisionEnabled (Variables|Default|GetCapsuleComponent) "QueryAndPhysics")
  (Default|CallUpdateCurrentHPtoWidget)
  (bind (_rotator _pos) (Class|BaseChaser|GetUpdatedTransform))
  (Transformation|SetActorTransform (Math|Transform|MakeTransform _pos _rotator (Transformation|GetActorScale3D)))
  (CallFunction|AttachStick)
  (Utilities|CheckMaterialAvailable
    (:Is%20Valid
      _)
    (:then
      _))
  (Variables|Default|Setdead false)
  (bind (_direction _niagara _material) (Timeline|Timeline_2 ReverseFromEnd)
    (:Update
      (Utilities|UpdateReSirviveNiagaraEffect _niagara _niagara _material _material)
      (if (<= _niagara 0.08)
        (Components|Activation|SetActive (Variables|Default|GetNM_Stick) false true)
        (Components|Activation|SetActive (Variables|Default|GetSpawnNiagra) false true)))))

(event Custom|HideUI
  ;[0.4531 0 0] Add Widget
  (Default|CallPlayHideResetFuseBoxUIAnim))

(event Custom|AddWidgetEvent
  ;[0.4531 0 0] Add Widget
  (Utilities|IsValid (Variables|Default|GetWBP_PlayerUI)
    (:Is%20Not%20Valid
      (bind _returnvalue (UserInterface|CreateWidget "/Game/Blueprints/WidgetBP/WBP_PlayerChaserStateUI.WBP_PlayerChaserStateUI_C" 0 self))
      (bind _output_get (Variables|Default|SetWBP_PlayerUI _returnvalue))
      (UserInterface|Viewport|AddtoViewport _output_get 0)
      (Default|CallUpdateCurrentHPtoWidget))))

(event Custom|ShowResetFuseBoxUI
  ;[0.4531 0 0] Add Widget
  (Default|CallPlayResetFuseBoxUIAnim))

(event Custom|ResetFuseBoxFirstPersonAnimEvent
  (Transformation|AttachComponentToComponent (Variables|Default|GetStick) (Variables|Character|GetMesh) "BagSocket" "SnapToTarget" "SnapToTarget" "SnapToTarget" true))

(event Custom|ResetFuseBoxThirdPersonAnimEvent
  (Transformation|AttachComponentToComponent (Variables|Default|GetStick) (Variables|Character|GetMesh) "BagSocket" "SnapToTarget" "SnapToTarget" "SnapToTarget" true))

(event Collision|EventActorBeginOverlap
  (params (OtherActor :type Actor%20Object%20Reference)))

(event EventTick
  (params (DeltaSeconds :type Float%20%28single-precision%29))
  (bind _dataupdater (Variables|Default|GetDataUpdater))
  (Class|BaseChaser|FindFuseBoxinView (Transformation|GetWorldLocation (Variables|Default|GetSpringArm)) (Transformation|GetWorldRotation (Variables|Default|GetCamera)) 1.5e+02)
  (Utilities|IsValid _dataupdater
    (:Is%20Valid
      (bind _returnvalue (Class|DataUpdater|GetCurrentSpeed _dataupdater))
      (Variables|Default|SetSpeed _returnvalue))))

(event EventBeginPlay
  (bind _dash_rate (Variables|Default|GetDash%20Rate))
  (Components|Timeline|SetPlayRate (Variables|Default|GetDashTM) _dash_rate)
  (Variables|Default|SetDash%20Speed (* _dash_rate (Variables|Default|GetDashDistance))))

(fn ConstructionScript
  (|CallParentFunction))

(fn PlayAttack)

(fn LaunchCharacterJelly
  (bind _returnvalue (Transformation|GetVelocity))
  (if (> (Math|Vector|VectorLength _returnvalue) 1e+03)
    (Character|LaunchCharacter (* (* (Transformation|GetVelocity) -1.0) 0.5) false false)
    (else
      (Character|LaunchCharacter (* (* _returnvalue -1.0) 4.0) false false))))

(fn DetachStick
  (bind _stick (Variables|Default|GetStick))
  (Transformation|DetachFromComponent (Variables|Default|GetStick) "KeepWorld" "KeepWorld" "KeepWorld" true)
  (Physics|SetSimulatePhysics _stick true)
  (Collision|SetCollisionEnabled _stick "QueryAndPhysics"))

(fn AttachStick
  (bind _stick (Variables|Default|GetStick))
  (Physics|SetSimulatePhysics _stick false)
  (Collision|SetCollisionEnabled _stick "NoCollision")
  (Transformation|AttachComponentToComponent (Variables|Default|GetStick) (Variables|Character|GetMesh) "WeaponSocket" "SnapToTarget" "SnapToTarget" "SnapToTarget" true))

(fn CreateStickDynamicMaterial
  (bind _returnvalue (Rendering|Material|CreateDynamicMaterialInstance (Variables|Default|GetStick) 0 (Rendering|Material|GetMaterial (Variables|Default|GetStick) 0) "None" :!class /Script/Engine.PrimitiveComponent))
  (Variables|Material|SetMI_Stick_handle _returnvalue)
  (bind _returnvalue_2 (Rendering|Material|CreateDynamicMaterialInstance (Variables|Default|GetStick) 1 (Rendering|Material|GetMaterial (Variables|Default|GetStick) 1) "None" :!class /Script/Engine.PrimitiveComponent))
  (Variables|Material|SetMI_Stick_head _returnvalue_2))

(fn CreateMeshDynamicMaterial
  (bind _returnvalue (Rendering|Material|CreateDynamicMaterialInstance (Variables|Character|GetMesh) 0 (Rendering|Material|GetMaterial (Variables|Character|GetMesh) 0) "None" :!class /Script/Engine.PrimitiveComponent))
  (Variables|Material|SetMI_Aebong2 _returnvalue))