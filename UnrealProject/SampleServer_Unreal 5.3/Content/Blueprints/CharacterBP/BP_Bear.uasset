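; Playable Bear runner character with a bomb cannon, extending a parent character with UI, damage, death, montages and foot/hand IK setup.
; Tick shows the held bomb by type, scans for item boxes, rebuilds a spline-mesh trajectory while aiming, and derives turn-in-place flags for local or remote players.
; Events drive the type-specific HUD and a timeline snap to fuse boxes.
; PacketExchange sends pickup, idle and interaction-end packets.
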(event OnComponentBeginOverlap(CapsuleComponent)
  (params (OverlappedComponent :type Primitive%20Component%20Object%20Reference) (OtherActor :type Actor%20Object%20Reference) (OtherComp :type Primitive%20Component%20Object%20Reference) (OtherBodyIndex :type Integer) (bFromSweep :type Boolean) (SweepResult :type Hit%20Result%20Structure%20%28by%20ref%29))
  (bind _asbp_fuse (Utilities|Casting|CastToBP_Fuse OtherActor))
  (bind _returnvalue (Class|DataUpdater|GetFuseCount (Variables|Default|GetDataUpdater)))
  (if (<= _returnvalue 0)
    (bind _returnvalue_2 (Class|Fuse|GetId _asbp_fuse))
    (Class|PacketExchangeComponent|SendGetItemPacket (Variables|Default|GetPacketExchange) _returnvalue_2)))

(event OnComponentEndOverlap(CapsuleComponent)
  (params (OverlappedComponent :type Primitive%20Component%20Object%20Reference) (OtherActor :type Actor%20Object%20Reference) (OtherComp :type Primitive%20Component%20Object%20Reference) (OtherBodyIndex :type Integer))
  (Utilities|Casting|CastToFuseBox OtherActor)
  (if (Variables|Default|GetnoticedFkeyEvent)
    (Default|CallHideNoticeFkey)
    (bind _output_get (Variables|Default|SetnoticedFkeyEvent false))
    (Class|DataUpdater|SetFuseBoxOpenability (Variables|Default|GetDataUpdater) _output_get)
    (Class|DataUpdater|SetFuseBoxOpenandInstall (Variables|Default|GetDataUpdater) -1)))

(event Custom|PlayEarnItem
  ;[1 0.8568 0] Anim
  (Animation|PlayAnimMontage "/Game/Animation/Bear/AMTG_EarnBomb.AMTG_EarnBomb" 1.0 "None"))

(event Custom|BombDecreaseEvent
  ;[0 0.6478 1] UI
  (Default|CallUsedPistol))

(event Custom|StopAimEvent
  ;[1 1 1] Aimming & Attack
  (CallFunction|NaviMode)
  (Default|CallAimHidden))

(event Custom|SetAimMode
  (if (Rendering|IsVisible (Variables|Default|GetStoredBomb))
    (CallFunction|AimMode)
    (Default|CallAimVisible)))

(event Custom|SendIdlePacket
  (Class|PacketExchangeComponent|SendIdlePacket (Variables|Default|GetPacketExchange)))

(event Custom|UpdateOpeningItemBoxStatusWidget
  ;[0 0.2831 0.4115] UI Widget Progress
  (Default|CallUpdateOpeningItemBoxStatus))

(event Custom|ResetOpeningItemBoxStatusWidget
  ;[0 0.2831 0.4115] UI Widget Progress
  (Default|CallResetOpeningItemBoxStatus))

(event Custom|PlayOpenBox
  ;[1 0.8568 0] Anim
  (Class|BaseRunner|SetOpeningBox true))

(event Custom|ShowBoxOpeningUI
  ;[0 0.2831 0.4115] UI Widget Progress
  (Default|CallChangeNoticeImageBox)
  (Default|CallPopupNoticeFKey))

(event Custom|ShowBombAcquiredUI
  ;[0 0.2831 0.4115] UI Widget Progress
  (if (not (Variables|Default|GetnoticeEqipFkey))
    (Default|CallPopupNoticeEqip)
    (Variables|Default|SetnoticeEqipFkey true)))

(event Custom|HideBombAcquiredUI
  ;[0 0.2831 0.4115] UI Widget Progress
  (if (Variables|Default|GetnoticeEqipFkey)
    (Default|CallHideNoticeEqip)
    (Variables|Default|SetnoticeEqipFkey false)))

(event Custom|ApplyDamage
  ;[1 0 0.4436] Damage Event
  (Animation|PlayAnimMontage "/Game/Animation/Bear/AMTG_BearHit.AMTG_BearHit" 1.0 "Hitted")
  (Default|CallGetDamage))

(event Custom|HideUI
  ;[0 0.2831 0.4115] UI Widget Progress
  (Default|CallHideNoticeFkey))

(event Custom|ShowFuseInstallUI
  ;[0 0.2831 0.4115] UI Widget Progress
  (Default|CallChangeNoticeImageFuse)
  (Default|CallPopupNoticeFKey))

(event Custom|ShowFuseBoxOpeningUI
  ;[0 0.2831 0.4115] UI Widget Progress
  (Default|CallChangeNoticeImageFuseBox)
  (Default|CallPopupNoticeFKey))

(event Custom|PlayOpenFuseBox
  ;[1 1 1] Open  FuseBox Interporation Transform
  (bind _returnvalue (Class|BaseRunner|GetCurrentOpeningFuseBox))
  (Variables|Default|SetcurrentFusebox _returnvalue)
  (Utilities|IsValid _returnvalue
    (:Is%20Valid
      (bind _asbp_fuse_box (Utilities|Casting|CastToBP_FuseBox (Variables|Default|GetcurrentFusebox)))
      (bind _interp (Timeline|InterporationFuseBox PlayFromStart)
        (:Update
          (bind (_returnvalue_z _returnvalue_roll _returnvalue_pitch _returnvalue_x _returnvalue_y _returnvalue_yaw) (Utilities|UpdateLerpLocationRotation (Variables|/Game/Blueprints/MyActor/BP_FuseBox.BP_FuseBox_C|GetArrow _asbp_fuse_box) _interp _interp (Variables|/Game/Blueprints/MyActor/BP_FuseBox.BP_FuseBox_C|GetArrow _asbp_fuse_box) (Variables|/Game/Blueprints/MyActor/BP_FuseBox.BP_FuseBox_C|GetArrow _asbp_fuse_box) (Variables|/Game/Blueprints/MyActor/BP_FuseBox.BP_FuseBox_C|GetArrow _asbp_fuse_box))))
        (:Finished
          _))
      (Transformation|SetActorLocationAndRotation (Math|Vector|MakeVector _returnvalue_x _returnvalue_y _returnvalue_z) (Math|Rotator|MakeRotator _returnvalue_roll _returnvalue_pitch _returnvalue_yaw))
      (Class|BaseRunner|SetOpeningFuseBox true))))

(event Custom|InteractionEnd)

(event Custom|SendStopInteractionPacket
  ;[1 1 1] Aimming & Attack
  (if (Variables|/Script/NPC_World.Ch_PlayerController|GetF_KeyPressed (Variables|Default|GetAs%20Ch%20Player%20Controller))
    (Class|PacketExchangeComponent|SendInteractionEndPacket (Variables|Default|GetPacketExchange))))

(event Custom|AttackEvent
  (bind _bombpacketarrow (Variables|Default|GetBombPacketArrow))
  (bind _returnvalue (Transformation|GetWorldLocation _bombpacketarrow))
  ;[1 1 1] Aimming & Attack
  (if (Rendering|IsVisible (Variables|Default|GetChildActor))
    (Camera|PlayWorldCameraShake "/Game/Blueprints/CameraSh_Shoot.CameraSh_Shoot_C" (Transformation|GetActorLocation) 0.0 8e+02)
    (Audio|SpawnSoundatLocation "/Game/Static/Sound/Skill/Runner/Missile-Whoosh.Missile-Whoosh" _returnvalue "0, 0, 0" 0.5 1.0 0.0 "/Game/ChaserDashAttenuation.ChaserDashAttenuation" 0)
    (Rendering|SetVisibility (Variables|Default|GetChildActor) false false)
    (Class|BaseRunner|Fire _returnvalue (Math|Vector|GetForwardVector _bombpacketarrow))))

(event Custom|EscapeEvent
  ;[1 0.08255 0] EscapeEvent
)

(event Custom|GameResultWidget
  (bind _win (Class|BaseRunner|GetGameResult))
  (if _win
    (Widget|RemovefromParent (Variables|Default|GetWBP_PlayerUI))
    (bind _returnvalue (UserInterface|CreateWidget "/Game/Blueprints/WidgetBP/WBP_RunnerWin.WBP_RunnerWin_C"))
    (UserInterface|Viewport|AddtoViewport _returnvalue 0)
    (else
      (Widget|RemovefromParent (Variables|Default|GetWBP_PlayerUI))
      (bind _returnvalue_2 (UserInterface|CreateWidget "/Game/Blueprints/WidgetBP/WBP_ChaserWin1.WBP_ChaserWin1_C"))
      (UserInterface|Viewport|AddtoViewport _returnvalue_2 0))))

(event Custom|BombCountEvent
  ;[0 0.6478 1] UI
  (Default|CallUpdatePossessPistol))

(event Custom|FuseCountEvent
  ;[0 0.6478 1] UI
  (Default|CallUpdatePossessFuse))

(event Custom|UpdatePortalStatusWidget
  ;[0 0.2831 0.4115] UI Widget Progress
  (Default|CallUpdatePortalStatus))

(event Custom|AddWidgetEvent
  ;[0.4531 0 0] Add Widget
  (Utilities|IsValid (Variables|Default|GetWBP_PlayerUI)
    (:Is%20Not%20Valid
      ;;[1 1 1] 1:cowboy              2:dancer             3: soldier          4:student        5: warrior
      (bind _returnvalue (Class|DataUpdater|GetCharacterType (Variables|Default|GetDataUpdater)))
      (switch int _returnvalue
        (:1
          ;;[0.2684 0.01967 1] Cowboy
          (bind _returnvalue_2 (UserInterface|CreateWidget "/Game/Blueprints/WidgetBP/RunnerFolder/WBP_CowboyStateUI.WBP_CowboyStateUI_C" 0 self))
          (Variables|Default|SetWBP_PlayerUI _returnvalue_2))
        (:2
          ;;[0.2684 0.01967 1] Dancer
          (bind _returnvalue_3 (UserInterface|CreateWidget "/Game/Blueprints/WidgetBP/RunnerFolder/WBP_DancerStateUI.WBP_DancerStateUI_C" 0 self))
          (Variables|Default|SetWBP_PlayerUI _returnvalue_3))
        (:3
          ;;[0.2684 0.01967 1] soldier
          (bind _returnvalue_4 (UserInterface|CreateWidget "/Game/Blueprints/WidgetBP/RunnerFolder/WBP_SoldierStateUI.WBP_SoldierStateUI_C" 0 self))
          (Variables|Default|SetWBP_PlayerUI _returnvalue_4))
        (:4
          ;;[0.2661 0 1] Student
          (bind _returnvalue_5 (UserInterface|CreateWidget "/Game/Blueprints/WidgetBP/RunnerFolder/WBP_StudentStateUI.WBP_StudentStateUI_C" 0 self))
          (Variables|Default|SetWBP_PlayerUI _returnvalue_5))
        (:5
          ;;[0.2661 0 1] Warrior
          (bind _returnvalue_6 (UserInterface|CreateWidget "/Game/Blueprints/WidgetBP/RunnerFolder/WBP_WarriorStateUI.WBP_WarriorStateUI_C" 0 self))
          (Variables|Default|SetWBP_PlayerUI _returnvalue_6)))
      (UserInterface|Viewport|AddtoViewport (Variables|Default|GetWBP_PlayerUI) 0)
      (Default|CallGetDamage))))

(event Custom|UpdateFuseStatusWidget
  ;[0 0.2831 0.4115] UI Widget Progress
  (Default|CallUsedFuse))

(event Custom|HideBoxOpeningUI
  ;[0 0.2831 0.4115] UI Widget Progress
  (Default|CallHideNoticeFkey))

(event Custom|DeadEvent
  (bind _charactermovement (Variables|Character|GetCharacterMovement))
  ;[1 0 0.4436] Damage Event
  (Default|CallGetDamage)
  (Utilities|FlowControl|DoOnce false
    (:Completed
      (Components|Animation|PlayAnimation (Variables|Character|GetMesh) "/Game/Static/Characters/Bear/Animation/Bear_Death.Bear_Death" false)
      (Utilities|FlowControl|Delay 2.5)
      (Rendering|SetVisibility (Variables|Character|GetMesh) false false)
      (Collision|SetCollisionEnabled (Variables|Default|GetCapsuleComponent) "NoCollision")
      (Collision|SetCollisionEnabled (Variables|Default|GetBox) "NoCollision")
      (Pawn|Components|CharacterMovement|SetMovementMode _charactermovement "MOVE_Flying" 0)
      (Rendering|SetVisibility (Variables|Default|GetCannonMesh) false false)
      (Variables|/Script/Engine.CharacterMovementComponent|SetGravityScale _charactermovement 0.0))))

(event EventBeginPlay
  (bind _cpt_footik (Variables|Default|GetCpt_FootIK))
  (bind _cpt_intersectionik (Variables|Default|GetCpt_IntersectionIK))
  (bind _returnvalue (Rendering|Material|CreateDynamicMaterialInstance (Variables|Default|GetStoredBomb) 0 "/Game/Static/Mesh/Bomb/material/MI_BombBody.MI_BombBody" "None" :!class /Script/Engine.PrimitiveComponent))
  (Variables|Bomb|SetMI_Bomb _returnvalue)
  (Variables|Default|SetBombMontage "/Game/Static/Characters/Bear/Animation/Bear_Shooting/Bear_Shooting_Animation_Montage.Bear_Shooting_Animation_Montage")
  (Variables|Default|SetprevRotatation (Transformation|GetActorRotation))
  (bind _asch_player_controller (Utilities|Casting|CastToCh_PlayerController (Game|GetPlayerController 0))
    (:then
      (Variables|Default|SetAs%20Ch%20Player%20Controller _asch_player_controller))
    (:CastFailed
      _))
  (Variables|/Script/NPC_World.Cpt_FootIK|Setm_sIKSocketName_LeftFoot _cpt_footik "Bip001-L-Foot")
  (Variables|/Script/NPC_World.Cpt_FootIK|Setm_sIKSocketName_RightFoot _cpt_footik "Bip001-R-Foot")
  (Variables|/Script/NPC_World.Cpt_IntersectionIK|Setm_sIKSocketName_LeftHand _cpt_intersectionik "Bip001-L-Forearm")
  (Variables|/Script/NPC_World.Cpt_IntersectionIK|Setm_sIKSocketName_RightHand _cpt_intersectionik "Bip001-R-Forearm")
  (|CallParentFunction))

(event Collision|EventActorBeginOverlap
  (params (OtherActor :type Actor%20Object%20Reference))
  (|CallParentFunction OtherActor) ; This node is disabled and will not be called.\nDrag off pins to build functionality.
)

(event EventTick
  (params (DeltaSeconds :type Float%20%28single-precision%29))
  (bind _returnvalue (Math|Float|MakeLiteralFloat 0.05))
  (bind _bombpacketarrow (Variables|Default|GetBombPacketArrow))
  (bind _spline (Variables|Default|GetSpline))
  (bind _spline_2 (Variables|Default|GetSpline))
  (bind _pointsarray (Variables|Default|GetPointsArray))
  (|CallParentFunction DeltaSeconds)
  (CallFunction|StoreBomb)
  (Class|BaseRunner|FindItemBoxandCheckEquipableBomb (Transformation|GetWorldLocation (Variables|Default|GetSpringArm)) (Transformation|GetWorldRotation (Variables|Default|GetCamera)) 1.5e+02)
  (Components|DestroyComponent _pointsarray)
  (Utilities|Array|Clear _pointsarray)
  (Spline|ClearSplinePoints (Variables|Default|GetSpline) true)
  (if (and (Variables|Default|GetAiming) (Class|Pawn|IsPawnControlled))
    (bind _outpathpositions (Class|GameplayStatics|BlueprintPredictProjectilePathbyObjectType (Transformation|GetWorldLocation _bombpacketarrow) (* (Math|Vector|GetForwardVector _bombpacketarrow) 5.5e+03) true 2e+01 (Utilities|Array|MakeArray "ObjectTypeQuery1") false 0 "None" 0.0 15.0 1e+01))
    (Utilities|FlowControl|Sequence
      (:then_0
        (if (Class|Pawn|IsPawnControlled) :!label _label
          (Variables|Default|SetARotation (Pawn|GetControlRotation :!class /Script/Engine.Pawn))
          (CallFunction|CheckLocalPlayerTurn)
          (else
            (Variables|Default|SetARotation (Variables|Default|GetprevRotatation))
            (CallFunction|CheckMultiPlayerTurn))))
      (:then_1
        (for (_array_element _array_index) _outpathpositions
          (Spline|AddSplinePointatIndex _spline _array_element _array_index "World" true))
        (Spline|SetSplinePointType _spline (Utilities|Array|LastIndex _outpathpositions) "CurveClamped" true)
        (for _index (range 0 (- (Spline|GetNumberOfSplinePoints _spline) 2))
          (bind _returnvalue_2 (AddComponent|AddSplineMeshComponent true))
          (SplineMesh|SetStartScale _returnvalue_2 (Math|Vector2D|MakeVector2D _returnvalue _returnvalue) true :!class /Script/Engine.SplineMeshComponent)
          (SplineMesh|SetEndScale _returnvalue_2 (Math|Vector2D|MakeVector2D _returnvalue _returnvalue) true :!class /Script/Engine.SplineMeshComponent)
          (Utilities|Array|Add (Variables|Default|GetPointsArray) _returnvalue_2)
          (SplineMesh|SetStartandEnd _returnvalue_2 (Utilities|Array|Get(acopy) _outpathpositions _index) (Spline|GetTangentatSplinePoint _spline_2 _index "World") (Utilities|Array|Get(acopy) _outpathpositions (+ _index 1)) (Spline|GetTangentatSplinePoint _spline_2 (+ _index 1) "World") true :!class /Script/Engine.SplineMeshComponent))))
    (else
      (goto _label))))

(fn ConstructionScript
  (|CallParentFunction))

(fn LaunchCharacterJelly
  (|CallParentFunction))

(fn NaviMode
  (|CallParentFunction))

(fn AimMode
  (bind _returnvalue (Class|BaseRunner|GetCurrentBombType))
  (if (!= _returnvalue 3)
    (|CallParentFunction)))

(fn CheckLocalPlayerTurn
  (bind _returnvalue (Transformation|GetActorRotation))
  (bind _charactermovement (Variables|Character|GetCharacterMovement))
  (bind _charactermovement_2 (Variables|Character|GetCharacterMovement))
  (bind _arotation (Variables|Default|GetARotation))
  (bind _returnvalue_2 (Math|Rotator|Delta(Rotator) _arotation _returnvalue))
  (Utilities|FlowControl|Sequence
    (:then_0
      (if (> (.yaw _returnvalue_2) 2e+01)
        (Variables|Default|SetTurnRight? true)
        (Variables|/Script/Engine.CharacterMovementComponent|SetbUseControllerDesiredRotation _charactermovement true)
        (Variables|/Script/Engine.CharacterMovementComponent|SetbOrientRotationToMovement _charactermovement_2 false)))
    (:then_1
      (if (< (.yaw _returnvalue_2) -25.0)
        (Variables|Default|SetTurnLeft? true)
        (Variables|/Script/Engine.CharacterMovementComponent|SetbUseControllerDesiredRotation _charactermovement true)
        (Variables|/Script/Engine.CharacterMovementComponent|SetbOrientRotationToMovement _charactermovement_2 false)))
    (:then_2
      (if (Math|Float|NearlyEqual(Float) (.yaw _returnvalue_2) 0.0 1.0)
        (Variables|Default|SetTurnRight? false)
        (Variables|Default|SetTurnLeft? false)
        (Variables|/Script/Engine.CharacterMovementComponent|SetbUseControllerDesiredRotation (Variables|Character|GetCharacterMovement) false)
        (Variables|/Script/Engine.CharacterMovementComponent|SetbOrientRotationToMovement (Variables|Character|GetCharacterMovement) false)))))

(fn CheckMultiPlayerTurn
  (bind _returnvalue (Transformation|GetActorRotation))
  (bind _charactermovement (Variables|Character|GetCharacterMovement))
  (bind _charactermovement_2 (Variables|Character|GetCharacterMovement))
  (bind _arotation (Variables|Default|GetARotation))
  (bind _returnvalue_2 (Math|Rotator|Delta(Rotator) _arotation _returnvalue))
  (Utilities|FlowControl|Sequence
    (:then_0
      (if (< (.yaw _returnvalue_2) 0.0)
        (Variables|Default|SetTurnRight? true)
        (Variables|/Script/Engine.CharacterMovementComponent|SetbUseControllerDesiredRotation _charactermovement true)
        (Variables|/Script/Engine.CharacterMovementComponent|SetbOrientRotationToMovement _charactermovement_2 false)))
    (:then_1
      (if (> (.yaw _returnvalue_2) 0.0)
        (Variables|Default|SetTurnLeft? true)
        (Variables|/Script/Engine.CharacterMovementComponent|SetbUseControllerDesiredRotation _charactermovement true)
        (Variables|/Script/Engine.CharacterMovementComponent|SetbOrientRotationToMovement _charactermovement_2 false)))
    (:then_2
      (if (Math|Float|NearlyEqual(Float) (.yaw _returnvalue_2) 0.0 1.0)
        (Variables|Default|SetTurnRight? false)
        (Variables|Default|SetTurnLeft? false)
        (Variables|/Script/Engine.CharacterMovementComponent|SetbUseControllerDesiredRotation (Variables|Character|GetCharacterMovement) false)
        (Variables|/Script/Engine.CharacterMovementComponent|SetbOrientRotationToMovement (Variables|Character|GetCharacterMovement) false))))
  (Variables|Default|SetprevRotatation (Transformation|GetActorRotation)))

(fn StoreBomb
  (bind _mi_bomb (Variables|Bomb|GetMI_Bomb))
  (bind _childactor (Variables|Default|GetChildActor))
  (if (Variables|Default|GetAiming)
    (Utilities|FlowControl|DoOnce false :!label _label
      (:Completed
        (Rendering|SetVisibility (Variables|Default|GetStoredBomb) false false)
        (bind _returnvalue (Class|BaseRunner|GetCurrentBombType))
        (switch int _returnvalue
          (:0
            (ChildActorComponent|SetChildActorClass _childactor "/Game/Blueprints/MyActor/BP_StunBomb.BP_StunBomb_C")
            (Rendering|SetVisibility _childactor true false :!label _label_2))
          (:1
            (ChildActorComponent|SetChildActorClass _childactor "/Game/Blueprints/MyActor/BP_ExplosiveBomb.BP_ExplosiveBomb_C")
            (goto _label_2))
          (:2
            (ChildActorComponent|SetChildActorClass _childactor "/Game/Blueprints/MyActor/BP_InkBomb.BP_InkBomb_C")
            (goto _label_2))
          (:3
            (Rendering|SetVisibility _childactor false false)))))
    (else
      (Utilities|FlowControl|Sequence
        (:then_0
          (goto _label Reset))
        (:then_1
          (Rendering|SetVisibility (Variables|Default|GetChildActor) false false)
          (bind _returnvalue_2 (Class|BaseRunner|GetCurrentBombType))
          (switch int _returnvalue_2
            (:Default
              (Rendering|SetVisibility (Variables|Default|GetStoredBomb) false false :!label _label_3))
            (:0
              (Rendering|Material|SetVectorParameterValue _mi_bomb "Color" "(R=1.000000,G=0.814847,B=0.000000,A=1.000000)" :!class /Script/Engine.MaterialInstanceDynamic)
              (Rendering|Material|SetMaterial (Variables|Default|GetStoredBomb) 0 (Variables|Bomb|GetMI_Bomb) :!label _label_4)
              (Rendering|SetVisibility (Variables|Default|GetStoredBomb) true false))
            (:1
              (Rendering|Material|SetVectorParameterValue _mi_bomb "Color" "(R=1.000000,G=0.000000,B=0.287441,A=1.000000)" :!class /Script/Engine.MaterialInstanceDynamic)
              (goto _label_4))
            (:2
              (Rendering|Material|SetVectorParameterValue _mi_bomb "Color" "(R=0.023153,G=0.023153,B=0.051269,A=1.000000)" :!class /Script/Engine.MaterialInstanceDynamic)
              (goto _label_4))
            (:3
              (goto _label_3))))))))