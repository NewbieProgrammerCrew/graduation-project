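; BP_Abong2 handles a networked skill with a cooldown, triggering Chaser2Skill on the locally controlled BP_Bear.
; SendSkillPacketEvent sends a use-skill packet and starts the dash cooldown display, guarded by the CoolTime flag and a DoOnce against repeat sends.
; SkillEvent starts the eight-second cooldown, calls the Bear's skill and re-arms the DoOnce.
; A looping one-second timer refreshes the cooldown display until the reset pauses it.
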(event Custom|SkillEvent
  ;[0 0.6116 1] Skill
  (Variables|Default|SetCool%20Time true)
  (Utilities|Time|SetTimerbyEvent (delegate Custom|ResetSkillCoolTime) 8.0)
  (bind _returnvalue (Utilities|Time|SetTimerbyEvent (delegate Custom|CustomEvent) 1.0 true))
  (Variables|Default|SetUpdateCoolTimeHandler _returnvalue)
  (bind _asmy_ch_player_controller (Utilities|Casting|CastToMyCh_PlayerController (Game|GetPlayerController 0))
    (:then
      (bind _asbp_bear (Utilities|Casting|CastToBP_Bear (Pawn|GetControlledPawn _asmy_ch_player_controller))
        (:then
          (Default|Chaser2Skill _asbp_bear)
          (Utilities|FlowControl|DoOnce false) ; enters at Reset
        )
        (:CastFailed
          (Utilities|FlowControl|DoOnce false) ; enters at Reset
        )))
    (:CastFailed
      (Utilities|FlowControl|DoOnce false) ; enters at Reset
    )))

(event Custom|SendSkillPacketEvent
  (if (not (Variables|Default|GetCool%20Time))
    (Utilities|FlowControl|DoOnce false
      (:Completed
        (Class|PacketExchangeComponent|SendUseSkillPacket (Variables|Default|GetPacketExchange) 6)
        (Default|CallDashCoolTime)))))

(event Custom|CustomEvent
  ;[0 0.6116 1] Skill
  (Default|CallUpdateCoolTime))

(event Custom|ResetSkillCoolTime
  ;[0 0.6116 1] Skill
  (Variables|Default|SetCool%20Time false)
  (CallFunction|ResetDashCoolTime)
  (Utilities|Time|PauseTimerbyHandle (Variables|Default|GetUpdateCoolTimeHandler)))

(event EventBeginPlay
  (|CallParentFunction)
  (Utilities|FlowControl|DoOnce false) ; enters at Reset
)

(event Collision|EventActorBeginOverlap
  (params (OtherActor :type Actor%20Object%20Reference))
  (|CallParentFunction OtherActor) ; This node is disabled and will not be called.\nDrag off pins to build functionality.
)

(event EventTick
  (params (DeltaSeconds :type Float%20%28single-precision%29))
  (|CallParentFunction DeltaSeconds) ; This node is disabled and will not be called.\nDrag off pins to build functionality.
)

(fn ConstructionScript
  (|CallParentFunction))