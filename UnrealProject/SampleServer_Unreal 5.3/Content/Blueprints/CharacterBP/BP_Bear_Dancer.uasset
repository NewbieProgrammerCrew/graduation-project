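; Bear dancer character Blueprint with a dance skill that shows a mirror ball for the length of a timeline.
; SendSkillPacketEvent sends a use-skill packet and disables the skill when it is neither active nor cooling down.
; SkillEvent runs the dance behind a resettable DoOnce, toggling the dancing state on the local player controller.
; When the timeline finishes, timers drive cooldown updates and later re-enable the skill.
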(event Custom|SkillEvent
  (if (not (Variables|Default|Getdance?))
    (bind _result (CallFunction|GetLocalController))
    (if _result
      (Class|ChPlayerController|ChangeDancing (Variables|Default|GetAs%20Ch%20Player%20Controller_0) true))
    (Utilities|FlowControl|DoOnce false :!label _label
      (:Completed
        (bind _output_get (Variables|Default|Setdance? true))
        (Variables|Default|SetbCoolTime _output_get)
        (Rendering|SetVisibility (Variables|Default|GetMirrorBall) true false)
        (Timeline|ActiveDancePosTime PlayFromStart
          (:Finished
            (Utilities|IsValid (Variables|Default|GetAs%20Ch%20Player%20Controller_0)
              (:Is%20Valid
                (Class|ChPlayerController|ChangeDancing (Variables|Default|GetAs%20Ch%20Player%20Controller_0) false))
              (:Is%20Not%20Valid
                _))
            (Variables|Default|Setdance? false)
            (Rendering|SetVisibility (Variables|Default|GetMirrorBall) false false)
            (Utilities|Time|SetTimerbyEvent (delegate Custom|ResetSkillCoolTime) 7.0)
            (bind _returnvalue (Utilities|Time|SetTimerbyEvent (delegate Custom|UpdateTime) 1.0 true))
            (Variables|Default|SetUpdateCoolTimeHandler _returnvalue)
            (goto _label Reset)))))))

(event Custom|SendSkillPacketEvent
  (if (and (not (Variables|Default|Getdance?)) (not (Variables|Default|GetbCoolTime)))
    (Class|PacketExchangeComponent|SendUseSkillPacket (Variables|Default|GetPacketExchange) 1)
    (Default|CallDisableSkill)))

(event Custom|UpdateTime
  (Default|CallUpdateSkillCoolTime))

(event Custom|ResetSkillCoolTime
  (Variables|Default|SetbCoolTime false)
  (Default|CallEnableSkill)
  (Utilities|Time|PauseTimerbyHandle (Variables|Default|GetUpdateCoolTimeHandler)))

(event EventBeginPlay
  (|CallParentFunction)
  (Variables|Default|SetcoolTime 4.0))

(event Collision|EventActorBeginOverlap
  (params (OtherActor :type Actor%20Object%20Reference))
  (|CallParentFunction OtherActor) ; This node is disabled and will not be called.\nDrag off pins to build functionality.
)

(event EventTick
  (params (DeltaSeconds :type Float%20%28single-precision%29))
  (|CallParentFunction DeltaSeconds) ; This node is disabled and will not be called.\nDrag off pins to build functionality.
)

(fn ConstructionScript
  (|CallParentFunction))

(fn GetLocalController
  (bind _asch_player_controller (Utilities|Casting|CastToCh_PlayerController (Pawn|GetController))
    (:then
      (Variables|Default|SetAs%20Ch%20Player%20Controller_0 _asch_player_controller)
      (Variables|Default|SetGetPlayerControllersucceed true))
    (:CastFailed
      (Variables|Default|SetAs%20Ch%20Player%20Controller_0 0)
      (Variables|Default|SetGetPlayerControllersucceed false)))
  (return (Variables|Default|GetGetPlayerControllersucceed)))