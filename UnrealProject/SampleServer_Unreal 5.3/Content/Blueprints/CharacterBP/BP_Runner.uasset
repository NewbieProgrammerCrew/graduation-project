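; BP_Runner is a runner character Blueprint that displays its current role on a text label in the world.
; Each tick, if its DataUpdater is valid, it copies that object's current speed into its Speed variable and writes the role to the TextRender.
; The label is rotated every tick to face the first player's camera, acting as a billboard.
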(event EventBeginPlay)

(event Collision|EventActorBeginOverlap
  (params (OtherActor :type Actor%20Object%20Reference)))

(event EventTick
  (params (DeltaSeconds :type Float%20%28single-precision%29))
  (bind _textrender (Variables|Default|GetTextRender))
  (bind _dataupdater (Variables|Default|GetDataUpdater))
  (Utilities|IsValid _dataupdater
    (:Is%20Valid
      (bind _returnvalue (Class|DataUpdater|GetCurrentSpeed _dataupdater))
      (bind _returnvalue_2 (Class|DataUpdater|GetRole _dataupdater))
      (Variables|Default|SetSpeed _returnvalue)
      (Rendering|Components|TextRender|SetText (Variables|Default|GetTextRender) (Utilities|Text|ToText(String) _returnvalue_2))
      (Transformation|SetWorldRotation _textrender (Math|Rotator|FindLookatRotation (Transformation|GetWorldLocation _textrender) (Camera|GetCameraLocation (Game|GetPlayerCameraManager 0))) false false))))

(fn ConstructionScript)