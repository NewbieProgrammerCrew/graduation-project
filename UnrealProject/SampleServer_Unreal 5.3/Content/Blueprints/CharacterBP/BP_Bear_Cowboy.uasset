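; Cowboy bear character Blueprint whose skill mounts a spawned horse for a forward dash.
; SendSkillPacketEvent sends the skill packet through a DoOnce, gated on grounded, unmounted and off cooldown.
; SkillEvent jumps, attaches BP_Horse, then a timeline drives forward movement and widens camera FOV at dash speed.
; When the timeline finishes, it destroys the horse, restores movement, starts cooldown timers and resets the DoOnce.
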(event Custom|SkillEvent
  (bind _returnvalue (Transformation|GetActorTransform))
  (bind _curr_jump (Class|DataUpdater|GetJumpStatus (Variables|Default|GetDataUpdater)))
  (if (not _curr_jump)
    (if (not (Variables|Default|GetonHorse?))
      (bind _result (CallFunction|GetLocalController))
      (if _result
        (Class|ChPlayerController|ChangeRideHorse (Variables|Default|GetAs%20Ch%20Player%20Controller_0) true))
      (Variables|Default|SetReturn%20Value%20Location%20Z (.z (.location _returnvalue)))
      (Variables|Default|SetonHorse? true)
      (Variables|Default|SethorseCoolTime true)
      (Character|Jump)
      (Utilities|FlowControl|Delay 0.2)
      (Variables|Default|SetReturn%20Value%20Rotation (.rotation _returnvalue))
      (Transformation|SetRelativeLocationAndRotation (Variables|Character|GetMesh) "0.000000,0.000000,80.000000" (.rotation (Transformation|GetRelativeTransform (Variables|Character|GetMesh))) false false)
      (bind _returnvalue_2 (Game|SpawnActorfromClass "/Game/Blueprints/MyActor/BP_Horse.BP_Horse_C" (Math|Transform|MakeTransform (Math|Vector|MakeVector (.x (.location _returnvalue)) (.y (.location _returnvalue)) (+ (Variables|Default|GetReturn%20Value%20Location%20Z) 45.5)) (Math|Rotator|MakeRotator (.Roll (Math|Rotator|BreakRotator (Variables|Default|GetReturn%20Value%20Rotation))) (.Pitch (Math|Rotator|BreakRotator (Variables|Default|GetReturn%20Value%20Rotation))) (.Yaw (Math|Rotator|BreakRotator (Variables|Default|GetReturn%20Value%20Rotation)))) (.scale _returnvalue)) "Undefined" "MultiplyWithRoot" 0 0))
      (bind _output_get (Variables|Default|SethorseActor _returnvalue_2))
      (Transformation|AttachActorToActor _output_get self "None" "KeepWorld" "KeepWorld" "KeepRelative" true)
      (Utilities|FlowControl|Delay 0.6)
      (Utilities|DashSetup (Variables|Default|GetDash%20Speed) 1e+09 "0.000000,1000000000.000000,0.000000" false)
      (bind _newtrack_0 (Timeline|Timeline_0 PlayFromStart)
        (:Update
          (Utilities|ForwardCharacter _newtrack_0))
        (:Finished
          (Utilities|DashSetup (Variables|Default|GetMax%20Acceleration) (Variables|Default|GetMax%20Walk%20Speed) "0.000000,290.000000,0.000000" false)
          (Utilities|IsValid (Variables|Default|GetAs%20Ch%20Player%20Controller_0)
            (:Is%20Valid
              (Class|ChPlayerController|ChangeRideHorse (Variables|Default|GetAs%20Ch%20Player%20Controller_0) false))
            (:Is%20Not%20Valid
              _))
          (Variables|Default|SetonHorse? false)
          (Transformation|DetachFromActor (Variables|Default|GethorseActor) "KeepWorld" "KeepWorld" "KeepWorld")
          (Actor|DestroyActor (Variables|Default|GethorseActor))
          (Transformation|SetRelativeLocationAndRotation (Variables|Character|GetMesh) "0.000000,0.000000,-53.549186" (.rotation (Transformation|GetRelativeTransform (Variables|Character|GetMesh))) false false)
          (Utilities|Time|SetTimerbyEvent (delegate Custom|ResetSkillCoolTime) 6.0)
          (bind _returnvalue_3 (Utilities|Time|SetTimerbyEvent (delegate Custom|UpdateTime) 1.0 true))
          (Variables|Default|SetUpdateCoolTimeHandler _returnvalue_3)
          (Utilities|FlowControl|DoOnce false) ; enters at Reset
        )))))

(event Custom|SendSkillPacketEvent
  (if (not (AI|Components|NavMovement|IsFalling (Variables|Character|GetCharacterMovement)))
    (if (not (Variables|Default|GethorseCoolTime))
      (if (not (Variables|Default|GetonHorse?))
        (Utilities|FlowControl|DoOnce false
          (:Completed
            (Class|PacketExchangeComponent|SendUseSkillPacket (Variables|Default|GetPacketExchange))
            (Default|CallDisableSkill)))))))

(event Custom|UpdateTime
  (Default|CallUpdateSkillCoolTime))

(event Custom|ResetSkillCoolTime
  (Variables|Default|SethorseCoolTime false)
  (Default|CallEnableSkill)
  (Utilities|Time|PauseTimerbyHandle (Variables|Default|GetUpdateCoolTimeHandler)))

(event EventBeginPlay
  (|CallParentFunction)
  (Variables|Default|SetcoolTime 4.0))

(event Collision|EventActorBeginOverlap
  (params (OtherActor :type Actor%20Object%20Reference))
  (|CallParentFunction OtherActor) ; This node is disabled and will not be called.\nDrag off pins to build functionality.
)

(event EventTick
  (params (DeltaSeconds :type Float%20%28single-precision%29))
  (|CallParentFunction DeltaSeconds) ; This node is disabled and will not be called.\nDrag off pins to build functionality.
)

(fn ConstructionScript
  (|CallParentFunction))

(fn GetLocalController
  (bind _asch_player_controller (Utilities|Casting|CastToCh_PlayerController (Pawn|GetController))
    (:then
      (Variables|Default|SetAs%20Ch%20Player%20Controller_0 _asch_player_controller)
      (Variables|Default|Setsucceed true))
    (:CastFailed
      (Variables|Default|SetAs%20Ch%20Player%20Controller_0 0)
      (Variables|Default|Setsucceed false)))
  (return (Variables|Default|Getsucceed)))