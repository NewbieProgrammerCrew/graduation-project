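; BP_Bear_Soldier is a character Blueprint whose skill event toggles a thermal vision camera effect.
; A FlipFlop alternates between applying thermal post-process settings to the camera and restoring normal ones once the fade-out finishes.
; Two timelines drive the Alpha parameter of a thermal imaging Material Parameter Collection, one reversed and one forward.
; A DoOnce, reset when each timeline finishes, blocks retriggering mid-transition.
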(event Custom|SkillEvent
  (Utilities|FlowControl|DoOnce false :!label _label
    (:Completed
      (Utilities|FlowControl|FlipFlop
        (:A
          (Variables|/Script/Engine.CameraComponent|SetPostProcessSettings (Variables|Default|GetCamera) (Variables|Default|GetThermalVision))
          (bind _value (Timeline|ProceduralMaterial ReverseFromEnd)
            (:Update
              (Rendering|Material|SetScalarParameterValue "/Game/Static/Effect/Material/MPC_ThermalImagingPostProcess.MPC_ThermalImagingPostProcess" "Alpha" _value :!class /Script/Engine.KismetMaterialLibrary))
            (:Finished
              (goto _label Reset))))
        (:B
          (bind _value_2 (Timeline|Timeline PlayFromStart)
            (:Update
              (Rendering|Material|SetScalarParameterValue "/Game/Static/Effect/Material/MPC_ThermalImagingPostProcess.MPC_ThermalImagingPostProcess" "Alpha" _value_2 :!class /Script/Engine.KismetMaterialLibrary))
            (:Finished
              (Variables|/Script/Engine.CameraComponent|SetPostProcessSettings (Variables|Default|GetCamera) (Variables|Default|GetNormalPP))
              (goto _label Reset))))))))

(event EventBeginPlay
  (|CallParentFunction) ; This node is disabled and will not be called.\nDrag off pins to build functionality.
)

(event Collision|EventActorBeginOverlap
  (params (OtherActor :type Actor%20Object%20Reference))
  (|CallParentFunction OtherActor) ; This node is disabled and will not be called.\nDrag off pins to build functionality.
)

(event EventTick
  (params (DeltaSeconds :type Float%20%28single-precision%29))
  (|CallParentFunction DeltaSeconds) ; This node is disabled and will not be called.\nDrag off pins to build functionality.
)

(fn ConstructionScript
  (|CallParentFunction))