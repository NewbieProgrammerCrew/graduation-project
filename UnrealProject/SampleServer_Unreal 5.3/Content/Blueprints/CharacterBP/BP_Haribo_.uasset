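; BP_Haribo_ is the Haribo bear player character, layering UI, animation and networking hooks onto its parent class.
; Events forward to the player state widget for prompts, item counts and damage, and drive aim, shooting and death animations.
; Tick probes from the camera for item boxes and equipable guns, while capsule overlaps collect fuses and clear fuse-box prompts.
; PacketExchange reports actions to the network; DataUpdater stores pistol and fuse-box state.
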(event OnComponentBeginOverlap(CapsuleComponent)
  (params (OverlappedComponent :type Primitive%20Component%20Object%20Reference) (OtherActor :type Actor%20Object%20Reference) (OtherComp :type Primitive%20Component%20Object%20Reference) (OtherBodyIndex :type Integer) (bFromSweep :type Boolean) (SweepResult :type Hit%20Result%20Structure%20%28by%20ref%29))
  (bind _asbp_fuse (Utilities|Casting|CastToBP_Fuse OtherActor))
  (bind _output_get (Variables|Default|SetAs%20BP%20Fuse _asbp_fuse))
  (Class|PacketExchangeComponent|SendGetItemPacket (Variables|Default|GetPacketExchange) (Variables|/Game/Blueprints/MyActor/BP_Fuse.BP_Fuse_C|Getitem_id _output_get))
  (Default|DestroySelf (Variables|Default|GetAs%20BP%20Fuse))
  (Variables|Default|SetAs%20BP%20Fuse 0))

(event OnComponentEndOverlap(CapsuleComponent)
  (params (OverlappedComponent :type Primitive%20Component%20Object%20Reference) (OtherActor :type Actor%20Object%20Reference) (OtherComp :type Primitive%20Component%20Object%20Reference) (OtherBodyIndex :type Integer))
  (Utilities|Casting|CastToFuseBox OtherActor)
  (if (Variables|Default|GetnoticedFkeyEvent)
    (Default|CallHideNoticeFkey)
    (bind _output_get (Variables|Default|SetnoticedFkeyEvent false))
    (Class|DataUpdater|SetFuseBoxOpenability (Variables|Default|GetDataUpdater) _output_get)
    (Class|DataUpdater|SetFuseBoxOpenandInstall (Variables|Default|GetDataUpdater) -1)))

(event Custom|DeadEvent
  ;[1 0 0.4436] Damage Event
  (Default|CallGetDamage)
  (Components|Animation|PlayAnimation (Variables|Character|GetMesh) "/Game/Static/Characters/Bear/Animation/Bear_Death.Bear_Death" false)
  (Utilities|FlowControl|Delay 2.5)
  (Development|SetHiddeninGame (Variables|Character|GetMesh) true false)
  (Pawn|Components|CharacterMovement|SetMovementMode (Variables|Character|GetCharacterMovement) "MOVE_Flying" 0))

(event Custom|PistolDecreaseEvent
  ;[0 0.6478 1] Item
  (Default|CallUsedPistol)
  (Class|DataUpdater|SetDecreasePistolCount (Variables|Default|GetDataUpdater)))

(event Custom|StopAimAnimEvent
  ;[1 0.8568 0] Anim
  (Class|BaseRunner|StopPlayAimAnimation "/Game/Animation/Bear/MTG_BearAttack.MTG_BearAttack" "None")
  (CallFunction|NaviMode)
  (Default|CallAimHidden))

(event Custom|AttackEvent
  (bind _camera (Variables|Default|GetCamera))
  ;[1 0.8568 0] Anim
  (Class|BaseRunner|PlayAttackMontage "/Game/Animation/Bear/MTG_BearAttack.MTG_BearAttack" "Shoot")
  ;;[0 1 0.255] Fire (Ray)
  (Class|BaseRunner|Fire (Transformation|GetWorldLocation _camera) (Transformation|GetWorldRotation _camera) 2e+03 "/Game/StarterContent/Particles/P_Explosion.P_Explosion" "/Game/StarterContent/Particles/P_Explosion.P_Explosion" "/Game/StarterContent/Particles/P_Explosion.P_Explosion" "0.500000,0.500000,0.500000")
  ;;[0.2595 0 1] SendPacket
  (Class|PacketExchangeComponent|SendUsedPistolPacket (Variables|Default|GetPacketExchange)))

(event Custom|SetAimMode
  ;[1 0.8568 0] Anim
  (CallFunction|AimMode)
  (Default|CallAimVisible))

(event Custom|SendIdlePacket
  ;[1 0.8568 0] Anim
  (Class|PacketExchangeComponent|SendIdlePacket (Variables|Default|GetPacketExchange)))

(event Custom|UpdateOpeningItemBoxStatusWidget
  ;[0.4115 0 0] Widget Progress
  (Default|CallUpdateOpeningItemBoxStatus))

(event Custom|ResetOpeningItemBoxStatusWidget
  ;[0.4115 0 0] Widget Progress
  (Default|CallResetOpeningItemBoxStatus))

(event Custom|PlayOpenBox
  ;[1 0.8568 0] Anim
  (Class|BaseRunner|SetOpeningBox true))

(event Custom|ShowBoxOpeningUI
  ;[0.4115 0 0] Widget Progress
  (Default|CallChangeNoticeImageBox)
  (Default|CallPopupNoticeFKey))

(event Custom|ShowGunAcquiredUI
  ;[0.4115 0 0] Widget Progress
  (if (not (Variables|Default|GetnoticeEqipFkey))
    (Default|CallPopupNoticeEqip)
    (Variables|Default|SetnoticeEqipFkey true)))

(event Custom|HideGunAcquiredUI
  ;[0.4115 0 0] Widget Progress
  (if (Variables|Default|GetnoticeEqipFkey)
    (Default|CallHideNoticeEqip)
    (Variables|Default|SetnoticeEqipFkey false)))

(event Custom|ApplyDamage
  ;[1 0 0.4436] Damage Event
  (Default|CallGetDamage))

(event Custom|HideUI
  ;[0.4115 0 0] Widget Progress
  (Default|CallHideNoticeFkey))

(event Custom|ShowFuseInstallUI
  ;[0.4115 0 0] Widget Progress
  (Default|CallChangeNoticeImageFuse)
  (Default|CallPopupNoticeFKey))

(event Custom|ShowFuseBoxOpeningUI
  ;[0.4115 0 0] Widget Progress
  (Default|CallChangeNoticeImageFuseBox)
  (Default|CallPopupNoticeFKey))

(event Custom|PlayOpenFuseBox
  ;[0.4115 0 0] Widget Progress
  (Class|BaseRunner|SetOpeningFuseBox true))

(event Custom|InteractionEnd
  ;[1 0.8568 0] Anim
)

(event Custom|SendStopInteractionPAcket
  (Class|PacketExchangeComponent|SendInteractionEndPacket (Variables|Default|GetPacketExchange)))

(event Custom|HitChaserEvent
  ;[1 0 0.4436] Damage Event
  (Class|PacketExchangeComponent|SendHittedPacket (Variables|Default|GetPacketExchange)))

(event Custom|PistolCountEvent
  ;[0 0.6478 1] Item
  (Default|CallUpdatePossessPistol))

(event Custom|FuseCountEvent
  ;[0 0.6478 1] Item
  (Default|CallUpdatePossessFuse))

(event Custom|UpdatePortalStatusWidget
  ;[0.4115 0 0] Widget Progress
  (Default|CallUpdatePortalStatus))

(event Custom|AddWidgetEvent
  ;[0.4531 0 0] Add Widget
  (Utilities|IsValid (Variables|Default|GetWBP_PlayerUI)
    (:Is%20Not%20Valid
      (bind _returnvalue (UserInterface|CreateWidget "/Game/Blueprints/WidgetBP/WBP_PlayerStateUI.WBP_PlayerStateUI_C" 0 self))
      (bind _output_get (Variables|Default|SetWBP_PlayerUI _returnvalue))
      (UserInterface|Viewport|AddtoViewport _output_get 0)
      (Default|CallGetDamage))))

(event Custom|UpdateFuseStatusWidget
  ;[0.4115 0 0] Widget Progress
  (Default|CallUsedFuse))

(event Custom|HideBoxOpeningUI
  ;[0.4115 0 0] Widget Progress
  (Default|CallHideNoticeFkey))

(event Custom|AimAnimEvent
  ;[1 0.8568 0] Anim
  (Class|BaseRunner|PlayAimAnimation "/Game/Animation/Bear/MTG_BearAttack.MTG_BearAttack" "Aim"))

(event EventBeginPlay
  (bind _cpt_footik (Variables|Default|GetCpt_FootIK))
  (bind _cpt_intersectionik (Variables|Default|GetCpt_IntersectionIK))
  (Variables|/Script/NPC_World.Cpt_FootIK|Setm_sIKSocketName_LeftFoot _cpt_footik "Bip001-L-Foot")
  (Variables|/Script/NPC_World.Cpt_FootIK|Setm_sIKSocketName_RightFoot _cpt_footik "Bip001-R-Foot")
  (Variables|/Script/NPC_World.Cpt_IntersectionIK|Setm_sIKSocketName_LeftHand _cpt_intersectionik "Bip001-L-Forearm")
  (Variables|/Script/NPC_World.Cpt_IntersectionIK|Setm_sIKSocketName_RightHand _cpt_intersectionik "Bip001-R-Forearm")
  (|CallParentFunction))

(event Collision|EventActorBeginOverlap
  (params (OtherActor :type Actor%20Object%20Reference))
  (|CallParentFunction OtherActor) ; This node is disabled and will not be called.\nDrag off pins to build functionality.
)

(event EventTick
  (params (DeltaSeconds :type Float%20%28single-precision%29))
  (|CallParentFunction DeltaSeconds)
  (Class|BaseRunner|FindItemBoxandCheckEquipableGun (Transformation|GetWorldLocation (Variables|Default|GetSpringArm)) (Transformation|GetWorldRotation (Variables|Default|GetCamera)) 1.5e+02))

(fn ConstructionScript
  (|CallParentFunction))

(fn LaunchCharacterJelly
  (|CallParentFunction))

(fn NaviMode
  (|CallParentFunction))

(fn AimMode
  (|CallParentFunction))