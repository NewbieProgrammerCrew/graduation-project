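; BP_Bear_Student is the bear student character Blueprint, handling four skills: Cowboy, Dancer, Soldier and Warrior.
; DataUpdater supplies the skill type for roulette selection and execution, while PacketExchange sends skill-use packets.
; Cowboy spawns a horse for a timed FOV-widening dash, and Dancer shows a mirror ball while setting controller dance state.
; Soldier fades thermal-vision post-processing through a material parameter collection, and Warrior spawns Niagara flower effects.
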(event Custom|DancerSkill
  (bind _as_ch_player_controller_0 (Variables|Default|GetAs%20Ch%20Player%20Controller_0))
  ;[1 1 1] Dancer
  (if (not (Variables|Default|Getdance?))
    (bind _result (CallFunction|GetLocalController))
    (if _result
      (Class|ChPlayerController|ChangeDancing (Variables|Default|GetAs%20Ch%20Player%20Controller_0) true))
    (Utilities|FlowControl|DoOnce false :!label _label
      (:Completed
        (Variables|Default|Setdance? true)
        (Rendering|SetVisibility (Variables|Default|GetMirrorBall) true false)
        (Timeline|Timeline_1 PlayFromStart
          (:Finished
            (Utilities|IsValid _as_ch_player_controller_0
              (:Is%20Valid
                (Class|ChPlayerController|ChangeDancing _as_ch_player_controller_0 false))
              (:Is%20Not%20Valid
                _))
            (Variables|Default|Setdance? false)
            (Rendering|SetVisibility (Variables|Default|GetMirrorBall) false false)
            (goto _label Reset)))))))

(event Custom|SendSkillPacketEvent
  (if (Utilities|Enum|Equal(Enum) (Variables|Default|GetskillEnum) "NewEnumerator4")
    (Class|PacketExchangeComponent|SendUseSkillPacket (Variables|Default|GetPacketExchange) 3)
    (else
      (Class|PacketExchangeComponent|SendUseSkillPacket (Variables|Default|GetPacketExchange) (Variables|Default|GetRandomSkillType)))))

(event Custom|SkillEvent
  (bind _returnvalue (Class|DataUpdater|GetSkillType (Variables|Default|GetDataUpdater)))
  (switch int _returnvalue
    (:0
      (Variables|Default|SetskillEnum "NewEnumerator0"))
    (:1
      (Variables|Default|SetskillEnum "NewEnumerator1"))
    (:2
      (Variables|Default|SetskillEnum "NewEnumerator2"))
    (:4
      (Variables|Default|SetskillEnum "NewEnumerator3")))
  (switch Utilities|FlowControl|Switch|SwitchonSkillEnum (Variables|Default|GetskillEnum)
    (:NewEnumerator0
      (CallFunction|CowboySkill))
    (:NewEnumerator1
      (CallFunction|DancerSkill))
    (:NewEnumerator2
      (CallFunction|SoldierSkill))
    (:NewEnumerator3
      (CallFunction|WarriorSkill)))
  (Variables|Default|SetskillEnum "NewEnumerator4"))

(event Custom|SoldierSkill
  ;[1 1 1] Soldier
  (if (not (Variables|Default|Getthermal))
    (Variables|Default|Setthermal true)
    (Variables|/Script/Engine.CameraComponent|SetPostProcessSettings (Variables|Default|GetCamera) (Variables|Default|GetThermalVision))
    (bind _value (Timeline|Timeline ReverseFromEnd)
      (:Update
        (Rendering|Material|SetScalarParameterValue "/Game/Static/Effect/Material/MPC_ThermalImagingPostProcess.MPC_ThermalImagingPostProcess" "Alpha" _value :!class /Script/Engine.KismetMaterialLibrary))
      (:Finished
        (bind _value_2 (Timeline|Timeline_3 PlayFromStart)
          (:Update
            (Rendering|Material|SetScalarParameterValue "/Game/Static/Effect/Material/MPC_ThermalImagingPostProcess.MPC_ThermalImagingPostProcess" "Alpha" _value_2 :!class /Script/Engine.KismetMaterialLibrary))
          (:Finished
            (Variables|/Script/Engine.CameraComponent|SetPostProcessSettings (Variables|Default|GetCamera) (Variables|Default|GetNormalPP))
            (Variables|Default|Setthermal false)))))))

(event Custom|SelectedSkillEvent
  (bind _returnvalue (Class|DataUpdater|GetSkillType (Variables|Default|GetDataUpdater)))
  (Variables|Default|SetRandomSkillType _returnvalue)
  (Default|CallSpinRoulettEvent)
  (Utilities|FlowControl|Delay 0.8)
  (switch int _returnvalue
    (:0
      (Variables|Default|SetskillEnum "NewEnumerator0"))
    (:1
      (Variables|Default|SetskillEnum "NewEnumerator1"))
    (:2
      (Variables|Default|SetskillEnum "NewEnumerator2"))
    (:4
      (Variables|Default|SetskillEnum "NewEnumerator3"))))

(event Custom|CowboySkill
  (bind _returnvalue (Transformation|GetActorTransform))
  (bind _as_ch_player_controller_0 (Variables|Default|GetAs%20Ch%20Player%20Controller_0))
  ;[1 1 1] Comment
  (bind _curr_jump (Class|DataUpdater|GetJumpStatus (Variables|Default|GetDataUpdater)))
  (if (not _curr_jump)
    (if (not (Variables|Default|GetonHorse?))
      (bind _result (CallFunction|GetLocalController))
      (if _result
        (Class|ChPlayerController|ChangeRideHorse (Variables|Default|GetAs%20Ch%20Player%20Controller_0) true))
      (Variables|Default|SetReturn%20Value%20Location%20Z (.z (.location _returnvalue)))
      (Character|Jump)
      (Utilities|FlowControl|Delay 0.2)
      (Variables|Default|SetonHorse? true)
      (Variables|Default|SetReturn%20Value%20Rotation (.rotation _returnvalue))
      (Transformation|SetRelativeLocationAndRotation (Variables|Character|GetMesh) "0.000000,0.000000,80.000000" (.rotation (Transformation|GetRelativeTransform (Variables|Character|GetMesh))) false false)
      (bind _returnvalue_2 (Game|SpawnActorfromClass "/Game/Blueprints/MyActor/BP_Horse.BP_Horse_C" (Math|Transform|MakeTransform (Math|Vector|MakeVector (.x (.location _returnvalue)) (.y (.location _returnvalue)) (+ (Variables|Default|GetReturn%20Value%20Location%20Z) 45.5)) (Math|Rotator|MakeRotator (.Roll (Math|Rotator|BreakRotator (Variables|Default|GetReturn%20Value%20Rotation))) (.Pitch (Math|Rotator|BreakRotator (Variables|Default|GetReturn%20Value%20Rotation))) (.Yaw (Math|Rotator|BreakRotator (Variables|Default|GetReturn%20Value%20Rotation)))) (.scale _returnvalue)) "Undefined" "MultiplyWithRoot" 0 0))
      (bind _output_get (Variables|Default|SethorseActor _returnvalue_2))
      (Transformation|AttachActorToActor _output_get self "None" "KeepWorld" "KeepWorld" "KeepRelative" true)
      (Utilities|FlowControl|Delay 0.6)
      (Utilities|DashSetup :Max%20Walk%20Speed (Variables|Default|GetDash%20Speed) :Max%20Acceleration 1e+09)
      (bind _newtrack_0 (Timeline|Timeline_2 PlayFromStart)
        (:Update
          (Utilities|ForwardCharacter _newtrack_0))
        (:Finished
          (Utilities|DashSetup (Variables|Default|GetMax%20Acceleration) (Variables|Default|GetMax%20Walk%20Speed) "0.000000,290.000000,0.000000" false)
          (Utilities|IsValid _as_ch_player_controller_0
            (:Is%20Valid
              (Class|ChPlayerController|ChangeRideHorse _as_ch_player_controller_0 false))
            (:Is%20Not%20Valid
              _))
          (Variables|Default|SetonHorse? false)
          (Transformation|DetachFromActor (Variables|Default|GethorseActor) "KeepWorld" "KeepWorld" "KeepWorld")
          (Actor|DestroyActor (Variables|Default|GethorseActor))
          (Transformation|SetRelativeLocationAndRotation (Variables|Character|GetMesh) "0.000000,0.000000,-53.549186" (.rotation (Transformation|GetRelativeTransform (Variables|Character|GetMesh))) false false))))))

(event Custom|WarriorSkill
  ;[1 1 1] Comment
  (Variables|Default|Setflowerend true)
  (bind _returnvalue (Niagara|SpawnSystemAttached "/Game/Static/Effect/NS_Flower.NS_Flower" (Variables|Character|GetMesh) "None" (- (Transformation|GetActorLocation) "0.000000,0.000000,51.000000") "0, 0, 0" "KeepWorldPosition" true))
  (Variables|Default|SetSkillEffect _returnvalue)
  (Niagara|SpawnSystemAttached "/Game/Static/Effect/NS_End_YT1.NS_End_YT1" (Variables|Character|GetMesh) "None" (- (Transformation|GetActorLocation) "0.000000,0.000000,51.000000") "0, 0, 0" "KeepWorldPosition" true)
  (Variables|Default|Setflowerend false))

(event EventBeginPlay
  (|CallParentFunction)
  (Variables|Default|SetskillEnum "NewEnumerator4"))

(event Collision|EventActorBeginOverlap
  (params (OtherActor :type Actor%20Object%20Reference))
  (|CallParentFunction OtherActor) ; This node is disabled and will not be called.\nDrag off pins to build functionality.
)

(event EventTick
  (params (DeltaSeconds :type Float%20%28single-precision%29))
  (|CallParentFunction DeltaSeconds) ; This node is disabled and will not be called.\nDrag off pins to build functionality.
)

(fn ConstructionScript
  (|CallParentFunction))

(fn GetLocalController
  (bind _asch_player_controller (Utilities|Casting|CastToCh_PlayerController (Pawn|GetController))
    (:then
      (Variables|Default|SetAs%20Ch%20Player%20Controller_0 _asch_player_controller)
      (Variables|Default|SetGetPlayerControllersucceed true))
    (:CastFailed
      (Variables|Default|SetAs%20Ch%20Player%20Controller_0 0)
      (Variables|Default|SetGetPlayerControllersucceed false)))
  (return (Variables|Default|GetGetPlayerControllersucceed)))