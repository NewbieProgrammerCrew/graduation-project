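; Bear Warrior character Blueprint that supplies this character's skill behavior on top of a parent class.
; The skill packet event sends use-skill ID 4 through PacketExchange.
; A separate skill event spawns two auto-destroying Niagara effects attached to the mesh, placed just below the actor's location, and stores the flower effect in SkillEffect.
; BeginPlay and construction only call the parent.
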(event Custom|SkillEvent
  (bind _returnvalue (Niagara|SpawnSystemAttached "/Game/Static/Effect/NS_Flower.NS_Flower" (Variables|Character|GetMesh) "None" (- (Transformation|GetActorLocation) "0.000000,0.000000,51.000000") "0, 0, 0" "KeepWorldPosition" true))
  (Variables|Default|SetSkillEffect _returnvalue)
  (Niagara|SpawnSystemAttached "/Game/Static/Effect/NS_End_YT1.NS_End_YT1" (Variables|Character|GetMesh) "None" (- (Transformation|GetActorLocation) "0.000000,0.000000,51.000000") "0, 0, 0" "KeepWorldPosition" true))

(event Custom|SendSkillPacketEvent
  (Class|PacketExchangeComponent|SendUseSkillPacket (Variables|Default|GetPacketExchange) 4))

(event EventBeginPlay
  (|CallParentFunction))

(event Collision|EventActorBeginOverlap
  (params (OtherActor :type Actor%20Object%20Reference))
  (|CallParentFunction OtherActor) ; This node is disabled and will not be called.\nDrag off pins to build functionality.
)

(event EventTick
  (params (DeltaSeconds :type Float%20%28single-precision%29))
  (|CallParentFunction DeltaSeconds) ; This node is disabled and will not be called.\nDrag off pins to build functionality.
)

(fn ConstructionScript
  (|CallParentFunction))