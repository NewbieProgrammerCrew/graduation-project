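; Metaball actor that gives its static mesh a dynamic MI_MetaBall material and slides itself along world X.
; BeginPlay creates the material instance, stores it in MMetaball and applies it to the mesh.
; Tick adds a sine-based X offset scaled by Opposite; the sine takes frame DeltaSeconds rather than elapsed time, so movement drifts with frame time instead of oscillating.
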(event EventBeginPlay
  (bind _returnvalue (Rendering|Material|CreateDynamicMaterialInstance (Variables|Debug|GetStaticMeshComponent) 0 "/Game/Static/Characters/Material/Haribo/MI_MetaBall.MI_MetaBall" "" :!class /Script/Engine.PrimitiveComponent))
  (bind _output_get (Variables|Default|SetM_Metaball _returnvalue))
  (Rendering|Material|SetMaterial (Variables|Debug|GetStaticMeshComponent) 0 _output_get))

(event Collision|EventActorBeginOverlap
  (params (OtherActor :type Actor%20Object%20Reference)))

(event EventTick
  (params (DeltaSeconds :type Float%20%28single-precision%29))
  (Transformation|SetActorLocation (+ (Transformation|GetActorLocation) (Math|Vector|MakeVector (* (* (Math|Trig|Sin(Radians) (* DeltaSeconds 1e+01)) 3.0) (Variables|Default|Getopposite)) 0.0 0.0)) false false))

(fn ConstructionScript)