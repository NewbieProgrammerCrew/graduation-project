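; Map load manager actor that puts the BP_Menu widget on screen at BeginPlay and enables mouse control for it.
; It passes itself to the menu as MapManager; no map loading logic lives in this Blueprint.
; ShowMouse switches the local player controller between Game And UI and Game Only input modes and sets cursor visibility to match.
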(event EventBeginPlay
  (bind _returnvalue (UserInterface|CreateWidget "/Game/Blueprints/WidgetBP/BP_Menu.BP_Menu_C" 0 self))
  (UserInterface|Viewport|AddtoViewport _returnvalue 0)
  (Input|SetInputModeGameandUI (Pawn|GetLocalViewingPlayerController (Game|Player|GetPlayerPawn 0)) 0 "DoNotLock" true false)
  (CallFunction|ShowMouse true))

(event Collision|EventActorBeginOverlap
  (params (OtherActor :type Actor%20Object%20Reference)))

(event EventTick
  (params (DeltaSeconds :type Float%20%28single-precision%29)))

(fn ConstructionScript)

(fn ShowMouse
  (params (mouse? :type Boolean))
  (bind _returnvalue (Game|Player|GetPlayerPawn 0))
  (bind _returnvalue_2 (Pawn|GetLocalViewingPlayerController _returnvalue))
  (if mouse?
    (Input|SetInputModeGameandUI _returnvalue_2 0 "DoNotLock" true false)
    (else
      (Input|SetInputModeGameOnly _returnvalue_2 mouse?)))
  (Variables|/Script/Engine.PlayerController|SetbShowMouseCursor _returnvalue_2 mouse?))