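; BP_lamp1 is a lamp actor with blink logic that flickers a rect light and the lamp's emissive switch together.
; BlinkTimer toggles a flag, sets the light intensity and drives the "sw" parameter on a lazily created dynamic material for Lamp1, then re-arms itself on a short fixed timer.
; BeginPlay checks Blink but starts nothing, and the Lamp2 material step is disconnected.
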(event Custom|BlinkTimer
  (if (Variables|Default|GetNewVar)
    (Variables|Default|SetNewVar false)
    (else
      (Variables|Default|SetNewVar true)))
  (Rendering|Components|Light|SetIntensity (Variables|Default|GetRectLight) (Math|Float|SelectFloat 0.0 82.100204 (Variables|Default|GetNewVar)))
  (Utilities|IsValid (Variables|Default|GetNewVar_0)
    (:Is%20Valid
      _)
    (:Is%20Not%20Valid
      (bind _returnvalue (Rendering|Material|CreateDynamicMaterialInstance (Variables|Default|Getlamp1) 0 "/Game/Static/Mesh/Level3_Asset/MI_lamp.MI_lamp" "None" :!class /Script/Engine.PrimitiveComponent))
      (Variables|Default|SetNewVar_0 _returnvalue)))
  (if (> (Math|Float|SelectFloat 0.0 82.100204 (Variables|Default|GetNewVar)) 0.0)
    (Rendering|Material|SetScalarParameterValue (Variables|Default|GetNewVar_0) "sw" 1.0 :!class /Script/Engine.MaterialInstanceDynamic)
    (else
      (Rendering|Material|SetScalarParameterValue (Variables|Default|GetNewVar_0) "sw" 0.0 :!class /Script/Engine.MaterialInstanceDynamic)))
  (Utilities|Time|SetTimerbyEvent (delegate Custom|BlinkTimer) (Math|Random|RandomFloatinRange 0.1 0.1)))

(event EventBeginPlay
  (if (Variables|Default|GetBlink?)
    _))

(event Collision|EventActorBeginOverlap
  (params (OtherActor :type Actor%20Object%20Reference)))

(event EventTick
  (params (DeltaSeconds :type Float%20%28single-precision%29)))

(fn ConstructionScript)

(fn BlinkLight)