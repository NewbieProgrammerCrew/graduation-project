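; BP_Horse is an actor with four wheel components and a handle mesh that it keeps spinning, apparently as a wheeled horse prop.
; Event Tick adds a shared DeltaRotationSpeed relative rotation to each wheel and a fixed local rotation to the handle.
; Both rotations are applied per frame without delta-time scaling, and the construction script is empty.
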(event Collision|EventActorBeginOverlap
  (params (OtherActor :type Actor%20Object%20Reference)))

(event EventTick
  (params (DeltaSeconds :type Float%20%28single-precision%29))
  (Transformation|AddRelativeRotation (Variables|Default|GetRBWheel) (Variables|Default|GetDelta%20RotationSpeed) false false)
  (Transformation|AddRelativeRotation (Variables|Default|GetRTWheel) (Variables|Default|GetDelta%20RotationSpeed) false false)
  (Transformation|AddRelativeRotation (Variables|Default|GetLBwheel) (Variables|Default|GetDelta%20RotationSpeed) false false)
  (Transformation|AddRelativeRotation (Variables|Default|GetLTWheel) (Variables|Default|GetDelta%20RotationSpeed) false false)
  (Transformation|AddLocalRotation (Variables|Default|Gethandle_mesh) "0.000000,0.000000,10.000000" false false))

(fn ConstructionScript)