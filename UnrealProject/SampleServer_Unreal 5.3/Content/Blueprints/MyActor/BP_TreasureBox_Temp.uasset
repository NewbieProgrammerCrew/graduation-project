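; BP_TreasureBox_Temp is a treasure box actor that drops a pistol pickup when a BP_Runner overlaps its Box trigger.
; Each such overlap spawns a BP_Pistol1 with a random Type, at a random XY point within Box1's extents around the actor and slightly above its origin.
; Nothing limits repeat spawns, and the Itemid set on BeginPlay is never read.
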(event OnComponentBeginOverlap(Box)
  (params (OverlappedComponent :type Primitive%20Component%20Object%20Reference) (OtherActor :type Actor%20Object%20Reference) (OtherComp :type Primitive%20Component%20Object%20Reference) (OtherBodyIndex :type Integer) (bFromSweep :type Boolean) (SweepResult :type Hit%20Result%20Structure%20%28by%20ref%29))
  (bind _returnvalue (Transformation|GetActorLocation))
  (bind _box1 (Variables|Default|GetBox1))
  (bind _returnvalue_2 (Components|Box|GetScaledBoxExtent _box1))
  (Utilities|Casting|CastToBP_Runner OtherActor)
  (Game|SpawnActorfromClass "/Game/Blueprints/MyActor/BP_Pistol1.BP_Pistol1_C" (Math|Transform|MakeTransform (Math|Vector|MakeVector (+ (Math|Random|RandomFloatinRange (* (.x _returnvalue_2) -1.0) (.x _returnvalue_2)) (.x _returnvalue)) (+ (Math|Random|RandomFloatinRange (* (.y _returnvalue_2) -1.0) (.y _returnvalue_2)) (.y _returnvalue)) (+ (.z _returnvalue) 1e+01)) "0, 0, 0" "1.000000,1.000000,1.000000") "Undefined" "MultiplyWithRoot" 0 (Math|Random|RandomIntegerinRange 0 2) 0))

(event EventBeginPlay
  (Variables|Default|Setitemid 20))

(event Collision|EventActorBeginOverlap
  (params (OtherActor :type Actor%20Object%20Reference)))

(event EventTick
  (params (DeltaSeconds :type Float%20%28single-precision%29)))

(fn ConstructionScript)