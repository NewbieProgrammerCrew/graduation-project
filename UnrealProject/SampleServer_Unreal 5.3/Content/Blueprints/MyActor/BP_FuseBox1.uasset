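; Color-coded fuse box actor with a sliding cover, cable and progress-bar widget that tracks its opening progress.
; BeginPlay creates dynamic materials; events tint body and cover by color ID, switching SideColor between that color and black for valid/invalid states.
; Other events show or hide widget and cable, update progress, and play cover Timelines.
; A BP_Bear leaving the box sends an interaction-end packet and stops the progress fill.
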(event OnComponentEndOverlap(Box)
  (params (OverlappedComponent :type Primitive%20Component%20Object%20Reference) (OtherActor :type Actor%20Object%20Reference) (OtherComp :type Primitive%20Component%20Object%20Reference) (OtherBodyIndex :type Integer))
  (bind _asbp_runner (Utilities|Casting|CastToBP_Runner OtherActor))
  (bind _output_get (Variables|Default|SetAs%20BP%20Runner _asbp_runner))
  (bind _asbp_bear (Utilities|Casting|CastToBP_Bear _output_get))
  (Class|PacketExchangeComponent|SendInteractionEndPacket (Variables|/Game/Blueprints/CharacterBP/BP_Bear.BP_Bear_C|GetPacketExchange _asbp_bear))
  (Class|FuseBox|StopFillingProgressBar)
  (Class|BaseRunner|SetOpeningFuseBox _asbp_bear false))

(event Custom|ChangeFuseBoxBaseColor
  (bind _returnvalue (Class|FuseBox|GetColorId))
  (bind _returnvalue_2 (Rendering|Material|CreateDynamicMaterialInstance (Variables|Default|GetSM_Box) 1 "/Game/Static/Mesh/Material/FuseMaterial/MI_FuseBox.MI_FuseBox" "None" :!class /Script/Engine.PrimitiveComponent))
  (Rendering|Material|SetVectorParameterValue _returnvalue_2 "BaseColor" (Utilities|Array|Get(acopy) (Variables|Default|Getcolor) _returnvalue) :!class /Script/Engine.MaterialInstanceDynamic)
  (bind _returnvalue_3 (Rendering|Material|CreateDynamicMaterialInstance (Variables|Default|Get01BoxCover_Box005) 0 "/Game/Static/Mesh/Material/FuseMaterial/MI_FuseBoxCover.MI_FuseBoxCover" "None" :!class /Script/Engine.PrimitiveComponent))
  (Rendering|Material|SetVectorParameterValue _returnvalue_3 "BaseColor" (Utilities|Array|Get(acopy) (Variables|Default|Getcolor) _returnvalue) :!class /Script/Engine.MaterialInstanceDynamic)
  (Rendering|Material|SetMaterial (Variables|Default|GetSM_Box) 1 _returnvalue_2)
  (Rendering|Material|SetMaterial (Variables|Default|Get01BoxCover_Box005) 0 _returnvalue_3))

(event Custom|HiddenWidgetAndCable
  (Development|SetHiddeninGame (Variables|Default|GetWidget) true false)
  (Development|SetHiddeninGame (Variables|Default|GetCable) true false))

(event Custom|VisibleCableAndWidget
  (Development|SetHiddeninGame (Variables|Default|GetWidget) false false)
  (Development|SetHiddeninGame (Variables|Default|GetCable) false false)
  (bind _output (Utilities|BaseColorBody))
  (Utilities|CoverColorBody _output))

(event Custom|UpdateOpeningFuseBoxStatusWidget
  (bind _as_wbp_fuse_box_progress_bar (Variables|Default|GetAs%20WBP%20Fuse%20Box%20Progress%20Bar))
  (bind _returnvalue (Class|FuseBox|GetFuseBoxCurrentProgress))
  (if (!= _returnvalue 0.0)
    (Default|Update _as_wbp_fuse_box_progress_bar _returnvalue)
    (else
      (Default|UpdateEmpty _as_wbp_fuse_box_progress_bar 0.0))))

(event Custom|FillMaxOpeningFuseBoxStatusWidget
  (Default|UpdateMax (Variables|Default|GetAs%20WBP%20Fuse%20Box%20Progress%20Bar) 1.0))

(event Custom|PlayFuseBoxOpen
  (bind _openbox (Timeline|OpenBox PlayFromStart)
    (:Update
      (Transformation|SetRelativeLocation (Variables|Default|Get01BoxCover_Box005) (Math|Vector|MakeVector 0.0 0.0 _openbox) false false))))

(event Custom|PlayFuseBoxClose
  (if (< (.z (Variables|/Script/Engine.SceneComponent|GetRelativeLocation (Variables|Default|Get01BoxCover_Box005))) 0.0)
    (bind _newtrack_0 (Timeline|CloseFuseBox PlayFromStart)
      (:Update
        (Transformation|SetRelativeLocation (Variables|Default|Get01BoxCover_Box005) (Math|Vector|MakeVector 0.0 0.0 _newtrack_0) false false)))))

(event Custom|ChangeValidColor
  (bind _output (Utilities|BaseColorBody))
  (Rendering|Material|SetVectorParameterValue (Variables|Default|GetMI_FuseBox) "SideColor" _output :!class /Script/Engine.MaterialInstanceDynamic)
  (Utilities|CoverColorBody _output)
  (Rendering|Material|SetVectorParameterValue (Variables|Default|GetMI_FuseBoxCover) "SideColor" _output :!class /Script/Engine.MaterialInstanceDynamic)
  (Rendering|Material|SetMaterial (Variables|Default|GetSM_Box) 1 (Variables|Default|GetMI_FuseBox))
  (Rendering|Material|SetMaterial (Variables|Default|Get01BoxCover_Box005) 0 (Variables|Default|GetMI_FuseBoxCover)))

(event Custom|ChangeInvalidColor
  (bind _output (Utilities|BaseColorBody))
  (Rendering|Material|SetVectorParameterValue :self (Variables|Default|GetMI_FuseBox) :ParameterName "SideColor" :!class /Script/Engine.MaterialInstanceDynamic)
  (Utilities|CoverColorBody _output)
  (Rendering|Material|SetVectorParameterValue :self (Variables|Default|GetMI_FuseBoxCover) :ParameterName "SideColor" :!class /Script/Engine.MaterialInstanceDynamic)
  (Rendering|Material|SetMaterial (Variables|Default|GetSM_Box) 1 (Variables|Default|GetMI_FuseBox))
  (Rendering|Material|SetMaterial (Variables|Default|Get01BoxCover_Box005) 0 (Variables|Default|GetMI_FuseBoxCover)))

(event EventTick
  (params (DeltaSeconds :type Float%20%28single-precision%29))
  ;[0.6023 0.7017 1] Rotate HP Bar
)

(event EventBeginPlay
  (bind _returnvalue (Rendering|Material|CreateDynamicMaterialInstance (Variables|Default|GetSM_Box) 1 "/Game/Static/Mesh/Material/FuseMaterial/MI_FuseBox.MI_FuseBox" "None" :!class /Script/Engine.PrimitiveComponent))
  (bind _output_get (Variables|Default|SetMI_FuseBox _returnvalue))
  (Rendering|Material|SetVectorParameterValue :self _output_get :ParameterName "SideColor" :!class /Script/Engine.MaterialInstanceDynamic)
  (bind _returnvalue_2 (Rendering|Material|CreateDynamicMaterialInstance (Variables|Default|Get01BoxCover_Box005) 0 "/Game/Static/Mesh/Material/FuseMaterial/MI_FuseBoxCover.MI_FuseBoxCover" "None" :!class /Script/Engine.PrimitiveComponent))
  (bind _output_get_2 (Variables|Default|SetMI_FuseBoxCover _returnvalue_2))
  (Rendering|Material|SetVectorParameterValue :self _output_get_2 :ParameterName "SideColor" :!class /Script/Engine.MaterialInstanceDynamic)
  (bind _output (Utilities|BaseColorBody))
  (Utilities|CoverColorBody _output)
  (bind _aswbp_fuse_box_progress_bar (Utilities|Casting|CastToWBP_FuseBoxProgressBar (UserInterface|GetUserWidgetObject (Variables|Default|GetWidget))))
  (Variables|Default|SetAs%20WBP%20Fuse%20Box%20Progress%20Bar _aswbp_fuse_box_progress_bar)
  (bind _returnvalue_3 (Rendering|Material|CreateDynamicMaterialInstance (Variables|Default|GetSM_Box) 0 "/Game/Static/Mesh/Material/FuseMaterial/MI_FuseAlert.MI_FuseAlert" "None" :!class /Script/Engine.PrimitiveComponent))
  (bind _output_get_3 (Variables|Default|SetMI_Alert _returnvalue_3))
  (Rendering|Material|SetScalarParameterValue _output_get_3 "Emissive" 0.0 :!class /Script/Engine.MaterialInstanceDynamic))

(fn ConstructionScript)