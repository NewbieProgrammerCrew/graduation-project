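; BP_BombWeapon is a bomb weapon actor with an animated handle and two feet; the graph holds only this cosmetic motion.
; Each Tick spins the Handle by a fixed step, so its speed depends on frame rate.
; A delta-time accumulator drives sine waves that swing the LFeet and RFeet pitch, phase-offset to fake walking without skeletal animation.
; No detonation, damage or movement logic is present.
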(event EventBeginPlay)

(event Collision|EventActorBeginOverlap
  (params (OtherActor :type Actor%20Object%20Reference)))

(event EventTick
  (params (DeltaSeconds :type Float%20%28single-precision%29))
  (Transformation|AddLocalRotation (Variables|Default|GetHandle) "0.000000,0.000000,5.000000" false false)
  (Variables|Default|SetNewVar (+ (* (Utilities|Time|GetWorldDeltaSeconds) 1e+01) (Variables|Default|GetNewVar)))
  (Transformation|SetRelativeRotation (Variables|Default|GetLFeet) (Math|Rotator|MakeRotator 0.0 (* (* (Math|Trig|Sin(Radians) (Variables|Default|GetNewVar)) 1e+01) 5.0) 0.0) false false)
  (Transformation|SetRelativeRotation (Variables|Default|GetRFeet) (Math|Rotator|MakeRotator 0.0 (* (* (Math|Trig|Sin(Radians) (- (Variables|Default|GetNewVar) 1e+01)) 1e+01) 5.0) 0.0) false false))

(fn ConstructionScript)