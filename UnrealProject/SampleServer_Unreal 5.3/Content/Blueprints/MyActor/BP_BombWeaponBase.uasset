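; Base bomb weapon actor with animated walking feet and a spinning handle, whose explosion effect is left to an empty SpawnexplosionEmitter function.
; ColOn arms the collision sphere and Niagara effect, which start with collision off.
; Overlaps other than runners, fuses and item boxes explode it once, also disabling collision on jellies hit.
; ExplosionEmitter offers a guarded alternative detonation; both paths hide the actor, while DestroyBomb destroys it.
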(event OnComponentBeginOverlap(Sphere)
  (params (OverlappedComponent :type Primitive%20Component%20Object%20Reference) (OtherActor :type Actor%20Object%20Reference) (OtherComp :type Primitive%20Component%20Object%20Reference) (OtherBodyIndex :type Integer) (bFromSweep :type Boolean) (SweepResult :type Hit%20Result%20Structure%20%28by%20ref%29))
  (Utilities|Casting|CastToBaseRunner OtherActor
    (:CastFailed
      (Utilities|Casting|CastToBP_Fuse OtherActor
        (:CastFailed
          (Utilities|Casting|CastToBP_ItemBox OtherActor
            (:CastFailed
              (bind _asbp_jelly_1 (Utilities|Casting|CastToBP_Jelly1 OtherActor)
                (:then
                  (Default|DisableCollision _asbp_jelly_1))
                (:CastFailed
                  _))
              (Variables|Default|Setexplosion true)
              (Collision|SetCollisionEnabled (Variables|Default|GetSphere) "NoCollision")
              (Utilities|FlowControl|DoOnce false
                (:Completed
                  (Components|Activation|SetActive (Variables|Default|GetNiagara) false false)
                  (CallFunction|SpawnexplosionEmitter)
                  (Utilities|FlowControl|Delay 0.1)
                  (Rendering|SetActorHiddenInGame true))))))))))

(event Custom|ColOn
  (Collision|SetCollisionEnabled (Variables|Default|GetSphere) "QueryAndPhysics")
  (Components|Activation|SetActive (Variables|Default|GetNiagara) true false))

(event Custom|ExplosionEmitter
  (if (not (Variables|Default|Getexplosion))
    (Utilities|FlowControl|DoOnce false
      (:Completed
        (Variables|Default|Setexplosion true)
        (CallFunction|SpawnexplosionEmitter)
        (Utilities|FlowControl|Delay 0.2)
        (Rendering|SetActorHiddenInGame true)
        (Collision|SetCollisionEnabled (Variables|Default|GetSphere) "NoCollision")
        (Components|Activation|SetActive (Variables|Default|GetNiagara) false false)))))

(event Custom|DestroyBomb
  (Actor|DestroyActor))

(event EventBeginPlay
  (CallFunction|SetColor)
  (Collision|SetCollisionEnabled (Variables|Default|GetSphere) "NoCollision"))

(event Collision|EventActorBeginOverlap
  (params (OtherActor :type Actor%20Object%20Reference)))

(event EventTick
  (params (DeltaSeconds :type Float%20%28single-precision%29))
  (Transformation|AddLocalRotation (Variables|Default|GetHandle) "0.000000,0.000000,5.000000" false false)
  (Variables|Default|SetNewVar (+ (* (Utilities|Time|GetWorldDeltaSeconds) 1e+01) (Variables|Default|GetNewVar)))
  (Transformation|SetRelativeRotation (Variables|Default|GetLFeet) (Math|Rotator|MakeRotator 0.0 (* (* (Math|Trig|Sin(Radians) (Variables|Default|GetNewVar)) 1e+01) 5.0) 0.0) false false)
  (Transformation|SetRelativeRotation (Variables|Default|GetRFeet) (Math|Rotator|MakeRotator 0.0 (* (* (Math|Trig|Sin(Radians) (- (Variables|Default|GetNewVar) 1e+01)) 1e+01) 5.0) 0.0) false false))

(fn ConstructionScript)

(fn SetColor
  (bind _returnvalue (Rendering|Material|CreateDynamicMaterialInstance (Variables|Default|GetBody) 0 "/Game/Static/Mesh/Bomb/material/MI_BombBody.MI_BombBody" "None" :!class /Script/Engine.PrimitiveComponent))
  (Variables|Default|SetBodyMaterial _returnvalue))

(fn SpawnexplosionEmitter)