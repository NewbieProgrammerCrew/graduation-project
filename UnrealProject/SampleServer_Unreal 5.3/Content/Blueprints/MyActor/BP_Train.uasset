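; BP_Train is an actor that shuttles a train back and forth along the world Y axis.
; Each Tick it offsets Y by a scaled sine of the frame delta times a direction variable, giving a small per-frame step rather than an oscillation.
; At hardcoded Y limits on either end, it reverses direction and flips yaw by 180 degrees.
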(event EventBeginPlay)

(event Collision|EventActorBeginOverlap
  (params (OtherActor :type Actor%20Object%20Reference)))

(event EventTick
  (params (DeltaSeconds :type Float%20%28single-precision%29))
  (bind _returnvalue (Transformation|GetActorLocation))
  (Transformation|SetActorLocationAndRotation (+ (Transformation|GetActorLocation) (Math|Vector|MakeVector 0.0 (* (* (Math|Trig|Sin(Radians) (* DeltaSeconds 3.0)) 1e+02) (Variables|Default|Getdir)) 0.0)) (Math|Rotator|MakeRotator 0.0 0.0 (Variables|Default|Getyaw)))
  (if (<= (.y _returnvalue) -7421.0)
    (Variables|Default|Setdir 1.0)
    (Variables|Default|Setyaw 1.8e+02)
    (elif (>= (.y _returnvalue) 6.04e+03)
      (Variables|Default|Setdir -1.0)
      (Variables|Default|Setyaw 0.0))))

(fn ConstructionScript)