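; BP_Jelly1 is a physics-simulated jelly that launches BP_Runner or BP_Abong_ characters when they overlap its skeletal mesh.
; Each character's own LaunchCharacterJelly handles the launch.
; ExplosionJellyEvent, not called within this Blueprint, disables physics and collision, then swaps the mesh for an initially hidden Geometry Cache that plays the explosion.
; Tick prints a debug message whenever that triggered playback is no longer running.
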(event OnComponentBeginOverlap(SkeletalMesh)
  (params (OverlappedComponent :type Primitive%20Component%20Object%20Reference) (OtherActor :type Actor%20Object%20Reference) (OtherComp :type Primitive%20Component%20Object%20Reference) (OtherBodyIndex :type Integer) (bFromSweep :type Boolean) (SweepResult :type Hit%20Result%20Structure%20%28by%20ref%29))
  (bind _asbp_runner (Utilities|Casting|CastToBP_Runner OtherActor)
    (:then
      (Default|LaunchCharacterJelly _asbp_runner))
    (:CastFailed
      (bind _asbp_abong_ (Utilities|Casting|CastToBP_Abong_ OtherActor))
      (Default|LaunchCharacterJelly _asbp_abong_))))

(event Custom|ExplosionJellyEvent
  (bind _skeletalmesh (Variables|Default|GetSkeletalMesh))
  (bind _geometrycache (Variables|Default|GetGeometryCache))
  (Physics|SetSimulatePhysics (Variables|Default|GetSkeletalMesh) false)
  (Collision|SetCollisionEnabled (Variables|Default|GetBox) "NoCollision")
  (Collision|SetCollisionEnabled _skeletalmesh "NoCollision")
  (Development|SetHiddeninGame _skeletalmesh true false)
  (Rendering|SetVisibility _geometrycache true false)
  (Components|Timeline|PlayfromStart _geometrycache)
  (Variables|Default|SetplayCacheGeometry true))

(event EventBeginPlay
  (Rendering|SetVisibility (Variables|Default|GetGeometryCache) false false))

(event Collision|EventActorBeginOverlap
  (params (OtherActor :type Actor%20Object%20Reference)))

(event EventTick
  (params (DeltaSeconds :type Float%20%28single-precision%29))
  (if (Variables|Default|GetplayCacheGeometry)
    (if (not (Audio|Components|Audio|IsPlaying (Variables|Default|GetGeometryCache)))
      (Development|PrintString "end!!!"))))

(fn ConstructionScript
  (Physics|SetSimulatePhysics (Variables|Default|GetSkeletalMesh) true))