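; BP_PortalGate is a portal gate actor that sends an escape packet when a BP_Bear overlaps its box while it is available.
; BeginPlay starts it closed, then runs the opening sequence: a signal sound, delayed Niagara activation and availability, then a portal idle sound.
; OpenPortal waits, then joins that same opening sequence.
; The overlap sends the packet through the bear's PacketExchange.
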(event OnComponentBeginOverlap(Box)
  (params (OverlappedComponent :type Primitive%20Component%20Object%20Reference) (OtherActor :type Actor%20Object%20Reference) (OtherComp :type Primitive%20Component%20Object%20Reference) (OtherBodyIndex :type Integer) (bFromSweep :type Boolean) (SweepResult :type Hit%20Result%20Structure%20%28by%20ref%29))
  (if (Variables|Default|Getavailable)
    (bind _asbp_bear (Utilities|Casting|CastToBP_Bear OtherActor))
    (Class|PacketExchangeComponent|SendEscapePacket (Variables|/Game/Blueprints/CharacterBP/BP_Bear.BP_Bear_C|GetPacketExchange _asbp_bear))))

(event Custom|OpenPortal
  (Utilities|FlowControl|Delay 8.0)
  (Audio|SpawnSoundAttached "/Game/Static/Sound/Actor/portal/boom-signal-4-207063.boom-signal-4-207063" (Variables|Default|GetStaticMesh) "None" (Transformation|GetActorLocation) "0, 0, 0" "KeepWorldPosition" false 1.5 1.0 0.0 0 0)
  (Utilities|FlowControl|Delay 0.5)
  (Components|Activation|SetActive (Variables|Default|GetNiagara) true false)
  (Variables|Default|Setavailable true)
  (Utilities|FlowControl|Delay 0.5)
  (Audio|PlaySoundatLocation "/Game/Static/Sound/Actor/portal/portal_idle-34022.portal_idle-34022" (Transformation|GetActorLocation) "0, 0, 0" 1.0 1.0 0.0 0 0 0 0))

(event EventBeginPlay
  (Components|Activation|SetActive (Variables|Default|GetNiagara) false false)
  (Variables|Default|Setavailable false)
  (Audio|SpawnSoundAttached "/Game/Static/Sound/Actor/portal/boom-signal-4-207063.boom-signal-4-207063" (Variables|Default|GetStaticMesh) "None" (Transformation|GetActorLocation) "0, 0, 0" "KeepWorldPosition" false 1.5 1.0 0.0 0 0)
  (Utilities|FlowControl|Delay 0.5)
  (Components|Activation|SetActive (Variables|Default|GetNiagara) true false)
  (Variables|Default|Setavailable true)
  (Utilities|FlowControl|Delay 0.5)
  (Audio|PlaySoundatLocation "/Game/Static/Sound/Actor/portal/portal_idle-34022.portal_idle-34022" (Transformation|GetActorLocation) "0, 0, 0" 1.0 1.0 0.0 0 0 0 0))

(event Collision|EventActorBeginOverlap
  (params (OtherActor :type Actor%20Object%20Reference)))

(event EventTick
  (params (DeltaSeconds :type Float%20%28single-precision%29)))

(fn ConstructionScript)