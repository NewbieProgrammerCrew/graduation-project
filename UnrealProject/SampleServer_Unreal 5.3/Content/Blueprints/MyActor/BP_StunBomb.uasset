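; BP_StunBomb is a bomb actor variant that supplies its own body color and explosion effects; no stun logic appears in this Blueprint.
; SetColor calls the parent, then tints the BodyMaterial yellow through its Color parameter if that material is valid.
; SpawnexplosionEmitter spawns a scaled-up explosion particle and plays a sound at the actor's location, without calling a parent version.
; The event graph is inactive, and a debug print is left disconnected.
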(event EventBeginPlay
  (|CallParentFunction) ; This node is disabled and will not be called.\nDrag off pins to build functionality.
)

(event Collision|EventActorBeginOverlap
  (params (OtherActor :type Actor%20Object%20Reference))
  (|CallParentFunction OtherActor) ; This node is disabled and will not be called.\nDrag off pins to build functionality.
)

(event EventTick
  (params (DeltaSeconds :type Float%20%28single-precision%29))
  (|CallParentFunction DeltaSeconds) ; This node is disabled and will not be called.\nDrag off pins to build functionality.
)

(fn ConstructionScript
  (|CallParentFunction))

(fn SetColor
  (bind _bodymaterial (Variables|Default|GetBodyMaterial))
  (|CallParentFunction)
  (Utilities|IsValid _bodymaterial
    (:Is%20Valid
      (Rendering|Material|SetVectorParameterValue _bodymaterial "Color" "(R=1.000000,G=0.814847,B=0.000000,A=1.000000)" :!class /Script/Engine.MaterialInstanceDynamic))))

(fn SpawnexplosionEmitter
  (Effects|SpawnEmitteratLocation "/Game/StarterContent/Particles/P_Explosion.P_Explosion" (Transformation|GetActorLocation) "0, 0, 0" "1.500000,1.500000,1.500000")
  (Audio|PlaySoundatLocation "/Game/Static/Sound/Explosion02.Explosion02" (Transformation|GetActorLocation) "0, 0, 0" 1.0 1.0 0.0 0 0 0 0))