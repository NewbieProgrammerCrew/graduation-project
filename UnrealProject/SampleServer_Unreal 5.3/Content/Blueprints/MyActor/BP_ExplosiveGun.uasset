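; BP_ExplosiveGun is a gun actor with a tinted mesh and an explosion particle effect.
; On BeginPlay it creates a dynamic material instance from MI_Gun on GunMesh and sets BaseColor to a pinkish red.
; The FireEmitter event spawns a scaled-down P_Explosion attached to the Arrow component.
; The separate Fire function is a stub that only prints a debug string and does not trigger the emitter.
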(event Custom|FireEmitter
  (bind _arrow (Variables|Default|GetArrow))
  (Effects|SpawnEmitterAttached "/Game/StarterContent/Particles/P_Explosion.P_Explosion" _arrow "None" (Variables|/Script/Engine.SceneComponent|GetRelativeLocation _arrow) "0.000000,90.000000,90.000000" "0.050000,0.050000,0.050000"))

(event EventBeginPlay
  (bind _returnvalue (Rendering|Material|CreateDynamicMaterialInstance (Variables|Default|GetGunMesh) 0 "/Game/Static/Mesh/Material/Gun/MI_Gun.MI_Gun" "None" :!class /Script/Engine.PrimitiveComponent))
  (bind _output_get (Variables|Default|SetNewVar _returnvalue))
  (Rendering|Material|SetVectorParameterValue _output_get "BaseColor" "(R=1.000000,G=0.000000,B=0.366678,A=1.000000)" :!class /Script/Engine.MaterialInstanceDynamic))

(event Collision|EventActorBeginOverlap
  (params (OtherActor :type Actor%20Object%20Reference)))

(event EventTick
  (params (DeltaSeconds :type Float%20%28single-precision%29)))

(fn ConstructionScript)

(fn Fire
  (Development|PrintString "fire"))