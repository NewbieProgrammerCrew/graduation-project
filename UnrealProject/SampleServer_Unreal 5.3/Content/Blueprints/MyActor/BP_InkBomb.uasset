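; BP_InkBomb is an ink bomb actor that supplies an explosion effect.
; SpawnexplosionEmitter prints a debug message, then spawns an enlarged Cascade explosion and plays a sound at the actor's location.
; The event graph holds only disabled stubs, so nothing in this file calls that function.
; An attached Niagara spawn on Body is left unconnected and never runs.
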(event EventBeginPlay
  (|CallParentFunction) ; This node is disabled and will not be called.\nDrag off pins to build functionality.
)

(event Collision|EventActorBeginOverlap
  (params (OtherActor :type Actor%20Object%20Reference))
  (|CallParentFunction OtherActor) ; This node is disabled and will not be called.\nDrag off pins to build functionality.
)

(event EventTick
  (params (DeltaSeconds :type Float%20%28single-precision%29))
  (|CallParentFunction DeltaSeconds) ; This node is disabled and will not be called.\nDrag off pins to build functionality.
)

(fn ConstructionScript
  (|CallParentFunction))

(fn SpawnexplosionEmitter
  (Development|PrintString "InkBomb!" true true "(R=0.328125,G=0.000000,B=0.104531,A=1.000000)")
  (Effects|SpawnEmitteratLocation "/Game/StarterContent/Particles/P_Explosion.P_Explosion" (Transformation|GetActorLocation) "0, 0, 0" "1.500000,1.500000,1.500000")
  (Audio|PlaySoundatLocation "/Game/StarterContent/Audio/Explosion02.Explosion02" (Transformation|GetActorLocation) "0, 0, 0" 1.0 1.0 0.0 0 0 0 0))