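; BP_ConveyerBelt is a conveyor belt actor that carries whatever actors overlap its box.
; Each tick it offsets those actors, except other belts, along the mesh's forward vector at Speed, without sweeping.
; The construction script creates a dynamic belt material with a random color.
; BeginPlay sets that material's negated scroll speed from the ratio of Speed to a default, capped at double.
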(event EventBeginPlay
  (bind _newvar (Variables|Default|GetNewVar))
  (Rendering|Material|SetScalarParameterValue _newvar "speedX" (* (Math|Float|Min(Float) (/ (Variables|Default|Getspeed) (Variables|Default|GetdefaultSpeped)) 2.0) -1.0) :!class /Script/Engine.MaterialInstanceDynamic)
  (Rendering|Material|SetMaterial (Variables|Default|GetConveyer_SM) 0 _newvar))

(event EventTick
  (params (DeltaSeconds :type Float%20%28single-precision%29))
  (for _array_element (Collision|GetOverlappingActors (Variables|Default|GetBox) 0 :!class /Script/Engine.PrimitiveComponent)
    (if (not (.bSuccess (Utilities|Casting|CastToBP_ConveyerBelt _array_element)))
      (Transformation|AddActorWorldOffset _array_element (* (* DeltaSeconds (Variables|Default|Getspeed)) (Math|Vector|GetForwardVector (Transformation|GetWorldRotation (Variables|Default|GetConveyer_SM))))))))

(fn ConstructionScript
  (bind _returnvalue (Rendering|Material|CreateDynamicMaterialInstance (Variables|Default|GetConveyer_SM) 0 "/Game/Static/Mesh/ConveyerBelt/MI_Conveybelt.MI_Conveybelt" "None" :!class /Script/Engine.PrimitiveComponent))
  (bind _output_get (Variables|Default|SetNewVar _returnvalue))
  (Rendering|Material|SetVectorParameterValue _output_get "Color" (Math|Color|MakeColor (Math|Random|RandomFloatinRange 0.0 1.0) (Math|Random|RandomFloatinRange 0.0 1.0) (Math|Random|RandomFloatinRange 0.0 1.0)) :!class /Script/Engine.MaterialInstanceDynamic))