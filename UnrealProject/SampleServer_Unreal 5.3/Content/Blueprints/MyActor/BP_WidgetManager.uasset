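; BP_WidgetManager is an actor that drives the pre-game selection UI flow.
; On BeginPlay it creates the role selection widget, stores it and adds it to the viewport.
; AddSelectCharacterWidget removes and clears that widget if valid, then creates and shows the Chaser character selection widget.
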(event Custom|AddSelectCharacterWidget
  (Utilities|IsValid (Variables|Default|GetSelectRole)
    (:Is%20Valid
      (Widget|RemovefromParent (Variables|Default|GetSelectRole))
      (Variables|Default|SetSelectRole 0))
    (:Is%20Not%20Valid
      _))
  (bind _returnvalue (UserInterface|CreateWidget "/Game/Blueprints/WidgetBP/WBP_SelectCharacter_Chaser.WBP_SelectCharacter_Chaser_C"))
  (Variables|Default|SetSelectCharacter _returnvalue)
  (UserInterface|Viewport|AddtoViewport (Variables|Default|GetSelectCharacter) 0))

(event Custom|AddSelectRoleWidget
  (bind _returnvalue (UserInterface|CreateWidget "/Game/Blueprints/WidgetBP/WBP_SelectRoleWidget.WBP_SelectRoleWidget_C"))
  (Variables|Default|SetSelectRole _returnvalue)
  (UserInterface|Viewport|AddtoViewport (Variables|Default|GetSelectRole) 0))

(event EventBeginPlay
  (CallFunction|AddSelectRoleWidget))

(fn ConstructionScript)