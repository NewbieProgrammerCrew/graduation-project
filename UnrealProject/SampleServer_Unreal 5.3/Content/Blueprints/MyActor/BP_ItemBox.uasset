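; Item box actor with a hinged lid and a bomb inside, which runners can open.
; Open and close events drive lid-rotation timelines and update box status, with the bomb recolored by type during opening.
; Dynamic material instances on body, cap and bomb switch glow colors for availability.
; Box overlap caches the BP_Runner; leaving clears its opening flag and, for BP_Bear, ends interaction and sends a network packet.
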(event OnComponentBeginOverlap(Box)
  (params (OverlappedComponent :type Primitive%20Component%20Object%20Reference) (OtherActor :type Actor%20Object%20Reference) (OtherComp :type Primitive%20Component%20Object%20Reference) (OtherBodyIndex :type Integer) (bFromSweep :type Boolean) (SweepResult :type Hit%20Result%20Structure%20%28by%20ref%29))
  (bind _asbp_runner (Utilities|Casting|CastToBP_Runner OtherActor))
  (Variables|Default|SetAs%20BP%20Runner _asbp_runner))

(event OnComponentEndOverlap(Box)
  (params (OverlappedComponent :type Primitive%20Component%20Object%20Reference) (OtherActor :type Actor%20Object%20Reference) (OtherComp :type Primitive%20Component%20Object%20Reference) (OtherBodyIndex :type Integer))
  (bind _asbp_runner (Utilities|Casting|CastToBP_Runner OtherActor))
  (bind _output_get (Variables|Default|SetAs%20BP%20Runner _asbp_runner))
  (bind _asbp_bear (Utilities|Casting|CastToBP_Bear _output_get))
  (Default|InteractionEnd _asbp_bear)
  (Class|PacketExchangeComponent|SendInteractionEndPacket (Variables|/Game/Blueprints/CharacterBP/BP_Bear.BP_Bear_C|GetPacketExchange _asbp_bear))
  (Class|BaseRunner|SetOpeningBox _output_get false))

(event Custom|CloseCustomEvent
  (bind _openbox (Timeline|Timeline_0 Reverse)
    (:Update
      (Transformation|SetWorldRotation (Variables|Default|GetHead) (Math|Rotator|MakeRotator _openbox 0.0 0.0) false false))
    (:Finished
      (Class|ItemBox|SetBoxStatus false))))

(event Custom|OpenCustomEvent
  (Class|ItemBox|SetBoxStatus true)
  (Utilities|IsValid (Variables|Default|GetAs%20BP%20Runner)
    (:Is%20Valid
      (Class|BaseRunner|SetOpeningBox (Variables|Default|GetAs%20BP%20Runner) false)
      (bind _openbox (Timeline|Timeline PlayFromStart)
        (:Update
          (Transformation|SetRelativeRotation (Variables|Default|GetHead) (Math|Rotator|MakeRotator _openbox 0.0 0.0) false false)
          (bind _returnvalue (Class|ItemBox|GetBombItem))
          (CallFunction|ChangeBombColor _returnvalue))))
    (:Is%20Not%20Valid
      (Timeline|Timeline PlayFromStart))))

(event Custom|DisavailableItemBox
  (bind _bodydynamicmaterialinstance (Variables|Default|GetBodyDynamicMaterialInstance))
  (bind _capdynamicmaterialinstance (Variables|Default|GetCapDynamicMaterialInstance))
  (Rendering|Material|SetVectorParameterValue _bodydynamicmaterialinstance "EmissiveColor" "(R=0.000000,G=0.000000,B=0.000000,A=1.000000)" :!class /Script/Engine.MaterialInstanceDynamic)
  (Rendering|Material|SetMaterial (Variables|Default|GetBody) 0 _bodydynamicmaterialinstance)
  (Rendering|Material|SetVectorParameterValue _capdynamicmaterialinstance "EmissiveColor" "(R=0.000000,G=0.000000,B=0.000000,A=1.000000)" :!class /Script/Engine.MaterialInstanceDynamic)
  (Rendering|Material|SetMaterial (Variables|Default|GetHead) 0 _capdynamicmaterialinstance))

(event Custom|ChangeBombTypeColor
  (bind _returnvalue (Class|ItemBox|GetBombItem))
  (CallFunction|ChangeBombColor _returnvalue))

(event Custom|AvailableItemBox
  (bind _bodydynamicmaterialinstance (Variables|Default|GetBodyDynamicMaterialInstance))
  (bind _capdynamicmaterialinstance (Variables|Default|GetCapDynamicMaterialInstance))
  (Rendering|Material|SetVectorParameterValue _bodydynamicmaterialinstance "EmissiveColor" "(R=0.000000,G=1.000000,B=0.985958,A=1.000000)" :!class /Script/Engine.MaterialInstanceDynamic)
  (Rendering|Material|SetMaterial (Variables|Default|GetBody) 0 _bodydynamicmaterialinstance)
  (Rendering|Material|SetVectorParameterValue _capdynamicmaterialinstance "EmissiveColor" "(R=0.000000,G=1.000000,B=0.985958,A=1.000000)" :!class /Script/Engine.MaterialInstanceDynamic)
  (Rendering|Material|SetMaterial (Variables|Default|GetHead) 0 _capdynamicmaterialinstance))

(event Custom|AvailableBomb
  (bind _bombdynamicmaterialinstance (Variables|Default|GetBombDynamicMaterialInstance))
  (Rendering|Material|SetVectorParameterValue _bombdynamicmaterialinstance "SideColor" "(R=0.000000,G=1.000000,B=0.985958,A=1.000000)" :!class /Script/Engine.MaterialInstanceDynamic)
  (Rendering|Material|SetMaterial (Variables|Default|GetBombBody) 0 _bombdynamicmaterialinstance))

(event Custom|DisavailableBomb
  (bind _bombdynamicmaterialinstance (Variables|Default|GetBombDynamicMaterialInstance))
  (Rendering|Material|SetVectorParameterValue _bombdynamicmaterialinstance "SideColor" "(R=0.000000,G=0.000000,B=0.000000,A=1.000000)" :!class /Script/Engine.MaterialInstanceDynamic)
  (Rendering|Material|SetMaterial (Variables|Default|GetBombBody) 0 _bombdynamicmaterialinstance))

(event Collision|EventActorBeginOverlap
  (params (OtherActor :type Actor%20Object%20Reference)))

(event EventBeginPlay
  (bind _returnvalue (Rendering|Material|CreateDynamicMaterialInstance (Variables|Default|GetBody) 0 "/Game/Static/Mesh/Texture/ItemBox/MI_ItemBox_Body.MI_ItemBox_Body" "None" :!class /Script/Engine.PrimitiveComponent))
  (Variables|Default|SetBodyDynamicMaterialInstance _returnvalue)
  (bind _returnvalue_2 (Rendering|Material|CreateDynamicMaterialInstance (Variables|Default|GetHead) 0 "/Game/Static/Mesh/Texture/ItemBox/MI_ItemBox_Cap.MI_ItemBox_Cap" "None" :!class /Script/Engine.PrimitiveComponent))
  (Variables|Default|SetCapDynamicMaterialInstance _returnvalue_2)
  (bind _returnvalue_3 (Rendering|Material|CreateDynamicMaterialInstance (Variables|Default|GetBombBody) 0 "/Game/Static/Mesh/Bomb/material/MI_BombBodyInBox.MI_BombBodyInBox" "None" :!class /Script/Engine.PrimitiveComponent))
  (Variables|Default|SetBombDynamicMaterialInstance _returnvalue_3))

(fn ConstructionScript)

(fn ChangeBombColor
  (params (type :type Integer))
  (bind _bombdynamicmaterialinstance (Variables|Default|GetBombDynamicMaterialInstance))
  (bind _bombbody (Variables|Default|GetBombBody))
  (switch int type
    (:0
      (Rendering|Material|SetVectorParameterValue (Variables|Default|GetBombDynamicMaterialInstance) "Color" "(R=1.000000,G=0.814847,B=0.000000,A=1.000000)" :!class /Script/Engine.MaterialInstanceDynamic)
      (Rendering|Material|SetMaterial _bombbody 0 (Variables|Default|GetBombDynamicMaterialInstance)))
    (:1
      (Rendering|Material|SetVectorParameterValue _bombdynamicmaterialinstance "Color" "(R=1.000000,G=0.000000,B=0.287441,A=1.000000)" :!class /Script/Engine.MaterialInstanceDynamic)
      (Rendering|Material|SetMaterial _bombbody 0 _bombdynamicmaterialinstance))
    (:2
      (Rendering|Material|SetVectorParameterValue (Variables|Default|GetBombDynamicMaterialInstance) "Color" "(R=0.023153,G=0.023153,B=0.051269,A=1.000000)" :!class /Script/Engine.MaterialInstanceDynamic)
      (Rendering|Material|SetMaterial _bombbody 0 (Variables|Default|GetBombDynamicMaterialInstance)))))