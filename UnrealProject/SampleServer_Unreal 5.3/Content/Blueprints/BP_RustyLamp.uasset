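; BP_RustyLamp is a lamp actor with a spotlight that blinks on and off at slightly irregular intervals.
; BeginPlay starts a timer with a short random delay that calls BlinkLight.
; BlinkLight flips a boolean, switches the spotlight intensity between zero and a fixed brightness, then re-arms the timer with a new random delay, so the flicker loops without Tick.
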(event EventBeginPlay
  (Utilities|Time|SetTimerbyFunctionName 0 "BlinkLight" (Math|Random|RandomFloatinRange 0.3 0.4)))

(event Collision|EventActorBeginOverlap
  (params (OtherActor :type Actor%20Object%20Reference)))

(event EventTick
  (params (DeltaSeconds :type Float%20%28single-precision%29)))

(fn ConstructionScript)

(fn BlinkLight
  (if (Variables|Default|GetNewVar)
    (Variables|Default|SetNewVar false)
    (else
      (Variables|Default|SetNewVar true)))
  (Rendering|Components|Light|SetIntensity (Variables|Default|GetSpotLight) (Math|Float|SelectFloat 0.0 1362.213013 (Variables|Default|GetNewVar)))
  (Utilities|Time|SetTimerbyFunctionName 0 "BlinkLight" (Math|Random|RandomFloatinRange 0.3 0.4)))